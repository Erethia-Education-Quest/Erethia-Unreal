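; Incomplete fresco puzzle (fresco02) that players complete by bringing four grabbable pieces to their slots.
; Four detection areas match pieces by actor tag, snap them to their positions and flag them attached.
; Snapping disables physics and collision and releases the grabbing player's hold, replicated by calling each player controller from the GameInstance's player list.
; Once all four pieces are attached, the fresco switches to its complete state.
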(event `self.ReceiveBeginPlay`
  (`parent.ReceiveBeginPlay`)
  (bind _asbp_game_instance (cast `/Game/Blueprint/GameInstance/BP_GameInstance` (`GameplayStatics.GetGameInstance`)))
  (set `self.Ref_GI` _asbp_game_instance)
  (bind _asgs_game (cast `/Game/Blueprint/GameState/GS_Game` (`GameplayStatics.GetGameState`)))
  (set `self.Ref_GS` _asgs_game))

(event `self.DetectionArea1.OnComponentBeginOverlap`
  (params (OverlappedComponent :type "PrimitiveComponent Object Reference") (OtherActor :type "Actor Object Reference") (OtherComp :type "PrimitiveComponent Object Reference") (OtherBodyIndex :type Integer) (bFromSweep :type Boolean) (SweepResult :type "HitResult Structure (by ref)"))
  (if (`self.ActorHasTag` OtherActor "Piece2_1")
    (`self.ReleaseAndSnapObjectNetwork` OtherActor (`self.SnapPosition_1`))
    (set `self.Piece_1_Attached` true)
    (`self.Finish?`)))

(event `self.DetectionArea2.OnComponentBeginOverlap`
  (params (OverlappedComponent :type "PrimitiveComponent Object Reference") (OtherActor :type "Actor Object Reference") (OtherComp :type "PrimitiveComponent Object Reference") (OtherBodyIndex :type Integer) (bFromSweep :type Boolean) (SweepResult :type "HitResult Structure (by ref)"))
  (if (`self.ActorHasTag` OtherActor "Piece2_2")
    (`self.ReleaseAndSnapObjectNetwork` OtherActor (`self.SnapPosition_2`))
    (set `self.Piece_2_Attached` true)
    (`self.Finish?`)))

(event `self.DetectionArea3.OnComponentBeginOverlap`
  (params (OverlappedComponent :type "PrimitiveComponent Object Reference") (OtherActor :type "Actor Object Reference") (OtherComp :type "PrimitiveComponent Object Reference") (OtherBodyIndex :type Integer) (bFromSweep :type Boolean) (SweepResult :type "HitResult Structure (by ref)"))
  (if (`self.ActorHasTag` OtherActor "Piece2_3")
    (`self.ReleaseAndSnapObjectNetwork` OtherActor (`self.SnapPosition_3`))
    (set `self.Piece_3_Attached` true)
    (`self.Finish?`)))

(event `self.DetectionArea4.OnComponentBeginOverlap`
  (params (OverlappedComponent :type "PrimitiveComponent Object Reference") (OtherActor :type "Actor Object Reference") (OtherComp :type "PrimitiveComponent Object Reference") (OtherBodyIndex :type Integer) (bFromSweep :type Boolean) (SweepResult :type "HitResult Structure (by ref)"))
  (if (`self.ActorHasTag` OtherActor "Piece2_4")
    (`self.ReleaseAndSnapObjectNetwork` OtherActor (`self.SnapPosition_4`))
    (set `self.Piece_4_Attached` true)
    (`self.Finish?`)))

(event `ReleaseAndSnapObjectNetwork`
  (params (FrescoPiece :type "Actor Object Reference") (SnapPosition :type "StaticMeshComponent Object Reference"))
  (bind _ref_gi (`self.Ref_GI`))
  (`self.ReleaseAndSnapObjectServeur` FrescoPiece SnapPosition)
  (if (and (`KismetSystemLibrary.IsValid` _ref_gi) (`KismetSystemLibrary.IsValid` (`self.Ref_GS`)))
    (for _array_element (`/Game/Blueprint/GameInstance/BP_GameInstance.ListPlayerInfo` _ref_gi)
      (bind _aspc_game (cast `/Game/Blueprint/PlayerController/PC_Game` (`.PC_11_776544A84872013AA63BC881D8B483A2` (break `/Game/Struct/S_PlayerInfo` _array_element))))
      (`/Game/Blueprint/PlayerController/PC_Game.ReleaseAndSnapObjectClient2` _aspc_game FrescoPiece self SnapPosition))))

(event `ReleaseAndSnapObjectServeur`
  (params (FrescoPiece :type "Actor Object Reference") (SnapPosition :type "StaticMeshComponent Object Reference"))
  (`self.ReleaseAndSnapObject` FrescoPiece SnapPosition))

(event `ReleaseAndSnapObjectClient2`
  (params (FrescoPiece :type "Actor Object Reference") (SnapPosition :type "StaticMeshComponent Object Reference"))
  (`self.ReleaseAndSnapObject` FrescoPiece SnapPosition))

(event `Finish?`
  (if (and (`self.Piece_1_Attached`) (`self.Piece_2_Attached`) (`self.Piece_3_Attached`) (`self.Piece_4_Attached`))
    (`self.ChangeCompleteState` true)))

(fn `ReleaseAndSnapObject`
  (params (FrescoPiece :type "Actor Object Reference") (SnapPosition :type "StaticMeshComponent Object Reference"))
  (bind _asbp_master_grabbable_objects (cast `/Game/Blueprint/InteractiveObject/Gabable_OBJ/BP_MasterGrabbableObjects` FrescoPiece))
  (`/Engine/EditorBlueprintResources/StandardMacros.IsValid` _asbp_master_grabbable_objects
    (:`Is Valid`
      (bind _object (`/Game/Blueprint/InteractiveObject/BP_MasterInteractive.Object` _asbp_master_grabbable_objects))
      (`PrimitiveComponent.SetSimulatePhysics` _object false)
      (`PrimitiveComponent.SetEnableGravity` _object false)
      (`/Game/Blueprint/InteractiveObject/Gabable_OBJ/BP_MasterGrabbableObjects.SetPositionFresco` _asbp_master_grabbable_objects (`SceneComponent.K2_GetComponentToWorld` SnapPosition))
      (`PrimitiveComponent.SetCollisionEnabled` _object "NoCollision")
      (bind _playergrabing (`/Game/Blueprint/InteractiveObject/Gabable_OBJ/BP_MasterGrabbableObjects.PlayerGrabing` _asbp_master_grabbable_objects))
      (`/Engine/EditorBlueprintResources/StandardMacros.IsValid` _playergrabing
        (:`Is Valid`
          (`/Game/Blueprint/Player/BP_Player.ReleaseObjectServer` _playergrabing "NewEnumerator1"))
        (:`Is Not Valid`
          _))
      (`/Engine/EditorBlueprintResources/StandardMacros.IsValid` _playergrabing
        (:`Is Valid`
          (`/Game/Blueprint/Player/BP_Player.ReleaseObjectServer` _playergrabing "NewEnumerator2"))))))

(fn `UserConstructionScript`)