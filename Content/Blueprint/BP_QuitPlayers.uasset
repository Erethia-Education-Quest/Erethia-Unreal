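; BP_QuitPlayers is a trigger volume that sends all players back to the lobby.
; It caches the GM_Game game mode on BeginPlay.
; When a BP_Player capsule overlaps its Box, the server calls SendAllPlayerToLobby on that game mode, so one player entering moves everyone.
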(event `self.ReceiveBeginPlay`
  (`|ExecutionSequence`
    (:`then_0`
      (bind _asgm_game (cast `/Game/Blueprint/GameMode/GM_Game` (`GameplayStatics.GetGameMode`)))
      (set `self.RefGM` _asgm_game))))

(event `self.Box.OnComponentBeginOverlap`
  (params (OverlappedComponent :type "PrimitiveComponent Object Reference") (OtherActor :type "Actor Object Reference") (OtherComp :type "PrimitiveComponent Object Reference") (OtherBodyIndex :type Integer) (bFromSweep :type Boolean) (SweepResult :type "HitResult Structure (by ref)"))
  (if (and (== (`GameplayStatics.GetObjectClass` OtherActor) "/Game/Blueprint/Player/BP_Player.BP_Player_C") (== (`GameplayStatics.GetObjectClass` OtherComp) "/Script/Engine.CapsuleComponent") (`self.HasAuthority`))
    (bind _refgm (`self.RefGM`)
      (:`then`
        (`/Game/Blueprint/GameMode/GM_Game.SendAllPlayerToLobby` _refgm))
      (:`else`))))

(fn `UserConstructionScript`)