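; Challenge manager that triggers a set of interactive items once all challenges in its list are completed.
; On BeginPlay it registers itself as each challenge's master and drops invalid entries.
; Challenges report completion or reversal to a counter; at full count it verifies every challenge, then activates the items on the server.
; It then has GS_Master relay activation for each player in the GameInstance's list, with a matching client-side activation event.
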(event `self.ReceiveBeginPlay`
  (`|ExecutionSequence`
    (:`then_0`
      (bind _asgs_master (cast `/Game/Blueprint/GameState/GS_Master` (`GameplayStatics.GetGameState`)))
      (set `self.RefGS` _asgs_master))
    (:`then_1`
      (bind _asbp_game_instance (cast `/Game/Blueprint/GameInstance/BP_GameInstance` (`GameplayStatics.GetGameInstance`)))
      (set `self.RefGI` _asbp_game_instance))
    (:`then_2`
      (for (_array_element _array_index) (`self.ListChallenge`)
        (`/Engine/EditorBlueprintResources/StandardMacros.IsValid` _array_element
          (:`Is Valid`
            (set `/Game/Blueprint/InteractiveObject/BP_MasterChallenge.RefMaster` self _array_element))
          (:`Is Not Valid`
            (`KismetArrayLibrary.Array_Remove` (`self.ListChallenge`) _array_index)
            (`KismetSystemLibrary.PrintText` (`|FormatText` "Challenge {name challenge} not valid in Challenge Manage {challenge manager name}, removing it from the list" (`KismetSystemLibrary.GetDisplayName` _array_element) (`KismetSystemLibrary.GetDisplayName` self)) true true (struct :`R` 1.0 :`B` 0.041236 :`A` 1.0) 10.0)))))))

(event `ChallengeFinished`
  (params (Challenge :type "/Game/Blueprint/InteractiveObject/BP_MasterChallenge Object Reference"))
  (if (`KismetArrayLibrary.Array_Contains` (`self.ListChallenge`) Challenge)
    (bind _result (`/Engine/EditorBlueprintResources/StandardMacros.IncrementInt` (`self.NumberChallengedFinished`))
      (:`  `
        (if (>= _result (`KismetArrayLibrary.Array_Length` (`self.ListChallenge`)))
          (set `self.ErrorChallenge?` false)
          (for _array_element (`self.ListChallenge`)
            (`/Engine/EditorBlueprintResources/StandardMacros.IsValid` _array_element
              (:`Is Valid`
                (if (not (`/Game/Blueprint/InteractiveObject/BP_MasterChallenge.IsCompleted?` _array_element))
                  (`KismetSystemLibrary.PrintString` "One Challenge Isn't finished but should be !!!!" true true (struct :`R` 1.0 :`G` 0.057708 :`A` 1.0) 10.0)
                  (set `self.ErrorChallenge?` true)))
              (:`Is Not Valid`
                (`KismetSystemLibrary.PrintString` "Challenge not valid !!!!" true true (struct :`R` 1.0 :`B` 0.011707 :`A` 1.0) 10.0)
                (set `self.ErrorChallenge?` true))))
          (if (not (`self.ErrorChallenge?`))
            (`self.ActivateInteractiveServer`)
            (`self.CheckGameInstance`
              (:`Valid`
                (`self.CheckGameState`
                  (:`Valid`
                    (for _array_element_2 (`/Game/Blueprint/GameInstance/BP_GameInstance.ListPlayerInfo` (`self.RefGI`))
                      (`/Game/Blueprint/GameState/GS_Master.ActivateInteractiveForChallengeManager` (`self.RefGS`) (`.PC_11_776544A84872013AA63BC881D8B483A2` (break `/Game/Struct/S_PlayerInfo` _array_element_2)) self))))))))))))

(event `ReduceNumberChallengeCompleted`
  (params (Challenge :type "/Game/Blueprint/InteractiveObject/BP_MasterChallenge Object Reference"))
  (bind _numberchallengedfinished (`self.NumberChallengedFinished`))
  (if (`KismetArrayLibrary.Array_Contains` (`self.ListChallenge`) Challenge)
    (`/Engine/EditorBlueprintResources/StandardMacros.DecrementInt` _numberchallengedfinished
      (:`  `
        (if (< _numberchallengedfinished 0)
          (set `self.NumberChallengedFinished` 0))))))

(event `ActivateInteractiveServer`
  (for _array_element (`self.ItemToTrigger`)
    (`/Engine/EditorBlueprintResources/StandardMacros.IsValid` _array_element
      (:`Is Valid`
        (`/Game/Blueprint/InteractiveObject/BP_MasterInteractive.AtActivation` _array_element))
      (:`Is Not Valid`
        (`KismetSystemLibrary.PrintText` (`|FormatText` "Item to trigger {name item} not valid !!!!!" (`KismetSystemLibrary.GetDisplayName` _array_element)) true true (struct :`R` 1.0 :`G` 0.003237 :`A` 1.0) 10.0)))))

(event `ActivateInteractiveClient`
  (for _array_element (`self.ItemToTrigger`)
    (`/Engine/EditorBlueprintResources/StandardMacros.IsValid` _array_element
      (:`Is Valid`
        (`/Game/Blueprint/InteractiveObject/BP_MasterInteractive.AtActivation` _array_element))
      (:`Is Not Valid`
        (`KismetSystemLibrary.PrintText` (`|FormatText` "Item to trigger {name item} not valid !!!!!" (`KismetSystemLibrary.GetDisplayName` _array_element)) true true (struct :`R` 1.0 :`G` 0.007579 :`A` 1.0) 10.0)))))

(fn `UserConstructionScript`)