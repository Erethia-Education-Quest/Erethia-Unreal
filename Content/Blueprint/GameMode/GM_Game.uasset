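; GM_Game is a Game Mode that sets up joining players and can return the session to the lobby.
; It extends the parent login: players of the first type enum value get a BP_Teacher spawned, possessed and written into their player info, replacing any existing pawn at its transform.
; It caches the GS_Game game state for the parent.
; On authority, it runs ServerTravel to the Game Instance's current lobby.
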(fn `CastToGs`
  (params (AlreadyCastGs :type "/Game/Blueprint/GameState/GS_Master Object Reference"))
  (bind _asgs_game (cast `/Game/Blueprint/GameState/GS_Game` (`GameplayStatics.GetGameState`)))
  (bind _output_get (set `self.RefGSGame` _asgs_game))
  (`parent.CastToGs` _output_get))

(fn `Login Player`
  (params (NewPc :type "PlayerController Object Reference"))
  (returns (InfoPlayer :type "/Game/Struct/S_PlayerInfo Structure") (`PC Player` :type "/Game/Blueprint/PlayerController/PC_Master Object Reference"))
  (locals (PlayerInfo :type "/Game/Struct/S_PlayerInfo Structure") (PC :type "/Game/Blueprint/PlayerController/PC_Master Object Reference"))
  (bind (_playerinfo_id _playerinfo_pawn _playerinfo_pc _playerinfo_type) (break `/Game/Struct/S_PlayerInfo` (`local.PlayerInfo`)))
  (bind (_playerinfo_id_2 _playerinfo_pawn_2) (break `/Game/Struct/S_PlayerInfo` (`local.PlayerInfo`)))
  (bind (_playerinfo_id_3 _playerinfo_pawn_3 _playerinfo_pc_2 _playerinfo_type_2) (break `/Game/Struct/S_PlayerInfo` (`local.PlayerInfo`)))
  (bind (_infoplayer _pc_player) (`parent.Login Player` NewPc))
  (set `local.PC` _pc_player)
  (bind _output_get (set `local.PlayerInfo` _infoplayer))
  (if (`|EnumEquality` (`.Type_15_719701CF4B6D9DF664F022817F190116` (break `/Game/Struct/S_PlayerInfo` _output_get)) "NewEnumerator0")
    (`/Engine/EditorBlueprintResources/StandardMacros.IsValid` (`.Pawn_16_F0557B3940946A7D12EB85B39451416E` (break `/Game/Struct/S_PlayerInfo` _output_get))
      (:`Is Valid`
        (bind _returnvalue (`|SpawnActorFromClass` "/Game/Blueprint/Player/BP_Teacher.BP_Teacher_C" (`self.GetTransform` (`.Pawn_16_F0557B3940946A7D12EB85B39451416E` (break `/Game/Struct/S_PlayerInfo` _output_get))) "Undefined" "MultiplyWithRoot" null null))
        (`/Engine/EditorBlueprintResources/StandardMacros.IsValid` _playerinfo_pawn_2
          (:`Is Valid`
            (`self.K2_DestroyActor` _playerinfo_pawn_2))
          (:`Is Not Valid`
            _))
        (`Controller.Possess` (`local.PC`) _returnvalue)
        (set `local.PlayerInfo` (make `/Game/Struct/S_PlayerInfo` _playerinfo_id_3 _returnvalue _playerinfo_pc_2 _playerinfo_type_2)))
      (:`Is Not Valid`
        (bind _returnvalue_2 (`|SpawnActorFromClass` "/Game/Blueprint/Player/BP_Teacher.BP_Teacher_C" (`KismetMathLibrary.MakeTransform` (0.0 0.0 0.0)) "Undefined" "MultiplyWithRoot" null null))
        (`Controller.Possess` (`local.PC`) _returnvalue_2)
        (set `local.PlayerInfo` (make `/Game/Struct/S_PlayerInfo` _playerinfo_id _returnvalue_2 _playerinfo_pc _playerinfo_type))))
    (return (`local.PlayerInfo`) (`local.PC`))
    (else
      (return (`local.PlayerInfo`) (`local.PC`)))))

(fn `SendAllPlayerToLobby`
  (if (`self.HasAuthority`)
    (bind _refgi (`self.RefGI`)
      (:`then`
        (`KismetSystemLibrary.ExecuteConsoleCommand` (`KismetTextLibrary.Conv_TextToString` (`|FormatText` "ServerTravel {lobby}" (`/Game/Blueprint/GameInstance/BP_GameInstance.CurrentLobby` _refgi))) null))
      (:`else`))))

(fn `UserConstructionScript`
  (`parent.UserConstructionScript`))