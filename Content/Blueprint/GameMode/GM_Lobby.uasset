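; Lobby game mode that relays buzzer presses to the lobby's players through the game state.
; ButtonPressed loops over the player info list in the game instance, casts each controller to PC_Lobby and calls ButtonPressedClient on GS_Lobby with that controller and the buzzer.
; The CastToGs override caches the game state as GS_Lobby, then passes it to the parent implementation.
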(event `/Game/Blueprint/Interface/GameMode/BPI_GMLobby.ButtonPressed`
  (params (BuzzerPressed :type "/Game/Blueprint/InteractiveObject/BuzzerLobby/BP_BuzzerLobby Object Reference"))
  (for _array_element (`/Game/Blueprint/GameInstance/BP_GameInstance.ListPlayerInfo` (`self.RefGI`))
    (bind _aspc_lobby (cast `/Game/Blueprint/PlayerController/PC_Lobby` (`.PC_11_776544A84872013AA63BC881D8B483A2` (break `/Game/Struct/S_PlayerInfo` _array_element))))
    (`/Game/Blueprint/GameState/GS_Lobby.ButtonPressedClient` (`self.RefGsLobby`) _aspc_lobby BuzzerPressed)))

(fn `CastToGs`
  (params (AlreadyCastGs :type "/Game/Blueprint/GameState/GS_Master Object Reference"))
  (bind _asgs_lobby (cast `/Game/Blueprint/GameState/GS_Lobby` (`GameplayStatics.GetGameState`)))
  (bind _output_get (set `self.RefGsLobby` _asgs_lobby))
  (`parent.CastToGs` _output_get))

(fn `UserConstructionScript`
  (`parent.UserConstructionScript`))