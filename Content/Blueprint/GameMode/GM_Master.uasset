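; Master multiplayer Game Mode that registers connecting players on the server and handles disconnecting one or all of them.
; Outside standalone, a looping timer polls for new PlayerControllers instead of using PostLogin, gating logins one at a time with DoOnce.
; Login possesses the BP_Player pawn, restores or allocates an ID, and stores player info in BP_GameInstance.
; GS_Master relays the player list and newcomer info to clients and executes disconnections.
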(event `self.ReceiveBeginPlay`
  (`|ExecutionSequence`
    (:`then_0`
      (`self.CastToGs` null))
    (:`then_1`
      (bind _asbp_game_instance (cast `/Game/Blueprint/GameInstance/BP_GameInstance` (`GameplayStatics.GetGameInstance`)))
      (set `self.RefGI` _asbp_game_instance))
    (:`then_2`
      (set `self.IsInitialized?` true)
      (if (and (`self.HasAuthority`) (not (`KismetSystemLibrary.IsStandalone`)))
        (`/Engine/EditorBlueprintResources/StandardMacros.DoOnce` false
          (:`Completed`
            (`KismetSystemLibrary.K2_SetTimerDelegate` (delegate `CheckNewClient`) 0.1 true)))))))

(event `CheckNewClient`
  (bind _playertoprocess (`self.PlayerToProcess`))
  (bind _outactors (`GameplayStatics.GetAllActorsOfClass` "/Script/Engine.PlayerController"))
  (`/Engine/EditorBlueprintResources/StandardMacros.IsValid` (`self.PlayerToProcess`)
    (:`Is Not Valid`
      (for _array_element _outactors :!label _label
        (if (and (not (`KismetArrayLibrary.Array_Contains` (`self.Pc Brut Already Connected`) _array_element)) (not (`KismetSystemLibrary.IsValid` (`self.PlayerToProcess`))))
          (set `self.PlayerToProcess` _array_element)
          (goto _label)))
      (`/Engine/EditorBlueprintResources/StandardMacros.IsValid` (`self.PlayerToProcess`)
        (:`Is Valid`
          (`/Engine/EditorBlueprintResources/StandardMacros.DoOnce` false :!label _label_2
            (:`Completed`
              (`KismetSystemLibrary.Delay` 0.2)
              (`self.Login Player` _playertoprocess)
              (`KismetArrayLibrary.Array_AddUnique` (`self.Pc Brut Already Connected`) _playertoprocess)
              (set `self.PlayerToProcess` null)
              (`self.ResetLogin`))))))))

(event `ResetLogin`
  (goto _label_2 :!via `Reset`))

(event `DisconnectAllPlayers`
  (`self.DisconnectClients`))

(event `Disconnect Specific Player`
  (params (ID :type Integer))
  (bind _refgi (`self.RefGI`)
    (:`then`
      (bind (_playerinfo _valid_) (`/Game/Blueprint/GameInstance/BP_GameInstance.GetSpecificID` _refgi ID))
      (if _valid_
        (bind (_id _pawn _pc) (break `/Game/Struct/S_PlayerInfo` _playerinfo))
        (`KismetArrayLibrary.Array_RemoveItem` (`/Game/Blueprint/GameInstance/BP_GameInstance.ListUsedID` _refgi) _id)
        (`/Game/Blueprint/GameState/GS_Master.DisconnectPlayerClient` (`self.RefGSMaster`) _pc)
        (`KismetArrayLibrary.Array_RemoveItem` (`/Game/Blueprint/GameInstance/BP_GameInstance.ListPlayerInfo` _refgi) _playerinfo)))
    (:`else`)))

(fn `AddPlayerInfoToGI`
  (params (PlayerInfo :type "/Game/Struct/S_PlayerInfo Structure"))
  (`KismetArrayLibrary.Array_AddUnique` (`/Game/Blueprint/GameInstance/BP_GameInstance.ListPlayerInfo` (`self.RefGI`)) PlayerInfo))

(fn `CastPc`
  (params (NewPc :type "PlayerController Object Reference"))
  (returns (Pc :type "/Game/Blueprint/PlayerController/PC_Master Object Reference"))
  (bind _aspc_master (cast `/Game/Blueprint/PlayerController/PC_Master` NewPc))
  (return _aspc_master))

(fn `CastToGs`
  (params (AlreadyCastGs :type "/Game/Blueprint/GameState/GS_Master Object Reference"))
  (`/Engine/EditorBlueprintResources/StandardMacros.IsValid` AlreadyCastGs
    (:`Is Valid`
      (set `self.RefGSMaster` AlreadyCastGs))
    (:`Is Not Valid`
      (bind _asgs_master (cast `/Game/Blueprint/GameState/GS_Master` (`GameplayStatics.GetGameState`)))
      (set `self.RefGSMaster` _asgs_master))))

(fn `DisconnectClients`
  (locals (ServerOwner :type "/Game/Blueprint/PlayerController/PC_Master Object Reference"))
  (for _array_element (`/Game/Blueprint/GameInstance/BP_GameInstance.ListPlayerInfo` (`self.RefGI`))
    (if (`self.HasAuthority` (`.PC_11_776544A84872013AA63BC881D8B483A2` (break `/Game/Struct/S_PlayerInfo` _array_element)))
      (`/Game/Blueprint/GameState/GS_Master.DisconnectPlayerClient` (`self.RefGSMaster`) (`.PC_11_776544A84872013AA63BC881D8B483A2` (break `/Game/Struct/S_PlayerInfo` _array_element)))
      (else
        (set `local.ServerOwner` (`.PC_11_776544A84872013AA63BC881D8B483A2` (break `/Game/Struct/S_PlayerInfo` _array_element))))))
  (`/Game/Blueprint/GameState/GS_Master.DisconnectPlayerServer` (`self.RefGSMaster`) (`local.ServerOwner`)))

(fn `Login Player`
  (params (NewPc :type "PlayerController Object Reference"))
  (returns (InfoPlayer :type "/Game/Struct/S_PlayerInfo Structure") (`PC Player` :type "/Game/Blueprint/PlayerController/PC_Master Object Reference"))
  (locals (Pc :type "/Game/Blueprint/PlayerController/PC_Master Object Reference") (Player :type "/Game/Blueprint/Player/BP_Player Object Reference") (NewPlayerInfo :type "/Game/Struct/S_PlayerInfo Structure"))
  (bind _pc (`self.CastPc` NewPc))
  (`/Engine/EditorBlueprintResources/StandardMacros.IsValid` _pc
    (:`Is Valid`
      (bind _output_get (set `local.Pc` _pc))
      (bind _asbp_player (cast `/Game/Blueprint/Player/BP_Player` (`Controller.K2_GetPawn` _output_get)))
      (set `local.Player` _asbp_player)
      (if (`/Game/Blueprint/Player/BP_Player.IsInitialized?` _asbp_player)
        (`Controller.Possess` (`local.Pc`) (`local.Player`))
        (bind _playerinfo (`self.Retrieve Previous Informations` (`local.Pc`)))
        (`self.RemovePlayerFromGI` (break `/Game/Struct/S_PlayerInfo` _playerinfo))
        (bind _output_get_2 (set `local.NewPlayerInfo` (make `/Game/Struct/S_PlayerInfo` (break `/Game/Struct/S_PlayerInfo` _playerinfo) (`local.Player`) (`local.Pc`) (`.Type_15_719701CF4B6D9DF664F022817F190116` (break `/Game/Struct/S_PlayerInfo` _playerinfo)))))
        (`self.AddPlayerInfoToGI` _output_get_2)
        (`self.SendAllInformationAtNewPlayer` (`local.Pc`) (`local.NewPlayerInfo`))
        (`self.SendNewPlayerInfoToAllPlayersAlreadyConnected` (`local.NewPlayerInfo`))
        (return (`local.NewPlayerInfo`) (`local.Pc`))))
    (:`Is Not Valid`
      (`KismetSystemLibrary.PrintString` "Pc Casted Not Valid (Login Player)" true true (struct :`R` 1.0 :`G` 0.016718 :`A` 1.0) 10.0))))

(fn `RemovePlayerFromGI`
  (params (IDToRemove :type Integer))
  (bind _refgi (`self.RefGI`))
  (bind _playerinfo (`/Game/Blueprint/GameInstance/BP_GameInstance.GetSpecificID` _refgi IDToRemove))
  (`KismetArrayLibrary.Array_RemoveItem` (`/Game/Blueprint/GameInstance/BP_GameInstance.ListPlayerInfo` _refgi) _playerinfo))

(fn `Retrieve Previous Informations`
  (params (NewPc :type "/Game/Blueprint/PlayerController/PC_Master Object Reference"))
  (returns (PlayerInfo :type "/Game/Struct/S_PlayerInfo Structure"))
  (locals (`IDFound?` :type Boolean) (CurrentIDLookedAt :type Integer))
  (bind _id (`/Game/Blueprint/PlayerController/PC_Master.ID` NewPc))
  (bind _currentidlookedat (`local.CurrentIDLookedAt`))
  (if (>= _id 0)
    (bind _playerinfo (`/Game/Blueprint/GameInstance/BP_GameInstance.GetSpecificID` (`self.RefGI`) _id))
    (return _playerinfo)
    (else
      (while (not (`local.IDFound?`))
        (if (`KismetArrayLibrary.Array_Contains` (`/Game/Blueprint/GameInstance/BP_GameInstance.ListUsedID` (`self.RefGI`)) (`local.CurrentIDLookedAt`))
          (`/Engine/EditorBlueprintResources/StandardMacros.IncrementInt` (`local.CurrentIDLookedAt`))
          (else
            (set `local.IDFound?` true))))
      (`KismetArrayLibrary.Array_AddUnique` (`/Game/Blueprint/GameInstance/BP_GameInstance.ListUsedID` (`self.RefGI`)) _currentidlookedat)
      (return (make `/Game/Struct/S_PlayerInfo` _currentidlookedat null null "NewEnumerator1")))))

(fn `SendAllInformationAtNewPlayer`
  (params (Pc :type "/Game/Blueprint/PlayerController/PC_Master Object Reference") (PlayerInfo :type "/Game/Struct/S_PlayerInfo Structure"))
  (`/Game/Blueprint/GameState/GS_Master.NewPlayerInfo` (`self.RefGSMaster`) (`local.Pc`) PlayerInfo)
  (`/Game/Blueprint/GameState/GS_Master.NewListOfAllPlayerInfo` (`self.RefGSMaster`) (`local.Pc`) (`/Game/Blueprint/GameInstance/BP_GameInstance.ListPlayerInfo` (`self.RefGI`))))

(fn `SendNewPlayerInfoToAllPlayersAlreadyConnected`
  (params (PlayerInfo :type "/Game/Struct/S_PlayerInfo Structure"))
  (bind _playerinfo_id (break `/Game/Struct/S_PlayerInfo` (`local.PlayerInfo`)))
  (for _array_element (`/Game/Blueprint/GameInstance/BP_GameInstance.ListPlayerInfo` (`self.RefGI`))
    (if (!= (break `/Game/Struct/S_PlayerInfo` _array_element) _playerinfo_id)
      (`/Game/Blueprint/GameState/GS_Master.SetupNewPlayer` (`self.RefGSMaster`) (`.PC_11_776544A84872013AA63BC881D8B483A2` (break `/Game/Struct/S_PlayerInfo` _array_element)) (`local.PlayerInfo`)))))

(fn `UserConstructionScript`)