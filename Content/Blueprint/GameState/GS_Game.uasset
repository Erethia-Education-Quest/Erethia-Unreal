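; GS_Game is the game state Blueprint that relays puzzle and sound actions to a given PC, likely a player controller.
; Its events cover grabbing statuettes, snapping fresco pieces, turning statues, moving and selecting pillars, and managing player sound queues.
; Each checks that the PC is valid, then calls its same-named Client event with the same arguments, holding no logic or state of its own.
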(event `GrabItemClient`
  (params (PC :type "/Game/Blueprint/PlayerController/PC_Game Object Reference") (Piedestal :type "/Game/Blueprint/InteractiveObject/Piedestal/BP_Piedestal Object Reference") (Statuette :type "/Game/Blueprint/InteractiveObject/Gabable_OBJ/Statue/BP_MasterPuzzleStatue Object Reference"))
  (`/Engine/EditorBlueprintResources/StandardMacros.IsValid` PC
    (:`Is Valid`
      (`/Game/Blueprint/PlayerController/PC_Game.GrabItemClient` PC Piedestal Statuette))))

(event `ReleaseAndSnapObjectClient`
  (params (PC :type "/Game/Blueprint/PlayerController/PC_Game Object Reference") (FrescoPiece :type "Actor Object Reference") (SnapPosition :type "StaticMeshComponent Object Reference") (FullFresco :type "/Game/AssetsErethia/objects/fresco/fresco01/BP_fresco01_incomplete Object Reference"))
  (`/Engine/EditorBlueprintResources/StandardMacros.IsValid` PC
    (:`Is Valid`
      (`/Game/Blueprint/PlayerController/PC_Game.ReleaseAndSnapObjectClient` PC FrescoPiece FullFresco SnapPosition))))

(event `ReleaseAndSnapObjectClient2`
  (params (PC :type "/Game/Blueprint/PlayerController/PC_Game Object Reference") (FrescoPiece :type "Actor Object Reference") (SnapPosition :type "StaticMeshComponent Object Reference") (FullFresco :type "/Game/AssetsErethia/objects/fresco/fresco02/BP_fresco02_incomplete Object Reference"))
  (`/Engine/EditorBlueprintResources/StandardMacros.IsValid` PC
    (:`Is Valid`
      (`/Game/Blueprint/PlayerController/PC_Game.ReleaseAndSnapObjectClient2` PC FrescoPiece FullFresco SnapPosition))))

(event `TurnStatueClient`
  (params (PC :type "/Game/Blueprint/PlayerController/PC_Game Object Reference") (CentralStatue :type "/Game/Blueprint/InteractiveObject/Statue/BP_CentralStatue Object Reference"))
  (`/Engine/EditorBlueprintResources/StandardMacros.IsValid` PC
    (:`Is Valid`
      (`/Game/Blueprint/PlayerController/PC_Game.TurnStatueClient` PC CentralStatue))))

(event `ClearSoundClient`
  (params (PC :type "/Game/Blueprint/PlayerController/PC_Game Object Reference") (PlayerSound :type "/Game/Blueprint/InteractiveObject/Sound/BP_PlayAllSound Object Reference"))
  (`/Engine/EditorBlueprintResources/StandardMacros.IsValid` PC
    (:`Is Valid`
      (`/Game/Blueprint/PlayerController/PC_Game.ClearSoundClient` PC PlayerSound))))

(event `StopSoundClient`
  (params (PC :type "/Game/Blueprint/PlayerController/PC_Game Object Reference") (PlayerSound :type "/Game/Blueprint/InteractiveObject/Sound/BP_PlayAllSound Object Reference"))
  (`/Engine/EditorBlueprintResources/StandardMacros.IsValid` PC
    (:`Is Valid`
      (`/Game/Blueprint/PlayerController/PC_Game.StopSoundClient` PC PlayerSound))))

(event `AddSoundToListClient`
  (params (PC :type "/Game/Blueprint/PlayerController/PC_Game Object Reference") (PlayerSound :type "/Game/Blueprint/InteractiveObject/Sound/BP_PlayAllSound Object Reference") (NewSound :type "SoundBase Object Reference") (ForcePlay :type Boolean))
  (`/Engine/EditorBlueprintResources/StandardMacros.IsValid` PC
    (:`Is Valid`
      (`/Game/Blueprint/PlayerController/PC_Game.AddSoundToListClient` PC PlayerSound NewSound ForcePlay))))

(event `MovePilarClient`
  (params (PC :type "/Game/Blueprint/PlayerController/PC_Game Object Reference") (Pilar :type "/Game/Blueprint/InteractiveObject/Pilar/NewPilar/BP_NewPilar Object Reference") (AllTargetLocation :type "Array of Vector2D Structure"))
  (`/Engine/EditorBlueprintResources/StandardMacros.IsValid` PC
    (:`Is Valid`
      (`/Game/Blueprint/PlayerController/PC_Game.MovePilarClient` PC Pilar AllTargetLocation))))

(event `SelectedPilarClient`
  (params (PC :type "/Game/Blueprint/PlayerController/PC_Game Object Reference") (Pilar :type "/Game/Blueprint/InteractiveObject/Pilar/NewPilar/BP_NewPilar Object Reference"))
  (`/Engine/EditorBlueprintResources/StandardMacros.IsValid` PC
    (:`Is Valid`
      (`/Game/Blueprint/PlayerController/PC_Game.SelectedPilarClient` PC Pilar))))

(event `UnselectedPilarClient`
  (params (PC :type "/Game/Blueprint/PlayerController/PC_Game Object Reference") (Pilar :type "/Game/Blueprint/InteractiveObject/Pilar/NewPilar/BP_NewPilar Object Reference"))
  (`/Engine/EditorBlueprintResources/StandardMacros.IsValid` PC
    (:`Is Valid`
      (`/Game/Blueprint/PlayerController/PC_Game.UnselectedPilarClient` PC Pilar))))

(fn `UserConstructionScript`
  (`parent.UserConstructionScript`))