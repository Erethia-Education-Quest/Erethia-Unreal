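; Master GameState that acts as a relay hub, passing multiplayer game events on to a specified player controller.
; Each custom event checks the controller is valid, then calls its same-named event with the same data, holding no logic or state of its own.
; Relayed events cover player info and setup, disconnects, VR hand grab and grip, object transforms, pressure plates, doors, challenge interactives and widget board updates.
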(event `NewPlayerInfo`
  (params (PC :type "/Game/Blueprint/PlayerController/PC_Master Object Reference") (PlayerInfo :type "/Game/Struct/S_PlayerInfo Structure"))
  (`/Engine/EditorBlueprintResources/StandardMacros.IsValid` PC
    (:`Is Valid`
      (`/Game/Blueprint/PlayerController/PC_Master.NewPlayerInfo` PC PlayerInfo))))

(event `NewListOfAllPlayerInfo`
  (params (PC :type "/Game/Blueprint/PlayerController/PC_Master Object Reference") (ListPlayerInfo :type "Array of /Game/Struct/S_PlayerInfo Structure"))
  (`/Engine/EditorBlueprintResources/StandardMacros.IsValid` PC
    (:`Is Valid`
      (`/Game/Blueprint/PlayerController/PC_Master.NewListOfAllPlayerInfo` PC ListPlayerInfo))))

(event `SetupNewPlayer`
  (params (PC :type "/Game/Blueprint/PlayerController/PC_Master Object Reference") (PlayerInfo :type "/Game/Struct/S_PlayerInfo Structure"))
  (`/Engine/EditorBlueprintResources/StandardMacros.IsValid` PC
    (:`Is Valid`
      (`/Game/Blueprint/PlayerController/PC_Master.SetupNewPlayer` PC PlayerInfo))))

(event `GrabClient`
  (params (PC :type "/Game/Blueprint/PlayerController/PC_Master Object Reference") (Pawn :type "/Game/Blueprint/Player/BP_Player Object Reference") (Component :type "/Game/VRTemplate/Blueprints/GrabComponent Object Reference") (Hand :type "/Game/Enum/E_KeyboardControlTypes Enum" :default "NewEnumerator0"))
  (`/Engine/EditorBlueprintResources/StandardMacros.IsValid` PC
    (:`Is Valid`
      (`/Game/Blueprint/PlayerController/PC_Master.GrabClient` PC Pawn Component Hand))))

(event `ReleaseClient`
  (params (PC :type "/Game/Blueprint/PlayerController/PC_Master Object Reference") (Pawn :type "/Game/Blueprint/Player/BP_Player Object Reference") (Hand :type "/Game/Enum/E_KeyboardControlTypes Enum" :default "NewEnumerator0"))
  (`/Engine/EditorBlueprintResources/StandardMacros.IsValid` PC
    (:`Is Valid`
      (`/Game/Blueprint/PlayerController/PC_Master.ReleaseClient` PC Pawn Hand))))

(event `ActivateInteractiveForChallengeManager`
  (params (PC :type "/Game/Blueprint/PlayerController/PC_Master Object Reference") (Manager :type "/Game/Blueprint/Challenge/BP_ChallengeManager Object Reference"))
  (`/Engine/EditorBlueprintResources/StandardMacros.IsValid` PC
    (:`Is Valid`
      (`/Game/Blueprint/PlayerController/PC_Master.ActivateInteractiveForChallengeManager` PC Manager))))

(event `PressPlateClient`
  (params (PC :type "/Game/Blueprint/PlayerController/PC_Master Object Reference") (PressurePlate :type "/Game/Blueprint/InteractiveObject/PressurePlate/PressurePlate Object Reference"))
  (`/Engine/EditorBlueprintResources/StandardMacros.IsValid` PC
    (:`Is Valid`
      (`/Game/Blueprint/PlayerController/PC_Master.PressPLateClient` PC PressurePlate))))

(event `UnpressPlateClient`
  (params (PC :type "/Game/Blueprint/PlayerController/PC_Master Object Reference") (PressurePlate :type "/Game/Blueprint/InteractiveObject/PressurePlate/PressurePlate Object Reference"))
  (`/Engine/EditorBlueprintResources/StandardMacros.IsValid` PC
    (:`Is Valid`
      (`/Game/Blueprint/PlayerController/PC_Master.UnpressPlateClient` PC PressurePlate))))

(event `MoveDoorClient`
  (params (PC :type "/Game/Blueprint/PlayerController/PC_Master Object Reference") (Door :type "/Game/Blueprint/InteractiveObject/Door/BP_DoorLeftRight Object Reference"))
  (`/Engine/EditorBlueprintResources/StandardMacros.IsValid` PC
    (:`Is Valid`
      (`/Game/Blueprint/PlayerController/PC_Master.MoveDoorClient` PC Door))))

(event `DisconnectPlayerClient`
  (params (PC :type "/Game/Blueprint/PlayerController/PC_Master Object Reference"))
  (`/Engine/EditorBlueprintResources/StandardMacros.IsValid` PC
    (:`Is Valid`
      (`/Game/Blueprint/PlayerController/PC_Master.DisconnectPlayerClient` PC))))

(event `DisconnectPlayerServer`
  (params (PC :type "/Game/Blueprint/PlayerController/PC_Master Object Reference"))
  (`/Engine/EditorBlueprintResources/StandardMacros.IsValid` PC
    (:`Is Valid`
      (`/Game/Blueprint/PlayerController/PC_Master.DisconnectPlayerServer` PC))))

(event `UpdateWidgetClient`
  (params (PC :type "/Game/Blueprint/PlayerController/PC_Master Object Reference") (WidgetManager :type "/Game/Blueprint/Widget/Menu/LobbyMenu/BP_ListPlayersManager Object Reference") (PlayerToAdd :type "Array of Text") (PlayerToRemove :type "Array of Text"))
  (`/Engine/EditorBlueprintResources/StandardMacros.IsValid` PC
    (:`Is Valid`
      (`/Game/Blueprint/PlayerController/PC_Master.UpdateWidgetClient` PC WidgetManager PlayerToAdd PlayerToRemove))))

(event `CheckupBoardIsUpdatedClient`
  (params (PC :type "/Game/Blueprint/PlayerController/PC_Master Object Reference") (WidgetManager :type "/Game/Blueprint/Widget/Menu/LobbyMenu/BP_ListPlayersManager Object Reference") (AllPlayers :type "Array of Text"))
  (`/Engine/EditorBlueprintResources/StandardMacros.IsValid` PC
    (:`Is Valid`
      (`/Game/Blueprint/PlayerController/PC_Master.CheckupBoardIsUpdatedClient` PC WidgetManager AllPlayers))))

(event `UpdateControllerGripClient`
  (params (PC :type "/Game/Blueprint/PlayerController/PC_Master Object Reference") (Player :type "/Game/Blueprint/Player/BP_Player Object Reference") (MotionController :type "MotionControllerComponent Object Reference") (Controller :type "/Game/Enum/E_KeyboardControlTypes Enum" :default "NewEnumerator0"))
  (`/Engine/EditorBlueprintResources/StandardMacros.IsValid` PC
    (:`Is Valid`
      (`/Game/Blueprint/PlayerController/PC_Master.UpdateControllerGripClient` PC Player MotionController Controller))))

(event `SetTransformObjectClient`
  (params (PC :type "/Game/Blueprint/PlayerController/PC_Master Object Reference") (Object :type "/Game/Blueprint/InteractiveObject/BP_MasterInteractive Object Reference") (ObjectTransform :type "Transform Structure"))
  (`/Engine/EditorBlueprintResources/StandardMacros.IsValid` PC
    (:`Is Valid`
      (`/Game/Blueprint/PlayerController/PC_Master.SetTransformObjectClient` PC Object ObjectTransform))))

(event `UpdateGrabblePosition`
  (params (PC :type "/Game/Blueprint/PlayerController/PC_Master Object Reference") (Object :type "/Game/Blueprint/InteractiveObject/Gabable_OBJ/BP_MasterGrabbableObjects Object Reference") (Location :type "Vector Structure") (Rotation :type "Rotator Structure"))
  (`/Engine/EditorBlueprintResources/StandardMacros.IsValid` PC
    (:`Is Valid`
      (`/Game/Blueprint/PlayerController/PC_Game.UpdateGrabblePosition` PC Object Location Rotation))))

(fn `UserConstructionScript`)