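; BP_MasterChallenge is an interactive-object challenge that tracks whether it is completed and reports changes to a referenced master object.
; ChangeCompleteState acts only when the value differs, storing it in IsCompleted.
; If RefMaster is valid, it calls ChallengeFinished on completion or ReduceNumberChallengeCompleted on reversal, passing itself.
; The event graph and construction script hold no logic.
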(fn `ChangeCompleteState`
  (params (NewValue :type Boolean))
  (if (!= NewValue (`self.IsCompleted?`))
    (bind _output_get (set `self.IsCompleted?` NewValue))
    (`/Engine/EditorBlueprintResources/StandardMacros.IsValid` (`self.RefMaster`)
      (:`Is Valid`
        (if _output_get
          (`/Game/Blueprint/Challenge/BP_ChallengeManager.ChallengeFinished` (`self.RefMaster`) self)
          (else
            (`/Game/Blueprint/Challenge/BP_ChallengeManager.ReduceNumberChallengeCompleted` (`self.RefMaster`) self)))))))

(fn `UserConstructionScript`)