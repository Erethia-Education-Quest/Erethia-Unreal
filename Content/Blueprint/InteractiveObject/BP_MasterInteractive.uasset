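; Base Blueprint for networked interactive objects, handling transform sync, highlighting and audio.
; On authority, a looping five-second timer sends the actor transform through GS_Master to each player in the GameInstance's list, and client events apply it by teleport.
; Highlight events set custom depth stencil values for normal, in-range and grabbed states.
; Activation on authority clears queued voice sounds and adds its own, while separate events play and stop an attached object sound.
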(event `self.ReceiveBeginPlay`
  (`|ExecutionSequence`
    (:`then_0`
      (bind _asbp_game_instance (cast `/Game/Blueprint/GameInstance/BP_GameInstance` (`GameplayStatics.GetGameInstance`)))
      (set `self.RefGI` _asbp_game_instance))
    (:`then_1`
      (bind _asgs_master (cast `/Game/Blueprint/GameState/GS_Master` (`GameplayStatics.GetGameState`)))
      (set `self.RefGS` _asgs_master))
    (:`then_2`
      (set `self.CurrentTransform` (`self.GetTransform`))
      (`/Engine/EditorBlueprintResources/ActorMacros.Switch Has Authority`
        (:`Authority`
          (`KismetSystemLibrary.K2_SetTimerDelegate` (delegate `UpdateTransformObject`) 5.0 true))))))

(event `UpdateTransformObject`
  (`/Engine/EditorBlueprintResources/ActorMacros.Switch Has Authority`
    (:`Authority`
      (`self.SetTransformObjectServer`))))

(event `SetTransformObjectServer`
  (set `self.CurrentTransform` (`self.GetTransform`))
  (`/Engine/EditorBlueprintResources/StandardMacros.IsValid` (`self.RefGS`)
    (:`Is Valid`
      (bind _refgi (`self.RefGI`)
        (:`then`
          (for _array_element (`/Game/Blueprint/GameInstance/BP_GameInstance.ListPlayerInfo` _refgi)
            (`/Game/Blueprint/GameState/GS_Master.SetTransformObjectClient` (`self.RefGS`) (`.PC_11_776544A84872013AA63BC881D8B483A2` (break `/Game/Struct/S_PlayerInfo` _array_element)) self (`self.CurrentTransform`))))
        (:`else`)))))

(event `SetTransformObjectClient`
  (params (ObjectTransform :type "Transform Structure"))
  (`self.K2_SetActorTransform` ObjectTransform false true))

(event `StopAllVoiceSound`
  (for _array_element (`self.SoundPlayerStop`)
    (`/Game/Blueprint/InteractiveObject/Sound/BP_PlayAllSound.ClearSound` _array_element)))

(event `AtActivation`
  (bind _voicesound (`self.VoiceSound`))
  (`/Engine/EditorBlueprintResources/ActorMacros.Switch Has Authority`
    (:`Authority`
      (`/Engine/EditorBlueprintResources/StandardMacros.IsValid` _voicesound
        (:`Is Valid`
          (`self.StopAllVoiceSound`)
          (`/Game/Blueprint/InteractiveObject/Sound/BP_PlayAllSound.AddSoundToList` (`self.SoundPlayer`) _voicesound (`self.ForcePlaySound`)))))))

(event `Debug`
  (params (text1 :type String) (text2 :type String) (text3 :type String) (text4 :type String) (bool :type Boolean) (int :type Integer) (OBJ_Name :type Name)))

(event `ChangeHighlightObjectClient`
  (params (Highlight :type "/Game/Enum/E_HighlightTypes Enum" :default "NewEnumerator0"))
  (`PrimitiveComponent.SetCustomDepthStencilValue` (`self.Object`) (select `/Game/Enum/E_HighlightTypes` Highlight :`NewEnumerator1` 1 :`NewEnumerator2` 2)))

(event `ChangeHighlightObjectServer`
  (params (Highlight :type "/Game/Enum/E_HighlightTypes Enum" :default "NewEnumerator0"))
  (`PrimitiveComponent.SetCustomDepthStencilValue` (`self.Object`) (select `/Game/Enum/E_HighlightTypes` Highlight :`NewEnumerator1` 1 :`NewEnumerator2` 2)))

(event `StopSound`
  (bind _playsoundref (`self.PlaySoundRef`))
  (`/Engine/EditorBlueprintResources/StandardMacros.IsValid` _playsoundref
    (:`Is Valid`
      (`AudioComponent.Stop` _playsoundref))))

(event `PlayOBJSound`
  (params (object :type "SceneComponent Object Reference"))
  (`/Engine/EditorBlueprintResources/StandardMacros.IsValid` object
    (:`Is Valid`
      (bind _returnvalue (`GameplayStatics.SpawnSoundAttached` (`self.OBJSound`) object "None" (0.0 0.0 0.0) (struct) "KeepRelativeOffset" true 0.01 1.0 0.0 "/Game/Blueprint/InteractiveObject/Sound/SoundAttenuation/BP_SoundAttenuationOBJ.BP_SoundAttenuationOBJ" null))
      (set `self.PlaySoundRef` _returnvalue))))

(fn `UserConstructionScript`)