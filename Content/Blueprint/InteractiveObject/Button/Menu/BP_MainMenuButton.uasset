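; BP_MainMenuButton is a main menu button, built on a parent interactive object, that animates the height of its Object component.
; On BeginPlay, a FlyTimeline drives the local Z offset as a floating motion.
; Pressed plays a PressedTimeline on the same offset, with an IsBeingPressed flag suppressing the float updates until the press animation finishes.
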(event `self.ReceiveBeginPlay`
  (`parent.ReceiveBeginPlay`)
  (bind (_direction _height) (`Timeline|FlyTimeline`)
    (:`Update`
      (if (not (`self.IsBeingPressed?`))
        (`SceneComponent.K2_SetRelativeLocation` (`self.Object`) (`KismetMathLibrary.MakeVector` 0.0 0.0 _height) false false)))))

(event `Pressed`
  (set `self.IsBeingPressed?` true)
  (bind (_direction _height) (`Timeline|PressedTimeline`)
    (:`Update`
      (`SceneComponent.K2_SetRelativeLocation` (`self.Object`) (`KismetMathLibrary.MakeVector` 0.0 0.0 _height) false false))
    (:`Finished`
      (set `self.IsBeingPressed?` false))))

(fn `UserConstructionScript`
  (`parent.UserConstructionScript`))