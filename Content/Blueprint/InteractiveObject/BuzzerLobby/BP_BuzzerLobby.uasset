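; BP_BuzzerLobby is a lobby buzzer that sends the server to L_MainLevel when pressed by hand.
; On authority, overlap by a "Hand"-tagged component from one specific player type fires ButtonPressedServer and notifies the game mode.
; That event issues ServerTravel, then plays a timeline subtracting its Z value from the button's current height each update.
; ButtonPressedClient replays the timeline but is not called here; an L_TestTheo travel command is unused.
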(event `self.Object.OnComponentBeginOverlap`
  (params (OverlappedComponent :type "PrimitiveComponent Object Reference") (OtherActor :type "Actor Object Reference") (OtherComp :type "PrimitiveComponent Object Reference") (OtherBodyIndex :type Integer) (bFromSweep :type Boolean) (SweepResult :type "HitResult Structure (by ref)"))
  (if (and (`ActorComponent.ComponentHasTag` OtherComp "Hand") (`self.HasAuthority`))
    (bind _type (message `/Game/Blueprint/Interface/Players/BPI_PlayerInterface.GetPlayerType` OtherActor))
    (if (`|EnumEquality` _type "NewEnumerator0")
      (`self.ButtonPressedServer`)
      (message `/Game/Blueprint/Interface/GameMode/BPI_GMLobby.ButtonPressed` (`GameplayStatics.GetGameMode`) self))))

(event `ButtonPressedServer`
  (bind _object (`self.Object`))
  (bind _returnvalue (`SceneComponent.GetRelativeTransform` _object))
  (`|ExecutionSequence`
    (:`then_0`
      (`KismetSystemLibrary.ExecuteConsoleCommand` "ServerTravel L_MainLevel" null))
    (:`then_1`
      (bind (_direction _z) (`Timeline|ButtonPressedTimeline` :!via `PlayFromStart` :!label _label)
        (:`Update`
          (`SceneComponent.K2_SetRelativeLocation` _object (`KismetMathLibrary.MakeVector` (.x (.location _returnvalue)) (.y (.location _returnvalue)) (- (.z (.location _returnvalue)) _z)) false false))))))

(event `ButtonPressedClient`
  (goto _label :!via `PlayFromStart`))

(fn `UserConstructionScript`
  (`parent.UserConstructionScript`))