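; Interactive calculator actor operated by touch, where components tagged "hand" press digit, operator, equals and clear keys through box overlaps.
; Digit keys append to the selected operand, NB1 or NB2, and ChangeText shows that operand on TextDisplay.
; Operator keys switch entry to NB2 or chain the pending operation through Calculator, which stores the result in NB1.
; The construction script labels each key with its component's object name.
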(event `self.ReceiveBeginPlay`
  (`TextRenderComponent.K2_SetText` (`self.TextDisplay`) (`KismetTextLibrary.Conv_DoubleToText` (`self.NB1`) "HalfToEven")))

(event `self.Box_0.OnComponentBeginOverlap`
  (params (OverlappedComponent :type "PrimitiveComponent Object Reference") (OtherActor :type "Actor Object Reference") (OtherComp :type "PrimitiveComponent Object Reference") (OtherBodyIndex :type Integer) (bFromSweep :type Boolean) (SweepResult :type "HitResult Structure (by ref)"))
  (if (`ActorComponent.ComponentHasTag` OtherComp "hand")
    (if (`self.NBSelectedIs1`)
      (bind _newnb (`self.ConstructNB` 1 (`self.NB1`)))
      (set `self.NB1` _newnb)
      (else
        (bind _newnb_2 (`self.ConstructNB` 1 (`self.NB2`)))
        (set `self.NB2` _newnb_2)))
    (`self.ChangeText` :!label _label)))

(event `self.Box2.OnComponentBeginOverlap`
  (params (OverlappedComponent :type "PrimitiveComponent Object Reference") (OtherActor :type "Actor Object Reference") (OtherComp :type "PrimitiveComponent Object Reference") (OtherBodyIndex :type Integer) (bFromSweep :type Boolean) (SweepResult :type "HitResult Structure (by ref)"))
  (if (`ActorComponent.ComponentHasTag` OtherComp "hand")
    (if (`self.NBSelectedIs1`)
      (bind _newnb (`self.ConstructNB` 3 (`self.NB1`)))
      (set `self.NB1` _newnb)
      (goto _label)
      (else
        (bind _newnb_2 (`self.ConstructNB` 3 (`self.NB2`)))
        (set `self.NB2` _newnb_2)
        (goto _label)))))

(event `self.Box1.OnComponentBeginOverlap`
  (params (OverlappedComponent :type "PrimitiveComponent Object Reference") (OtherActor :type "Actor Object Reference") (OtherComp :type "PrimitiveComponent Object Reference") (OtherBodyIndex :type Integer) (bFromSweep :type Boolean) (SweepResult :type "HitResult Structure (by ref)"))
  (if (`ActorComponent.ComponentHasTag` OtherComp "hand")
    (if (`self.NBSelectedIs1`)
      (bind _newnb (`self.ConstructNB` 2 (`self.NB1`)))
      (set `self.NB1` _newnb)
      (goto _label)
      (else
        (bind _newnb_2 (`self.ConstructNB` 2 (`self.NB2`)))
        (set `self.NB2` _newnb_2)
        (goto _label)))))

(event `self.Box6.OnComponentBeginOverlap`
  (params (OverlappedComponent :type "PrimitiveComponent Object Reference") (OtherActor :type "Actor Object Reference") (OtherComp :type "PrimitiveComponent Object Reference") (OtherBodyIndex :type Integer) (bFromSweep :type Boolean) (SweepResult :type "HitResult Structure (by ref)"))
  (if (`ActorComponent.ComponentHasTag` OtherComp "hand")
    (if (`self.NBSelectedIs1`)
      (bind _newnb (`self.ConstructNB` 7 (`self.NB1`)))
      (set `self.NB1` _newnb)
      (goto _label)
      (else
        (bind _newnb_2 (`self.ConstructNB` 7 (`self.NB2`)))
        (set `self.NB2` _newnb_2)
        (goto _label)))))

(event `self.Box3.OnComponentBeginOverlap`
  (params (OverlappedComponent :type "PrimitiveComponent Object Reference") (OtherActor :type "Actor Object Reference") (OtherComp :type "PrimitiveComponent Object Reference") (OtherBodyIndex :type Integer) (bFromSweep :type Boolean) (SweepResult :type "HitResult Structure (by ref)"))
  (if (`ActorComponent.ComponentHasTag` OtherComp "hand")
    (if (`self.NBSelectedIs1`)
      (bind _newnb (`self.ConstructNB` 4 (`self.NB1`)))
      (set `self.NB1` _newnb)
      (goto _label)
      (else
        (bind _newnb_2 (`self.ConstructNB` 4 (`self.NB2`)))
        (set `self.NB2` _newnb_2)
        (goto _label)))))

(event `self.Box4.OnComponentBeginOverlap`
  (params (OverlappedComponent :type "PrimitiveComponent Object Reference") (OtherActor :type "Actor Object Reference") (OtherComp :type "PrimitiveComponent Object Reference") (OtherBodyIndex :type Integer) (bFromSweep :type Boolean) (SweepResult :type "HitResult Structure (by ref)"))
  (if (`ActorComponent.ComponentHasTag` OtherComp "hand")
    (if (`self.NBSelectedIs1`)
      (bind _newnb (`self.ConstructNB` 5 (`self.NB1`)))
      (set `self.NB1` _newnb)
      (goto _label)
      (else
        (bind _newnb_2 (`self.ConstructNB` 5 (`self.NB2`)))
        (set `self.NB2` _newnb_2)
        (goto _label)))))

(event `self.Box5.OnComponentBeginOverlap`
  (params (OverlappedComponent :type "PrimitiveComponent Object Reference") (OtherActor :type "Actor Object Reference") (OtherComp :type "PrimitiveComponent Object Reference") (OtherBodyIndex :type Integer) (bFromSweep :type Boolean) (SweepResult :type "HitResult Structure (by ref)"))
  (if (`ActorComponent.ComponentHasTag` OtherComp "hand")
    (if (`self.NBSelectedIs1`)
      (bind _newnb (`self.ConstructNB` 6 (`self.NB1`)))
      (set `self.NB1` _newnb)
      (goto _label)
      (else
        (bind _newnb_2 (`self.ConstructNB` 6 (`self.NB2`)))
        (set `self.NB2` _newnb_2)
        (goto _label)))))

(event `self.Box_1.OnComponentBeginOverlap`
  (params (OverlappedComponent :type "PrimitiveComponent Object Reference") (OtherActor :type "Actor Object Reference") (OtherComp :type "PrimitiveComponent Object Reference") (OtherBodyIndex :type Integer) (bFromSweep :type Boolean) (SweepResult :type "HitResult Structure (by ref)"))
  (if (`ActorComponent.ComponentHasTag` OtherComp "hand")
    (if (`self.NBSelectedIs1`)
      (bind _newnb (`self.ConstructNB` 0 (`self.NB1`)))
      (set `self.NB1` _newnb)
      (goto _label)
      (else
        (bind _newnb_2 (`self.ConstructNB` 0 (`self.NB2`)))
        (set `self.NB2` _newnb_2)
        (goto _label)))))

(event `self.Box8.OnComponentBeginOverlap`
  (params (OverlappedComponent :type "PrimitiveComponent Object Reference") (OtherActor :type "Actor Object Reference") (OtherComp :type "PrimitiveComponent Object Reference") (OtherBodyIndex :type Integer) (bFromSweep :type Boolean) (SweepResult :type "HitResult Structure (by ref)"))
  (if (`ActorComponent.ComponentHasTag` OtherComp "hand")
    (if (`self.NBSelectedIs1`)
      (bind _newnb (`self.ConstructNB` 9 (`self.NB1`)))
      (set `self.NB1` _newnb)
      (goto _label)
      (else
        (bind _newnb_2 (`self.ConstructNB` 9 (`self.NB2`)))
        (set `self.NB2` _newnb_2)
        (goto _label)))))

(event `self.Box7.OnComponentBeginOverlap`
  (params (OverlappedComponent :type "PrimitiveComponent Object Reference") (OtherActor :type "Actor Object Reference") (OtherComp :type "PrimitiveComponent Object Reference") (OtherBodyIndex :type Integer) (bFromSweep :type Boolean) (SweepResult :type "HitResult Structure (by ref)"))
  (if (`ActorComponent.ComponentHasTag` OtherComp "hand")
    (if (`self.NBSelectedIs1`)
      (bind _newnb (`self.ConstructNB` 8 (`self.NB1`)))
      (set `self.NB1` _newnb)
      (goto _label)
      (else
        (bind _newnb_2 (`self.ConstructNB` 8 (`self.NB2`)))
        (set `self.NB2` _newnb_2)
        (goto _label)))))

(event `self.Box12.OnComponentBeginOverlap`
  (params (OverlappedComponent :type "PrimitiveComponent Object Reference") (OtherActor :type "Actor Object Reference") (OtherComp :type "PrimitiveComponent Object Reference") (OtherBodyIndex :type Integer) (bFromSweep :type Boolean) (SweepResult :type "HitResult Structure (by ref)"))
  (if (`ActorComponent.ComponentHasTag` OtherComp "hand")
    (if (`self.NBSelectedIs1`)
      (set `self.NBSelectedIs1` false)
      (set `self.NB2` 0.0)
      (else
        (`self.Calculator`)))
    (set `self.LastOperator` "-")
    (`self.ChangeText` :!label _label_2)))

(event `self.Box9.OnComponentBeginOverlap`
  (params (OverlappedComponent :type "PrimitiveComponent Object Reference") (OtherActor :type "Actor Object Reference") (OtherComp :type "PrimitiveComponent Object Reference") (OtherBodyIndex :type Integer) (bFromSweep :type Boolean) (SweepResult :type "HitResult Structure (by ref)"))
  (if (`ActorComponent.ComponentHasTag` OtherComp "hand")
    (if (`self.NBSelectedIs1`)
      (set `self.NBSelectedIs1` false)
      (set `self.NB2` 0.0)
      (else
        (`self.Calculator`)))
    (set `self.LastOperator` "*")
    (goto _label_2)))

(event `self.Box10.OnComponentBeginOverlap`
  (params (OverlappedComponent :type "PrimitiveComponent Object Reference") (OtherActor :type "Actor Object Reference") (OtherComp :type "PrimitiveComponent Object Reference") (OtherBodyIndex :type Integer) (bFromSweep :type Boolean) (SweepResult :type "HitResult Structure (by ref)"))
  (if (`ActorComponent.ComponentHasTag` OtherComp "hand")
    (if (`self.NBSelectedIs1`)
      (set `self.NBSelectedIs1` false)
      (set `self.NB2` 0.0)
      (else
        (`self.Calculator`)))
    (set `self.LastOperator` "/")
    (goto _label_2)))

(event `self.Box11.OnComponentBeginOverlap`
  (params (OverlappedComponent :type "PrimitiveComponent Object Reference") (OtherActor :type "Actor Object Reference") (OtherComp :type "PrimitiveComponent Object Reference") (OtherBodyIndex :type Integer) (bFromSweep :type Boolean) (SweepResult :type "HitResult Structure (by ref)"))
  (if (`ActorComponent.ComponentHasTag` OtherComp "hand")
    (if (`self.NBSelectedIs1`)
      (set `self.NBSelectedIs1` false)
      (set `self.NB2` 0.0)
      (else
        (`self.Calculator`)))
    (set `self.LastOperator` "+")
    (goto _label_2)))

(event `self.Box13.OnComponentBeginOverlap`
  (params (OverlappedComponent :type "PrimitiveComponent Object Reference") (OtherActor :type "Actor Object Reference") (OtherComp :type "PrimitiveComponent Object Reference") (OtherBodyIndex :type Integer) (bFromSweep :type Boolean) (SweepResult :type "HitResult Structure (by ref)"))
  (if (`ActorComponent.ComponentHasTag` OtherComp "hand")
    (set `self.NBSelectedIs1` true)
    (`self.Calculator`)
    (`self.ChangeText`)))

(event `self.Box_2.OnComponentBeginOverlap`
  (params (OverlappedComponent :type "PrimitiveComponent Object Reference") (OtherActor :type "Actor Object Reference") (OtherComp :type "PrimitiveComponent Object Reference") (OtherBodyIndex :type Integer) (bFromSweep :type Boolean) (SweepResult :type "HitResult Structure (by ref)"))
  (if (`ActorComponent.ComponentHasTag` OtherComp "hand")
    (set `self.NB1` 0.0)
    (set `self.NB2` 0.0)
    (set `self.NBSelectedIs1` true)
    (`self.ChangeText`)))

(fn `Calculator`
  (if (== "+" (`self.LastOperator`))
    (set `self.NB1` (+ (`self.NB1`) (`self.NB2`)))
    (elif (== "-" (`self.LastOperator`))
      (set `self.NB1` (- (`self.NB1`) (`self.NB2`)))
      (elif (== "*" (`self.LastOperator`))
        (set `self.NB1` (* (`self.NB1`) (`self.NB2`)))
        (elif (== "/" (`self.LastOperator`))
          (set `self.NB1` (/ (`self.NB1`) (`self.NB2`)))))))
  (set `self.NB2` 0.0))

(fn `ChangeText`
  (bind _textdisplay (`self.TextDisplay`))
  (if (`self.NBSelectedIs1`)
    (`TextRenderComponent.K2_SetText` _textdisplay (`KismetTextLibrary.Conv_DoubleToText` (`self.NB1`) "HalfToEven"))
    (else
      (`TextRenderComponent.K2_SetText` _textdisplay (`KismetTextLibrary.Conv_DoubleToText` (`self.NB2`) "HalfToEven")))))

(fn `ConstructNB`
  (params (Input :type Integer) (NbSelected :type "Float (double-precision)"))
  (returns (NewNB :type "Float (double-precision)"))
  (return (+ (* NbSelected 10.0) Input)))

(fn `UserConstructionScript`
  (bind _x (`self.X`))
  (bind _9 (`self.9`))
  (bind _8 (`self.8`))
  (bind __ (`self./`))
  (bind ___2 (`self.+`))
  (bind ___3 (`self.-`))
  (bind _2 (`self.2`))
  (bind _3 (`self.3`))
  (bind _1 (`self.1`))
  (bind _6 (`self.6`))
  (bind _5 (`self.5`))
  (bind _4 (`self.4`))
  (bind _7 (`self.7`))
  (bind _0 (`self.0`))
  (bind ___4 (`self.=`))
  (bind _c (`self.C`))
  (`TextRenderComponent.K2_SetText` _x (`KismetTextLibrary.Conv_StringToText` (`KismetSystemLibrary.GetObjectName` _x)))
  (`TextRenderComponent.K2_SetText` _9 (`KismetTextLibrary.Conv_StringToText` (`KismetSystemLibrary.GetObjectName` _9)))
  (`TextRenderComponent.K2_SetText` _8 (`KismetTextLibrary.Conv_StringToText` (`KismetSystemLibrary.GetObjectName` _8)))
  (`TextRenderComponent.K2_SetText` __ (`KismetTextLibrary.Conv_StringToText` (`KismetSystemLibrary.GetObjectName` __)))
  (`TextRenderComponent.K2_SetText` ___2 (`KismetTextLibrary.Conv_StringToText` (`KismetSystemLibrary.GetObjectName` ___2)))
  (`TextRenderComponent.K2_SetText` ___3 (`KismetTextLibrary.Conv_StringToText` (`KismetSystemLibrary.GetObjectName` ___3)))
  (`TextRenderComponent.K2_SetText` _2 (`KismetTextLibrary.Conv_StringToText` (`KismetSystemLibrary.GetObjectName` _2)))
  (`TextRenderComponent.K2_SetText` _3 (`KismetTextLibrary.Conv_StringToText` (`KismetSystemLibrary.GetObjectName` _3)))
  (`TextRenderComponent.K2_SetText` _1 (`KismetTextLibrary.Conv_StringToText` (`KismetSystemLibrary.GetObjectName` _1)))
  (`TextRenderComponent.K2_SetText` _6 (`KismetTextLibrary.Conv_StringToText` (`KismetSystemLibrary.GetObjectName` _6)))
  (`TextRenderComponent.K2_SetText` _5 (`KismetTextLibrary.Conv_StringToText` (`KismetSystemLibrary.GetObjectName` _5)))
  (`TextRenderComponent.K2_SetText` _4 (`KismetTextLibrary.Conv_StringToText` (`KismetSystemLibrary.GetObjectName` _4)))
  (`TextRenderComponent.K2_SetText` _7 (`KismetTextLibrary.Conv_StringToText` (`KismetSystemLibrary.GetObjectName` _7)))
  (`TextRenderComponent.K2_SetText` _0 (`KismetTextLibrary.Conv_StringToText` (`KismetSystemLibrary.GetObjectName` _0)))
  (`TextRenderComponent.K2_SetText` ___4 (`KismetTextLibrary.Conv_StringToText` (`KismetSystemLibrary.GetObjectName` ___4)))
  (`TextRenderComponent.K2_SetText` _c (`KismetTextLibrary.Conv_StringToText` (`KismetSystemLibrary.GetObjectName` _c))))