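; BP_FuelChecker is an interactive object that checks delivered fuel against an expected recipe.
; When a BP_Fuel overlaps its Box, it copies the fuel's FuelIngredient map and destroys that actor.
; It compares keys and values index by index with its Result map, so entry order matters, breaking on a mismatch.
; ChangeCompleteState(true) follows the loop, even after a mismatch break.
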(event `self.Box.OnComponentBeginOverlap`
  (params (OverlappedComponent :type "PrimitiveComponent Object Reference") (OtherActor :type "Actor Object Reference") (OtherComp :type "PrimitiveComponent Object Reference") (OtherBodyIndex :type Integer) (bFromSweep :type Boolean) (SweepResult :type "HitResult Structure (by ref)"))
  (bind _asbp_fuel (cast `/Game/Blueprint/InteractiveObject/Fuel/BP_Fuel` OtherActor))
  (bind _output_get (set `self.FuelIngredient` (`/Game/Blueprint/InteractiveObject/Fuel/BP_Fuel.FuelIngredient` _asbp_fuel)))
  (`self.K2_DestroyActor` OtherActor)
  (bind _keys (`BlueprintMapLibrary.Map_Keys` _output_get))
  (for (_array_element _array_index) _keys
    (bind _keys_2 (`BlueprintMapLibrary.Map_Keys` (`self.Result`)))
    (if (== _array_element (`KismetMathLibrary.Conv_ByteToInt` (`|GetArrayItem` _keys_2 _array_index)))
      (bind _values (`BlueprintMapLibrary.Map_Values` (`self.Result`)))
      (bind _values_2 (`BlueprintMapLibrary.Map_Values` (`self.FuelIngredient`)))
      (if (not (== (`|GetArrayItem` _values_2 _array_index) (`|GetArrayItem` _values _array_index)))
        (break))
      (else
        (break))))
  (`self.ChangeCompleteState` true))

(fn `UserConstructionScript`
  (`parent.UserConstructionScript`))