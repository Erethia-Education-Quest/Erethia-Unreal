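; BP_FuelMerger is an interactive machine that collects dropped ingredients and combines them into fuel.
; Ingredients entering Box are destroyed and their quantities summed by type in the ListIngredient map, which is shown on TextScreen and printed for debug.
; A component tagged "hand" touching Boxvalidate spawns a BP_Fuel offset by the Cube's bounds and passes it the map, which is never cleared.
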(event `self.Box.OnComponentBeginOverlap`
  (params (OverlappedComponent :type "PrimitiveComponent Object Reference") (OtherActor :type "Actor Object Reference") (OtherComp :type "PrimitiveComponent Object Reference") (OtherBodyIndex :type Integer) (bFromSweep :type Boolean) (SweepResult :type "HitResult Structure (by ref)"))
  (bind _listingredient (`self.ListIngredient`))
  (bind _returnvalue (`KismetTextLibrary.Conv_StringToText` (`self.ToDisplay`)))
  (bind _asbp_ingredient (cast `/Game/Blueprint/InteractiveObject/Fuel/BP_ingredient` OtherActor))
  (bind _ingredienttype (`/Game/Blueprint/InteractiveObject/Fuel/BP_ingredient.IngredientType` _asbp_ingredient))
  (bind (_value _returnvalue_2) (`BlueprintMapLibrary.Map_Find` (`self.ListIngredient`) _ingredienttype))
  (if _returnvalue_2
    (bind _quantity (`/Game/Blueprint/InteractiveObject/Fuel/BP_ingredient.Quantity` _asbp_ingredient))
    (`BlueprintMapLibrary.Map_Add` (`self.ListIngredient`) _ingredienttype (+ _value _quantity))
    (else
      (`BlueprintMapLibrary.Map_Add` (`self.ListIngredient`) _ingredienttype _quantity)))
  (`self.K2_DestroyActor` OtherActor)
  (set `self.ToDisplay` "")
  (bind _keys (`BlueprintMapLibrary.Map_Keys` _listingredient))
  (for (_array_element _array_index) _keys
    (bind _values (`BlueprintMapLibrary.Map_Values` _listingredient))
    (`self.SetDisplayString` _array_element (`|GetArrayItem` _values _array_index)))
  (`TextRenderComponent.K2_SetText` (`self.text_screen`) _returnvalue)
  (`KismetSystemLibrary.PrintString` (`KismetTextLibrary.Conv_TextToString` _returnvalue) true true (struct :`R` 1.0 :`G` 0.073834 :`B` 0.053938 :`A` 1.0)))

(event `self.boxvalidate.OnComponentBeginOverlap`
  (params (OverlappedComponent :type "PrimitiveComponent Object Reference") (OtherActor :type "Actor Object Reference") (OtherComp :type "PrimitiveComponent Object Reference") (OtherBodyIndex :type Integer) (bFromSweep :type Boolean) (SweepResult :type "HitResult Structure (by ref)"))
  (bind (_returnvalue_location _returnvalue_rotation _returnvalue_scale) (`KismetMathLibrary.BreakTransform` (`SceneComponent.K2_GetComponentToWorld` (`self.Object`))))
  (bind (_min _max) (`StaticMeshComponent.GetLocalBounds` (`self.Cube`)))
  (if (`ActorComponent.ComponentHasTag` OtherComp "hand")
    (bind _returnvalue (`|SpawnActorFromClass` "/Game/Blueprint/InteractiveObject/Fuel/BP_Fuel.BP_Fuel_C" (`KismetMathLibrary.MakeTransform` (- (- _returnvalue_location (`KismetMathLibrary.MakeVector` (.x _max))) (`KismetMathLibrary.MakeVector` (/ (.x _max) 10.0))) _returnvalue_rotation _returnvalue_scale) "AdjustIfPossibleButAlwaysSpawn" "MultiplyWithRoot" null null))
    (`/Game/Blueprint/InteractiveObject/Fuel/BP_Fuel.Add_IngredientList` _returnvalue (`self.ListIngredient`))))

(event `SetDisplayString`
  (params (IngredientType :type "/Game/Enum/E_Ingredient_Type Enum" :default "NewEnumerator0") (IngredientAmount :type "Float (double-precision)"))
  (set `self.ToDisplay` (`KismetStringLibrary.Concat_StrStr` (`self.ToDisplay`) (`KismetStringLibrary.Concat_StrStr` (`KismetStringLibrary.Concat_StrStr` (`KismetStringLibrary.Concat_StrStr` (`|GetEnumeratorNameAsString` IngredientType) ":         ") (`KismetStringLibrary.Conv_DoubleToString` IngredientAmount)) "<br>"))))

(fn `UserConstructionScript`
  (`parent.UserConstructionScript`))