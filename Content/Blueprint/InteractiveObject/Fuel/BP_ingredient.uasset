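; BP_ingredient is an interactive ingredient object in the Fuel folder that carries an ingredient type and a quantity.
; Setter events assign the type and quantity.
; SetPhysics switches its Object component to simulated physics with gravity and query-and-physics collision.
; BeginPlay and the construction script only call their parent versions.
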(event `self.ReceiveBeginPlay`
  (`parent.ReceiveBeginPlay`))

(event `SetIngredientEnum`
  (params (ing :type "/Game/Enum/E_Ingredient_Type Enum" :default "NewEnumerator0"))
  (set `self.IngredientType` ing))

(event `SETQuantity`
  (params (IngQuantity :type "Float (double-precision)"))
  (set `self.Quantity` IngQuantity))

(event `SetPhysics`
  (bind _object (`self.Object`))
  (`PrimitiveComponent.SetSimulatePhysics` _object true)
  (`PrimitiveComponent.SetEnableGravity` _object true)
  (`PrimitiveComponent.SetCollisionEnabled` _object "QueryAndPhysics"))

(fn `UserConstructionScript`
  (`parent.UserConstructionScript`))