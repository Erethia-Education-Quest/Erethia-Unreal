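; Master Blueprint for grabbable interactive objects, tracking which player holds each one.
; On authority, Tick passes the actor's transform to the game state for every player in the game instance's list, and an update event applies received location and rotation.
; The parent's transform update runs only while the object is not grabbed.
; A fresco function repositions the object component and hides a child decal.
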(event `UpdateGrabblePosition`
  (params (Location :type "Vector Structure") (Rotation :type "Rotator Structure"))
  (`self.K2_SetActorLocationAndRotation` Location Rotation))

(event `self.ReceiveBeginPlay`
  (`parent.ReceiveBeginPlay`)
  (bind _asgs_game (cast `/Game/Blueprint/GameState/GS_Game` (`self.RefGS`)))
  (set `self.RefGsGame` _asgs_game))

(event `self.ReceiveTick`
  (params (DeltaSeconds :type "Float (single-precision)"))
  (bind (_returnvalue_location _returnvalue_rotation) (`KismetMathLibrary.BreakTransform` (`self.GetTransform`)))
  (`/Engine/EditorBlueprintResources/ActorMacros.Switch Has Authority`
    (:`Authority`
      (for _array_element (`/Game/Blueprint/GameInstance/BP_GameInstance.ListPlayerInfo` (`self.RefGI`))
        (`/Game/Blueprint/GameState/GS_Master.UpdateGrabblePosition` (`self.RefGsGame`) (`.PC_11_776544A84872013AA63BC881D8B483A2` (break `/Game/Struct/S_PlayerInfo` _array_element)) self _returnvalue_location _returnvalue_rotation)))))

(event `set PlayerGrabing`
  (params (Player :type "/Game/Blueprint/Player/BP_Player Object Reference"))
  (set `self.PlayerGrabing` Player)
  (set `self.IsGrabbed?` true))

(event `RealeseGrab`
  (set `self.PlayerGrabing` null)
  (set `self.IsGrabbed?` false))

(event `SetVisible`
  (`SceneComponent.SetVisibility` (`self.Object`) true false))

(event `self.UpdateTransformObject`
  (if (not (`self.IsGrabbed?`))
    (`parent.UpdateTransformObject`)))

(fn `SetPositionFresco`
  (params (NewTransform :type "Transform Structure"))
  (bind _object (`self.Object`))
  (`SceneComponent.K2_SetWorldTransform` _object NewTransform false false)
  (for _array_element (`SceneComponent.GetChildrenComponents` _object false)
    (bind _asdecal_component (cast `DecalComponent` _array_element)
      (:`then`
        (`SceneComponent.SetVisibility` _asdecal_component false false))
      (:`CastFailed`
        _))
    (return)))

(fn `UserConstructionScript`
  (`parent.UserConstructionScript`))