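; BP_MasterPuzzleStatue is a grabbable puzzle statue that can rotate and shows a menu widget while held.
; On begin play its object gets query and physics collision but ignores pawns.
; Grabbing places the widget at the left or right anchor according to the holding hand, and releasing hides it.
; A Rotation event plays a timeline that adds yaw incrementally to the object, zeroing pitch and roll.
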(event `self.ReceiveBeginPlay`
  (bind _object (`self.Object`))
  (`parent.ReceiveBeginPlay`)
  (`PrimitiveComponent.SetCollisionEnabled` _object "QueryAndPhysics")
  (`PrimitiveComponent.SetCollisionResponseToChannel` _object "ECC_Pawn" "ECR_Ignore"))

(event `Rotation`
  (bind (_relativerotation_roll _relativerotation_pitch _relativerotation_yaw) (`KismetMathLibrary.BreakRotator` (`SceneComponent.RelativeRotation` (`self.Object`))))
  (bind (_direction _alpha) (`Timeline|Chronologie`)
    (:`Update`
      (`SceneComponent.K2_SetWorldRotation` (`self.Object`) (`KismetMathLibrary.MakeRotator` 0.0 0.0 (+ _relativerotation_yaw (* _alpha 2.0))) false false))))

(event `/Game/Blueprint/Interface/BPI_GrabObject.GrabInterraction`
  (params (PlayerGrabber :type "/Game/Blueprint/Player/BP_Player Object Reference"))
  (if (== (`/Game/Blueprint/Player/BP_Player.RefGrabbedObejct` PlayerGrabber) self)
    (`/Engine/EditorBlueprintResources/StandardMacros.IsValid` (`/Game/Blueprint/Player/BP_Player.HeldComponentLeft` PlayerGrabber)
      (:`Is Valid`
        (`SceneComponent.K2_SetRelativeLocation` (`self.Widget`) (`SceneComponent.RelativeLocation` (`self.PosMenuLeft`)) false false))
      (:`Is Not Valid`
        (`/Engine/EditorBlueprintResources/StandardMacros.IsValid` (`/Game/Blueprint/Player/BP_Player.HeldComponentRight` PlayerGrabber)
          (:`Is Valid`
            (`SceneComponent.K2_SetRelativeLocation` (`self.Widget`) (`SceneComponent.RelativeLocation` (`self.PosMenuRight`)) false false)))))
    (`SceneComponent.SetHiddenInGame` (`self.Widget`) false false)))

(event `/Game/Blueprint/Interface/BPI_GrabObject.ReleaseInterraction`
  (params (PlayerRelease :type "/Game/Blueprint/Player/BP_Player Object Reference"))
  (if (== (`/Game/Blueprint/Player/BP_Player.RefGrabbedObejct` PlayerRelease) self)
    (`SceneComponent.SetHiddenInGame` (`self.Widget`) true false)))

(fn `UserConstructionScript`
  (`parent.UserConstructionScript`))