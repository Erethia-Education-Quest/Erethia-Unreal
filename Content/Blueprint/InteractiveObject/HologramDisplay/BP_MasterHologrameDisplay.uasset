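; Master controller for the level's BP_HologrameDisplay actors, cycling them through eight orientation patterns when a "hand"-tagged component overlaps its box.
; Each pattern maps materials to displays by their GetAllActorsOfClass index, hiding any display without a valid material.
; Only the authority advances the index, then relays it through GS_Game for player controllers listed in the game instance, rather than using replicated variables.
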(event `SetOrientaion`
  (params (OrientationIndex :type Integer))
  (`self.ActualiseHologram` (`|GetArrayItem` (`self.PatternList`) OrientationIndex)))

(event `ChangeOrientation`
  (bind _result (`/Engine/EditorBlueprintResources/StandardMacros.IncrementInt` (`self.OriantationIndex`))
    (:`  `
      (bind _output_get (set `self.OriantationIndex` _result))
      (if (>= _output_get 8)
        (set `self.OriantationIndex` 0))
      (`self.ActualiseHologram` (`|GetArrayItem` (`self.PatternList`) (`self.OriantationIndex`))))))

(event `self.ReceiveBeginPlay`
  (`parent.ReceiveBeginPlay`)
  (bind _outactors (`GameplayStatics.GetAllActorsOfClass` "/Game/Blueprint/InteractiveObject/HologramDisplay/BP_HologrameDisplay.BP_HologrameDisplay_C"))
  (set `self.AllHolograme` _outactors)
  (bind _asbp_game_instance (cast `/Game/Blueprint/GameInstance/BP_GameInstance` (`GameplayStatics.GetGameInstance`)))
  (set `self.Ref_GI` _asbp_game_instance)
  (bind _asgs_game (cast `/Game/Blueprint/GameState/GS_Game` (`GameplayStatics.GetGameState`)))
  (set `self.Ref_GS` _asgs_game))

(event `ActualiseHologram`
  (params (Pattern :type "/Game/Blueprint/InteractiveObject/HologramDisplay/ST_PatternMaterial Structure"))
  (for (_array_element _array_index) (`self.AllHolograme`)
    (bind _output (`|GetArrayItem` Pattern_Pattern_1_3_D740088F4D9EE2D39501EAB061DB710D _array_index))
    (`/Engine/EditorBlueprintResources/StandardMacros.IsValid` _output
      (:`Is Valid`
        (`/Game/Blueprint/InteractiveObject/HologramDisplay/BP_HologrameDisplay.SetVisible` _array_element true)
        (`/Game/Blueprint/InteractiveObject/HologramDisplay/BP_HologrameDisplay.ChangeMaterial` _array_element _output))
      (:`Is Not Valid`
        (`/Game/Blueprint/InteractiveObject/HologramDisplay/BP_HologrameDisplay.SetVisible` _array_element false)))))

(event `self.Box.OnComponentBeginOverlap`
  (params (OverlappedComponent :type "PrimitiveComponent Object Reference") (OtherActor :type "Actor Object Reference") (OtherComp :type "PrimitiveComponent Object Reference") (OtherBodyIndex :type Integer) (bFromSweep :type Boolean) (SweepResult :type "HitResult Structure (by ref)"))
  (if (`ActorComponent.ComponentHasTag` OtherComp "hand")
    (`self.ChangeOrientationNetwork`)))

(event `ChangeOrientationNetwork`
  (bind _ref_gi (`self.Ref_GI`))
  (bind _ref_gs (`self.Ref_GS`))
  (`/Engine/EditorBlueprintResources/ActorMacros.Switch Has Authority`
    (:`Authority`
      (`self.ChangeOrientationServeur`)
      (if (and (`KismetSystemLibrary.IsValid` _ref_gi) (`KismetSystemLibrary.IsValid` _ref_gs))
        (for _array_element (`/Game/Blueprint/GameInstance/BP_GameInstance.ListPlayerInfo` _ref_gi)
          (bind _aspc_game (cast `/Game/Blueprint/PlayerController/PC_Game` (`.PC_11_776544A84872013AA63BC881D8B483A2` (break `/Game/Struct/S_PlayerInfo` _array_element))))
          (`/Game/Blueprint/GameState/GS_Game.ChangeOrientationClient` _ref_gs _aspc_game self (`self.OriantationIndex`)))))))

(event `ChangeOrientationServeur`
  (`self.ChangeOrientation`))

(event `ChangeOrientationClient`
  (params (OrientationIndex :type Integer))
  (`self.SetOrientaion` OrientationIndex))

(fn `UserConstructionScript`
  (`parent.UserConstructionScript`))