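; Puzzle pedestal that accepts its assigned statue when that object overlaps its box, activating once and notifying StatueRef.
; GrabItem snaps the statuette above the cube, disables its physics and collision, releases it from the grabbing player and starts its Rotation.
; The snap runs through a server event, then GS_Game is called for each player controller listed in the GameInstance to relay it to clients.
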(event `self.ReceiveBeginPlay`
  (`parent.ReceiveBeginPlay`)
  (bind _asbp_game_instance (cast `/Game/Blueprint/GameInstance/BP_GameInstance` (`GameplayStatics.GetGameInstance`)))
  (set `self.Ref_GI` _asbp_game_instance)
  (bind _asgs_game (cast `/Game/Blueprint/GameState/GS_Game` (`GameplayStatics.GetGameState`)))
  (set `self.Ref_GS` _asgs_game))

(event `self.Box.OnComponentBeginOverlap`
  (params (OverlappedComponent :type "PrimitiveComponent Object Reference") (OtherActor :type "Actor Object Reference") (OtherComp :type "PrimitiveComponent Object Reference") (OtherBodyIndex :type Integer) (bFromSweep :type Boolean) (SweepResult :type "HitResult Structure (by ref)"))
  (bind _ref_gi (`self.Ref_GI`))
  (bind _ref_gs (`self.Ref_GS`))
  (if (== OtherActor (`self.Interact_OBJ`))
    (if (not (`self.IsActivated`))
      (bind _output_get (set `self.IsActivated` (not (`self.IsActivated`))))
      (if _output_get
        (`/Game/Blueprint/InteractiveObject/Statue/BP_CentralStatue.OnPiedestalActivated` (`self.StatueRef`) self)
        (bind _asbp_master_puzzle_statue (cast `/Game/Blueprint/InteractiveObject/Gabable_OBJ/Statue/BP_MasterPuzzleStatue` OtherActor))
        (`self.GrabItemServeur` _asbp_master_puzzle_statue)
        (if (and (`KismetSystemLibrary.IsValid` _ref_gi) (`KismetSystemLibrary.IsValid` _ref_gs))
          (for _array_element (`/Game/Blueprint/GameInstance/BP_GameInstance.ListPlayerInfo` _ref_gi)
            (bind _aspc_game (cast `/Game/Blueprint/PlayerController/PC_Game` (`.PC_11_776544A84872013AA63BC881D8B483A2` (break `/Game/Struct/S_PlayerInfo` _array_element))))
            (`/Game/Blueprint/GameState/GS_Game.GrabItemClient` _ref_gs _aspc_game self _asbp_master_puzzle_statue)))))))

(event `GrabItemClient`
  (params (Statuettee :type "/Game/Blueprint/InteractiveObject/Gabable_OBJ/Statue/BP_MasterPuzzleStatue Object Reference"))
  (`self.GrabItem` Statuettee))

(event `GrabItemServeur`
  (params (Statuettee :type "/Game/Blueprint/InteractiveObject/Gabable_OBJ/Statue/BP_MasterPuzzleStatue Object Reference"))
  (`self.GrabItem` Statuettee))

(fn `GrabItem`
  (params (Statuette :type "/Game/Blueprint/InteractiveObject/Gabable_OBJ/Statue/BP_MasterPuzzleStatue Object Reference"))
  (bind _object (`/Game/Blueprint/InteractiveObject/BP_MasterInteractive.Object` Statuette))
  (bind _playergrabing (`/Game/Blueprint/InteractiveObject/Gabable_OBJ/BP_MasterGrabbableObjects.PlayerGrabing` Statuette))
  (bind (_returnvalue_x _returnvalue_y _returnvalue_z) (`KismetMathLibrary.BreakVector` (`SceneComponent.K2_GetComponentLocation` (`self.Cube`))))
  (`PrimitiveComponent.SetSimulatePhysics` _object false)
  (`PrimitiveComponent.SetEnableGravity` _object false)
  (`SceneComponent.K2_SetWorldLocation` _object (`KismetMathLibrary.MakeVector` _returnvalue_x _returnvalue_y (+ _returnvalue_z 100.0)) false false)
  (`SceneComponent.K2_SetWorldRotation` :`self` _object)
  (`PrimitiveComponent.SetCollisionEnabled` _object "NoCollision")
  (`/Engine/EditorBlueprintResources/StandardMacros.IsValid` _playergrabing
    (:`Is Valid`
      (`/Game/Blueprint/Player/BP_Player.ReleaseObjectServer` _playergrabing "NewEnumerator1"))
    (:`Is Not Valid`
      _))
  (`/Engine/EditorBlueprintResources/StandardMacros.IsValid` _playergrabing
    (:`Is Valid`
      (`/Game/Blueprint/Player/BP_Player.ReleaseObjectServer` _playergrabing "NewEnumerator2"))
    (:`Is Not Valid`
      _))
  (`/Game/Blueprint/InteractiveObject/Gabable_OBJ/Statue/BP_MasterPuzzleStatue.Rotation` Statuette))

(fn `UserConstructionScript`
  (`parent.UserConstructionScript`)
  (`DecalComponent.SetDecalMaterial` (`self.Decal`) (`self.DecalMaterial`)))