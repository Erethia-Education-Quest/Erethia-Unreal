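; Checkerboard actor that tracks which tiles of a grid are overlapped by BP_Pilar actors.
; The construction script divides the SizeBoard box into rows and columns of generated box components, mapping each to a 2D grid coordinate.
; It also binds every tile's begin and end overlap events, which set that coordinate's flag in the AllTIles map to true or false.
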(event `EndOverlapTile`
  (params (OverlappedComponent :type "PrimitiveComponent Object Reference") (OtherActor :type "Actor Object Reference") (OtherComp :type "PrimitiveComponent Object Reference") (OtherBodyIndex :type Integer))
  (if (== (`GameplayStatics.GetObjectClass` OtherActor) "/Game/Blueprint/InteractiveObject/Pilar/BP_Pilar.BP_Pilar_C")
    (bind _asbox_collision (cast `BoxComponent` OverlappedComponent))
    (bind (_value _returnvalue) (`BlueprintMapLibrary.Map_Find` (`self.AllTilesRefBoxColision`) _asbox_collision))
    (if _returnvalue
      (`BlueprintMapLibrary.Map_Add` (`self.AllTIles`) _value)
      (`KismetSystemLibrary.PrintString` "EndOverlap" false false))))

(event `LinkOnBeginOverlapTile`
  (bind _keys (`BlueprintMapLibrary.Map_Keys` (`self.AllTilesRefBoxColision`)))
  (for _array_element _keys
    (add `PrimitiveComponent.OnComponentBeginOverlap` _array_element (delegate `OverlapetedTile`))
    (add `PrimitiveComponent.OnComponentEndOverlap` _array_element (delegate `EndOverlapTile`))))

(event `OverlapetedTile`
  (params (OverlappedComponent :type "PrimitiveComponent Object Reference") (OtherActor :type "Actor Object Reference") (OtherComp :type "PrimitiveComponent Object Reference") (OtherBodyIndex :type Integer) (bFromSweep :type Boolean) (SweepResult :type "HitResult Structure (by ref)"))
  (if (== (`GameplayStatics.GetObjectClass` OtherActor) "/Game/Blueprint/InteractiveObject/Pilar/BP_Pilar.BP_Pilar_C")
    (bind _asbox_collision (cast `BoxComponent` OverlappedComponent))
    (bind (_value _returnvalue) (`BlueprintMapLibrary.Map_Find` (`self.AllTilesRefBoxColision`) _asbox_collision))
    (if _returnvalue
      (`BlueprintMapLibrary.Map_Add` (`self.AllTIles`) _value true)
      (`KismetSystemLibrary.PrintString` "Startoverlap" false false))))

(fn `CalcTilesSize`
  (bind (_returnvalue_x _returnvalue_y) (`KismetMathLibrary.BreakVector` (`BoxComponent.GetUnscaledBoxExtent` (`self.SizeBoard`))))
  (set `self.SizeX` (/ _returnvalue_x (`self.NbrBoxByLine`)))
  (set `self.SizeY` (/ _returnvalue_y (`self.NbrBoxByRow`))))

(fn `CreationTiles`
  (bind (_currentlocation_x _currentlocation_y _currentlocation_z) (`KismetMathLibrary.BreakVector` (`self.CurrentLocation`)))
  (bind (_currentlocation_x_2 _currentlocation_y_2 _currentlocation_z_2) (`KismetMathLibrary.BreakVector` (`self.CurrentLocation`)))
  (bind (_returnvalue_x _returnvalue_y) (`KismetMathLibrary.BreakVector2D` (+ (`self.ActualCreatedTile`) (0.0 1.0))))
  (for _ (range (`self.NbrBoxByRow`))
    (for _ (range (`self.NbrBoxByLine`))
      (`self.SpawnAndSetUp`)
      (set `self.CurrentLocation` (`KismetMathLibrary.MakeVector` (+ _currentlocation_x (* (`self.SizeX`) 2.0)) _currentlocation_y _currentlocation_z))
      (set `self.ActualCreatedTile` (+ (`self.ActualCreatedTile`) (1.0 0.0))))
    (set `self.CurrentLocation` (`KismetMathLibrary.MakeVector` _currentlocation_x_2 (+ _currentlocation_y_2 (* (`self.SizeY`) 2.0)) _currentlocation_z_2))
    (`self.ResetX`)
    (set `self.ActualCreatedTile` (`KismetMathLibrary.MakeVector2D` 0.0 _returnvalue_y))))

(fn `ResetX`
  (bind _sizeboard (`self.SizeBoard`))
  (bind (_currentlocation_x _currentlocation_y _currentlocation_z) (`KismetMathLibrary.BreakVector` (`self.CurrentLocation`)))
  (bind _returnvalue_x (`KismetMathLibrary.BreakVector` (`BoxComponent.GetUnscaledBoxExtent` _sizeboard)))
  (bind _relativelocation_x (`KismetMathLibrary.BreakVector` (`SceneComponent.RelativeLocation` _sizeboard)))
  (set `self.CurrentLocation` (`KismetMathLibrary.MakeVector` (+ (- _relativelocation_x _returnvalue_x) (`self.SizeX`)) _currentlocation_y _currentlocation_z)))

(fn `SetLocationTile`
  (bind _sizeboard (`self.SizeBoard`))
  (bind (_returnvalue_x _returnvalue_y) (`KismetMathLibrary.BreakVector` (`BoxComponent.GetUnscaledBoxExtent` _sizeboard)))
  (bind (_relativelocation_x _relativelocation_y _relativelocation_z) (`KismetMathLibrary.BreakVector` (`SceneComponent.RelativeLocation` _sizeboard)))
  (set `self.CurrentLocation` (`KismetMathLibrary.MakeVector` (+ (- _relativelocation_x _returnvalue_x) (`self.SizeX`)) (+ (- _relativelocation_y _returnvalue_y) (`self.SizeY`)) _relativelocation_z)))

(fn `SpawnAndSetUp`
  (bind _actualcreatedtile (`self.ActualCreatedTile`))
  (bind _returnvalue (`AddComponent|NODE_AddBoxComponent-0` :`bManualAttachment` true))
  (`SceneComponent.K2_AttachToComponent` _returnvalue (`self.SizeBoard`) "None" "KeepRelative" "KeepRelative" "KeepRelative" true)
  (`BoxComponent.SetBoxExtent` _returnvalue (`KismetMathLibrary.MakeVector` (`self.SizeX`) (`self.SizeY`)) true)
  (`SceneComponent.K2_SetRelativeLocation` _returnvalue (`self.CurrentLocation`) false false)
  (`BlueprintMapLibrary.Map_Add` (`self.AllTilesRefBoxColision`) _returnvalue _actualcreatedtile)
  (`BlueprintMapLibrary.Map_Add` (`self.AllTIles`) _actualcreatedtile))

(fn `UserConstructionScript`
  (`self.CalcTilesSize`)
  (`self.SetLocationTile`)
  (`self.CreationTiles`)
  (`self.LinkOnBeginOverlapTile`))