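; Puzzle pillar that moves across a tile board and can activate linked objects, such as doors, through PilarManager.
; Player overlaps report selection to the manager, while tile overlaps record board coordinates and snap the pillar on first contact.
; BeginPlay briefly moves it to the origin and back.
; Tick interpolates it through queued tile coordinates, resolved via the board's collision-box map, then triggers linked objects if the manager's result check passes.
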(event `self.ReceiveBeginPlay`
  (`parent.ReceiveBeginPlay`)
  (set `self.PosStart` (`self.K2_GetActorLocation`))
  (`self.K2_SetActorLocation` (0.0 0.0 0.0))
  (`KismetSystemLibrary.Delay` 0.2)
  (`self.K2_SetActorLocation` (`self.PosStart`)))

(event `ChangeColor`
  (params (Material :type "Material Object Reference"))
  (`PrimitiveComponent.SetMaterial` (`self.Cube`) 0 Material)
  (set `self.IsSelected` (not (`self.IsSelected`))))

(event `MoveTo`
  (`KismetArrayLibrary.Array_Remove` (`self.AllTargetLocation`))
  (set `self.IsMoving?` true))

(event `self.ReceiveTick`
  (params (DeltaSeconds :type "Float (single-precision)"))
  (bind (_returnvalue_x _returnvalue_y _returnvalue_z) (`KismetMathLibrary.BreakVector` (`self.K2_GetActorLocation`)))
  (bind _pilarmanager (`self.PilarManager`))
  (bind (_returnvalue_x_2 _returnvalue_y_2) (`KismetMathLibrary.BreakVector` (`SceneComponent.K2_GetComponentLocation` (`self.NextTileToGo`))))
  (if (`self.IsMoving?`)
    (`self.Move`)
    (if (== (`KismetMathLibrary.MakeVector` _returnvalue_x _returnvalue_y _returnvalue_z) (`KismetMathLibrary.MakeVector` _returnvalue_x_2 _returnvalue_y_2 _returnvalue_z) :`ErrorTolerance` 2.0)
      (set `self.NextTileToGo` null)
      (`KismetArrayLibrary.Array_Remove` (`self.AllTargetLocation`))
      (`KismetSystemLibrary.PrintText` (`|FormatText` "Arrived at location") false false)
      (if (<= (`KismetArrayLibrary.Array_Length` (`self.AllTargetLocation`)) 0)
        (set `self.IsMoving?` false)
        (bind _newparam (`/Game/Blueprint/InteractiveObject/Pilar/BP_PilarManager.CheckResult` _pilarmanager))
        (if _newparam
          (for _array_element (`/Game/Blueprint/InteractiveObject/Pilar/BP_PilarManager.InteractWith` _pilarmanager)
            (`/Engine/EditorBlueprintResources/StandardMacros.IsValid` _array_element
              (:`Is Valid`
                (`self.AtActivation` _array_element)
                (`KismetSystemLibrary.PrintText` (`|FormatText` "door open"))))))))))

(event `AdminSelection`
  (`/Game/Blueprint/InteractiveObject/Pilar/BP_PilarManager.PilarSelection` (`self.PilarManager`) self (`self.IsSelected`) :!label _label))

(event `self.Box.OnComponentBeginOverlap`
  (params (OverlappedComponent :type "PrimitiveComponent Object Reference") (OtherActor :type "Actor Object Reference") (OtherComp :type "PrimitiveComponent Object Reference") (OtherBodyIndex :type Integer) (bFromSweep :type Boolean) (SweepResult :type "HitResult Structure (by ref)"))
  (bind (_returnvalue_x _returnvalue_y _returnvalue_z) (`KismetMathLibrary.BreakVector` (`self.K2_GetActorLocation` self)))
  (if (`self.IsMoving?`)
    _
    (elif (== (`GameplayStatics.GetObjectClass` OtherActor) "/Game/Blueprint/Player/BP_Player.BP_Player_C")
      (goto _label)
      (else
        _)))
  (bind _asbox_collision (cast `BoxComponent` OtherComp))
  (bind (_value _returnvalue) (`BlueprintMapLibrary.Map_Find` (`/Game/Blueprint/InteractiveObject/Pilar/BP_CheckerBoard.AllTilesRefBoxColision` (`/Game/Blueprint/InteractiveObject/Pilar/BP_PilarManager.RefBoard` (`self.PilarManager`))) _asbox_collision))
  (if _returnvalue
    (set `self.CurrentTileCoord` (`KismetMathLibrary.MakeVector2D` (`KismetMathLibrary.BreakVector2D` _value) (`.Y` (`KismetMathLibrary.BreakVector2D` _value))))
    (if (`self.FirstTime`)
      (bind (_returnvalue_x_2 _returnvalue_y_2) (`KismetMathLibrary.BreakVector` (`SceneComponent.K2_GetComponentLocation` _asbox_collision)))
      (`self.K2_SetActorLocation` (`KismetMathLibrary.MakeVector` _returnvalue_x_2 _returnvalue_y_2 _returnvalue_z))
      (set `self.FirstTime` false))
    (`KismetSystemLibrary.PrintText` (`|FormatText` "{pillar} In Collision with actor {name}" (`KismetSystemLibrary.GetObjectName` self) (`KismetSystemLibrary.GetDisplayName` _asbox_collision)) false false (struct :`G` 0.66 :`B` 1.0 :`A` 1.0) 50.0)))

(event `self.Box.OnComponentEndOverlap`
  (params (OverlappedComponent :type "PrimitiveComponent Object Reference") (OtherActor :type "Actor Object Reference") (OtherComp :type "PrimitiveComponent Object Reference") (OtherBodyIndex :type Integer))
  (if (and (not (`self.IsMoving?`)) (== (`GameplayStatics.GetObjectClass` OtherActor) "/Game/Blueprint/Player/BP_Player.BP_Player_C"))
    (`/Game/Blueprint/InteractiveObject/Pilar/BP_PilarManager.PilarSelection` (`self.PilarManager`) self true)))

(fn `DebugMovementPilar`
  (bind (_returnvalue_x _returnvalue_y _returnvalue_z) (`KismetMathLibrary.BreakVector` (`self.K2_GetActorLocation`)))
  (bind _alltargetlocation (`self.AllTargetLocation`))
  (bind _alltilesrefboxcolision (`/Game/Blueprint/InteractiveObject/Pilar/BP_CheckerBoard.AllTilesRefBoxColision` (`/Game/Blueprint/InteractiveObject/Pilar/BP_PilarManager.RefBoard` (`self.PilarManager`))))
  (bind _alltilesrefboxcolision_2 (`/Game/Blueprint/InteractiveObject/Pilar/BP_CheckerBoard.AllTilesRefBoxColision` (`/Game/Blueprint/InteractiveObject/Pilar/BP_PilarManager.RefBoard` (`self.PilarManager`))))
  (for (_ _array_index) _alltargetlocation
    (bind _keys (`BlueprintMapLibrary.Map_Keys` _alltilesrefboxcolision_2))
    (for _array_element _keys
      (if (== (`BlueprintMapLibrary.Map_Find` _alltilesrefboxcolision_2 _array_element) (`|GetArrayItem` (`self.AllTargetLocation`)))
        (if (== _array_index 0)
          (bind (_returnvalue_x_2 _returnvalue_y_2) (`KismetMathLibrary.BreakVector` (`SceneComponent.K2_GetComponentLocation` _array_element)))
          (bind _returnvalue (`KismetMathLibrary.MakeVector` _returnvalue_x_2 _returnvalue_y_2 _returnvalue_z))
          (`KismetSystemLibrary.LineTraceSingle` :`Start` (`KismetMathLibrary.MakeVector` _returnvalue_x _returnvalue_y _returnvalue_z) :`End` _returnvalue :`TraceChannel` "TraceTypeQuery2" :`DrawDebugType` "Persistent")
          (break)
          (else
            (bind _keys_2 (`BlueprintMapLibrary.Map_Keys` _alltilesrefboxcolision))
            (for _array_element_2 _keys_2
              (if (== (`BlueprintMapLibrary.Map_Find` _alltilesrefboxcolision _array_element_2) (`|GetArrayItem` _alltargetlocation (- _array_index 1)))
                (bind (_returnvalue_x_3 _returnvalue_y_3) (`KismetMathLibrary.BreakVector` (`SceneComponent.K2_GetComponentLocation` _array_element_2)))
                (`KismetSystemLibrary.LineTraceSingle` :`Start` (`KismetMathLibrary.MakeVector` _returnvalue_x_3 _returnvalue_y_3 _returnvalue_z) :`End` _returnvalue :`TraceChannel` "TraceTypeQuery2" :`DrawDebugType` "Persistent")
                (break)))))))))

(fn `Move`
  (locals (TileToGo :type "BoxComponent Object Reference"))
  (bind (_returnvalue_x _returnvalue_y _returnvalue_z) (`KismetMathLibrary.BreakVector` (`self.K2_GetActorLocation`)))
  (bind (_returnvalue_x_2 _returnvalue_y_2) (`KismetMathLibrary.BreakVector` (`SceneComponent.K2_GetComponentLocation` (`self.NextTileToGo`))))
  (bind _alltilesrefboxcolision (`/Game/Blueprint/InteractiveObject/Pilar/BP_CheckerBoard.AllTilesRefBoxColision` (`/Game/Blueprint/InteractiveObject/Pilar/BP_PilarManager.RefBoard` (`self.PilarManager`))))
  (`/Engine/EditorBlueprintResources/StandardMacros.IsValid` (`self.NextTileToGo`)
    (:`Is Valid`
      _)
    (:`Is Not Valid`
      (bind _keys (`BlueprintMapLibrary.Map_Keys` _alltilesrefboxcolision))
      (for _array_element _keys
        (if (== (`BlueprintMapLibrary.Map_Find` _alltilesrefboxcolision _array_element) (`|GetArrayItem` (`self.AllTargetLocation`)))
          (set `self.NextTileToGo` _array_element)
          (break)))))
  (`self.K2_SetActorLocation` (`KismetMathLibrary.VInterpTo` (`KismetMathLibrary.MakeVector` _returnvalue_x _returnvalue_y _returnvalue_z) (`KismetMathLibrary.MakeVector` _returnvalue_x_2 _returnvalue_y_2 _returnvalue_z) (`GameplayStatics.GetWorldDeltaSeconds`) (`self.MoveSpeed`))))

(fn `UserConstructionScript`
  (`parent.UserConstructionScript`))