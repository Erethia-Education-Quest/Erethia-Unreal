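; Manager for a pillar puzzle on a tile board: selecting two pillars makes them swap places.
; SwapPilar builds both routes with a recursive four-direction search that keeps the shortest path, then moves both if found.
; The second route checks the first to avoid collisions, and border tiles are avoided unless next to the goal or leaving a corner.
; CheckResult compares pillar coordinates to FinalPositionResult and sets IsCompleted on a match.
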(event `PilarSelection`
  (params (Pilar :type "/Game/Blueprint/InteractiveObject/Pilar/BP_Pilar Object Reference") (IsSelected :type Boolean))
  (bind _selectedpilar (`self.SelectedPilar`))
  (bind _selectedpilar_2 (`self.SelectedPilar`))
  (bind _selectedpilar_3 (`self.SelectedPilar`))
  (bind _output (`|GetArrayItem` _selectedpilar_2))
  (bind _output_2 (`|GetArrayItem` _selectedpilar_2 1))
  (if IsSelected
    (`/Game/Blueprint/InteractiveObject/Pilar/BP_Pilar.ChangeColor` Pilar (`self.BaseMaterial`))
    (`KismetArrayLibrary.Array_RemoveItem` _selectedpilar Pilar)
    (else
      (`/Game/Blueprint/InteractiveObject/Pilar/BP_Pilar.ChangeColor` Pilar (`self.SelectedMaterial`))
      (`KismetArrayLibrary.Array_Add` _selectedpilar Pilar)
      (if (== (`KismetArrayLibrary.Array_Length` _selectedpilar) 2)
        (`KismetSystemLibrary.PrintText` (`|FormatText` "Tile {x} is close to goal {y}" (`KismetSystemLibrary.GetObjectName` _output) (`KismetSystemLibrary.GetObjectName` _output_2)) true true (struct :`G` 0.66 :`B` 1.0 :`A` 1.0) 5.0)
        (set `/Game/Blueprint/InteractiveObject/Pilar/BP_Pilar.IsMoving?` true _output)
        (set `/Game/Blueprint/InteractiveObject/Pilar/BP_Pilar.IsMoving?` true _output_2)
        (`self.SwapPilar` _output _output_2)
        (for _array_element _selectedpilar_3
          (`/Game/Blueprint/InteractiveObject/Pilar/BP_Pilar.ChangeColor` _array_element (`self.BaseMaterial`)))
        (`KismetArrayLibrary.Array_Clear` _selectedpilar_3)))))

(fn `AllowBypassDeadEnd?`
  (params (StartPos :type "Vector2D Structure"))
  (returns (`CanByPass?` :type Boolean))
  (return (and (or (== StartPos_X (- (`/Game/Blueprint/InteractiveObject/Pilar/BP_CheckerBoard.NbrBoxByLine` (`self.RefBoard`)) 1)) (== StartPos_X 0.0)) (or (== StartPos_Y 0.0) (== StartPos_Y (- (`/Game/Blueprint/InteractiveObject/Pilar/BP_CheckerBoard.NbrBoxByRow` (`self.RefBoard`)) 1))))))

(fn `Check Path`
  (params (`CanPass?` :type Boolean) (PathToFollow :type "Array of Vector2D Structure") (`ByPassDeadEnd?` :type Boolean) (AlreadyExistingPath :type "Array of Vector2D Structure") (CurrentPos :type "Vector2D Structure") (TileToCheck :type "Vector2D Structure") (Goal :type "Vector2D Structure"))
  (returns (ResultPath :type "Array of Vector2D Structure"))
  (locals (FollowingPath :type "Array of Vector2D Structure"))
  (set `local.FollowingPath` PathToFollow)
  (if (not `ByPassDeadEnd?`)
    (bind _deadend_ (`self.CheckDontGoDeadEnd` TileToCheck Goal))
    (if (and `CanPass?` (not _deadend_))
      _
      (else
        (return (`local.FollowingPath`)))))
  (bind _canpass_ (`self.CheckTileAvalaible` (`local.CurrentPos`) (`local.FollowingPath`) (`local.TileToCheck`) (`local.AlreadyExistingPath`)))
  (if _canpass_
    (`KismetArrayLibrary.Array_Add` (`local.FollowingPath`) (`local.TileToCheck`))
    (bind _pathfound (`self.FindPathForPilar` (`local.TileToCheck`) (`local.Goal`) (`local.FollowingPath`) (`local.AlreadyExistingPath`)))
    (if (not (!= (`|GetArrayItem` _pathfound (- (`KismetArrayLibrary.Array_Length` _pathfound) 1)) (`local.Goal`)))
      (bind _shorterpath (`self.CheckNewPathIsShorterThanPreviousOne` _pathfound (`local.FollowingPath`) (`local.Goal`)))
      (set `local.FollowingPath` _shorterpath))
    (return (`local.FollowingPath`))
    (else
      (return (`local.FollowingPath`)))))

(fn `CheckDontGoDeadEnd`
  (params (TileToCheck :type "Vector2D Structure") (Goal :type "Vector2D Structure"))
  (returns (`DeadEnd?` :type Boolean))
  (if (or (== TileToCheck_X 0.0) (== TileToCheck_X (- (`/Game/Blueprint/InteractiveObject/Pilar/BP_CheckerBoard.NbrBoxByLine` (`self.RefBoard`)) 1)) (== TileToCheck_Y 0.0) (== TileToCheck_Y (- (`/Game/Blueprint/InteractiveObject/Pilar/BP_CheckerBoard.NbrBoxByRow` (`self.RefBoard`)) 1)))
    (bind _pathfound_ (`self.CheckNextTileIsGoal` (`local.TileToCheck`) (`local.Goal`)))
    (return (not _pathfound_))
    (else
      (return false))))

(fn `CheckNewPathIsShorterThanPreviousOne`
  (params (NewPath :type "Array of Vector2D Structure") (OldPath :type "Array of Vector2D Structure") (Goal :type "Vector2D Structure"))
  (returns (ShorterPath :type "Array of Vector2D Structure"))
  (if (`KismetArrayLibrary.Array_Contains` NewPath Goal)
    (if (`KismetArrayLibrary.Array_Contains` (`local.OldPath`) (`local.Goal`))
      (if (> (`KismetArrayLibrary.Array_Length` (`local.OldPath`)) (`KismetArrayLibrary.Array_Length` (`local.NewPath`)))
        (return (`local.NewPath`))
        (else
          (return (`local.OldPath`))))
      (else
        (return (`local.NewPath`))))
    (else
      (return (`local.OldPath`)))))

(fn `CheckNextTileIsGoal`
  (params (CurrentTile :type "Vector2D Structure") (Goal :type "Vector2D Structure"))
  (returns (`PathFound?` :type Boolean))
  (bind (_x _y) (`KismetMathLibrary.BreakVector2D` CurrentTile))
  (bind _currenttile_x (`KismetMathLibrary.BreakVector2D` (`local.CurrentTile`)))
  (bind (_currenttile_x_2 _currenttile_y) (`KismetMathLibrary.BreakVector2D` (`local.CurrentTile`)))
  (bind (_currenttile_x_3 _currenttile_y_2) (`KismetMathLibrary.BreakVector2D` (`local.CurrentTile`)))
  (bind _returnvalue (`KismetMathLibrary.MakeVector2D` (- _x 1.0) _currenttile_y))
  (bind _returnvalue_2 (`KismetMathLibrary.MakeVector2D` (+ _x 1.0) _currenttile_y_2))
  (bind _returnvalue_3 (`KismetMathLibrary.MakeVector2D` _currenttile_x_3 (+ _y 1.0)))
  (bind _returnvalue_4 (`KismetMathLibrary.MakeVector2D` _currenttile_x (- _y 1.0)))
  (`|ExecutionSequence`
    (:`then_0`
      (if (== _returnvalue (`local.Goal`))
        (`KismetSystemLibrary.PrintText` (`|FormatText` "Tile {x} is close to goal {y}" (`KismetStringLibrary.Conv_Vector2dToString` (`local.CurrentTile`)) (`KismetStringLibrary.Conv_Vector2dToString` (`local.Goal`))) false false :!label _label)
        (return true)))
    (:`then_1`
      (if (== _returnvalue_2 (`local.Goal`))
        (goto _label)))
    (:`then_2`
      (if (== _returnvalue_3 (`local.Goal`))
        (goto _label)))
    (:`then_3`
      (if (== _returnvalue_4 (`local.Goal`))
        (goto _label)))
    (:`then_4`
      (`KismetSystemLibrary.PrintText` (`|FormatText` "Tile {x} isn't close to goal {y} \nVectorChecked are: \n{a} \n{b} \n{c} \n{d}" (`KismetStringLibrary.Conv_Vector2dToString` (`local.CurrentTile`)) (`KismetStringLibrary.Conv_Vector2dToString` (`local.Goal`)) (`KismetStringLibrary.Conv_Vector2dToString` _returnvalue) (`KismetStringLibrary.Conv_Vector2dToString` _returnvalue_2) (`KismetStringLibrary.Conv_Vector2dToString` _returnvalue_3) (`KismetStringLibrary.Conv_Vector2dToString` _returnvalue_4)) false false)
      (return false))))

(fn `CheckResult`
  (returns (NewParam :type Boolean))
  (locals (Increment :type Integer))
  (bind _finalpositionresult (`self.FinalPositionResult`))
  (bind _keys (`BlueprintMapLibrary.Map_Keys` _finalpositionresult))
  (bind _values (`BlueprintMapLibrary.Map_Values` _finalpositionresult))
  (for (_array_element _array_index) _keys
    (bind _currenttilecoord (`/Game/Blueprint/InteractiveObject/Pilar/BP_Pilar.CurrentTileCoord` _array_element))
    (bind _output (`|GetArrayItem` _values _array_index))
    (if (not (and (== (`KismetMathLibrary.GetMin2D` _currenttilecoord) (`KismetMathLibrary.GetMin2D` _output)) (== (`KismetMathLibrary.GetMax2D` _currenttilecoord) (`KismetMathLibrary.GetMax2D` _output))))
      (return false)))
  (set `self.IsCompleted?` true)
  (return true))

(fn `CheckTileAvalaible`
  (params (CurrentPos :type "Vector2D Structure") (PathAlreadyTaken :type "Array of Vector2D Structure") (TileToCheck :type "Vector2D Structure") (AlreadyExistingPath :type "Array of Vector2D Structure"))
  (returns (`CanPass?` :type Boolean))
  (bind _returnvalue (`KismetArrayLibrary.Array_Find` (`local.AlreadyExistingPath`) (`local.TileToCheck`)))
  (bind (_value _returnvalue_2) (`BlueprintMapLibrary.Map_Find` (`/Game/Blueprint/InteractiveObject/Pilar/BP_CheckerBoard.AllTIles` (`self.RefBoard`)) TileToCheck))
  (if (or (`KismetArrayLibrary.Array_Contains` PathAlreadyTaken TileToCheck) (and _value _returnvalue_2))
    (return false)
    (elif (`KismetArrayLibrary.Array_Contains` (`local.AlreadyExistingPath`) (`local.TileToCheck`))
      (if (or (== (`|GetArrayItem` (`local.AlreadyExistingPath`) (+ _returnvalue 0)) (`local.CurrentPos`)) (== _returnvalue (`KismetArrayLibrary.Array_Length` (`local.PathAlreadyTaken`))))
        (return false)
        (else
          (return true)))
      (else
        (return true)))))

(fn `FindPathForPilar`
  (params (Pos :type "Vector2D Structure") (Goal :type "Vector2D Structure") (CurrentPath :type "Array of Vector2D Structure") (AlreadyExistingPath :type "Array of Vector2D Structure") (`ByPassDeadEnd?` :type Boolean))
  (returns (PathFound :type "Array of Vector2D Structure"))
  (locals (PathToFollow :type "Array of Vector2D Structure") (TempPath :type "Array of Vector2D Structure") (ActualPos :type "Vector2D Structure"))
  (bind _actualpos_x (`KismetMathLibrary.BreakVector2D` (`local.ActualPos`)))
  (bind (_actualpos_x_2 _actualpos_y) (`KismetMathLibrary.BreakVector2D` (`local.ActualPos`)))
  (bind (_actualpos_x_3 _actualpos_y_2) (`KismetMathLibrary.BreakVector2D` (`local.ActualPos`)))
  (bind (_x _y) (`KismetMathLibrary.BreakVector2D` (`local.ActualPos`)))
  (bind _returnvalue (+ _x 1.0))
  (bind _returnvalue_2 (- _x 1.0))
  (bind _returnvalue_3 (+ _y 1.0))
  (bind _returnvalue_4 (- _y 1.0))
  (set `local.ActualPos` Pos)
  (set `local.PathToFollow` CurrentPath)
  (`|ExecutionSequence`
    (:`then_0`
      (bind _pathfound_ (`self.CheckNextTileIsGoal` (`local.ActualPos`) (`local.Goal`)))
      (if _pathfound_
        (`KismetArrayLibrary.Array_AddUnique` (`local.PathToFollow`) (`local.Goal`))
        (return (`local.PathToFollow`))))
    (:`then_1`
      (bind _resultpath (`self.Check Path` (`KismetMathLibrary.InRange_FloatFloat` _returnvalue_2 0.0 (`KismetMathLibrary.Conv_IntToDouble` (`/Game/Blueprint/InteractiveObject/Pilar/BP_CheckerBoard.NbrBoxByLine` (`self.RefBoard`))) true false) (`local.PathToFollow`) (`local.ByPassDeadEnd?`) (`local.AlreadyExistingPath`) (`local.ActualPos`) (`KismetMathLibrary.MakeVector2D` _returnvalue_2 _actualpos_y) (`local.Goal`)))
      (bind _shorterpath (`self.CheckNewPathIsShorterThanPreviousOne` _resultpath (`local.TempPath`) (`local.Goal`)))
      (set `local.TempPath` _shorterpath))
    (:`then_2`
      (bind _resultpath_2 (`self.Check Path` (`KismetMathLibrary.InRange_FloatFloat` _returnvalue 0.0 (`KismetMathLibrary.Conv_IntToDouble` (`/Game/Blueprint/InteractiveObject/Pilar/BP_CheckerBoard.NbrBoxByLine` (`self.RefBoard`))) true false) (`local.PathToFollow`) (`local.ByPassDeadEnd?`) (`local.AlreadyExistingPath`) (`local.ActualPos`) (`KismetMathLibrary.MakeVector2D` _returnvalue _actualpos_y_2) (`local.Goal`)))
      (bind _shorterpath_2 (`self.CheckNewPathIsShorterThanPreviousOne` _resultpath_2 (`local.TempPath`) (`local.Goal`)))
      (set `local.TempPath` _shorterpath_2))
    (:`then_3`
      (bind _resultpath_3 (`self.Check Path` (`KismetMathLibrary.InRange_FloatFloat` _returnvalue_3 0.0 (`KismetMathLibrary.Conv_IntToDouble` (`/Game/Blueprint/InteractiveObject/Pilar/BP_CheckerBoard.NbrBoxByRow` (`self.RefBoard`))) true false) (`local.PathToFollow`) (`local.ByPassDeadEnd?`) (`local.AlreadyExistingPath`) (`local.ActualPos`) (`KismetMathLibrary.MakeVector2D` _actualpos_x_3 _returnvalue_3) (`local.Goal`)))
      (bind _shorterpath_3 (`self.CheckNewPathIsShorterThanPreviousOne` _resultpath_3 (`local.TempPath`) (`local.Goal`)))
      (set `local.TempPath` _shorterpath_3))
    (:`then_4`
      (bind _resultpath_4 (`self.Check Path` (`KismetMathLibrary.InRange_FloatFloat` _returnvalue_4 0.0 (`KismetMathLibrary.Conv_IntToDouble` (`/Game/Blueprint/InteractiveObject/Pilar/BP_CheckerBoard.NbrBoxByRow` (`self.RefBoard`))) true false) (`local.PathToFollow`) (`local.ByPassDeadEnd?`) (`local.AlreadyExistingPath`) (`local.ActualPos`) (`KismetMathLibrary.MakeVector2D` _actualpos_x _returnvalue_4) (`local.Goal`)))
      (bind _shorterpath_4 (`self.CheckNewPathIsShorterThanPreviousOne` _resultpath_4 (`local.TempPath`) (`local.Goal`)))
      (set `local.TempPath` _shorterpath_4))
    (:`then_5`
      (bind _shorterpath_5 (`self.CheckNewPathIsShorterThanPreviousOne` (`local.TempPath`) (`local.PathToFollow`) (`local.Goal`)))
      (return _shorterpath_5))))

(fn `SwapPilar`
  (params (Pilar1 :type "/Game/Blueprint/InteractiveObject/Pilar/BP_Pilar Object Reference") (Pilar2 :type "/Game/Blueprint/InteractiveObject/Pilar/BP_Pilar Object Reference"))
  (bind _currenttilecoord (`/Game/Blueprint/InteractiveObject/Pilar/BP_Pilar.CurrentTileCoord` Pilar2))
  (bind _currenttilecoord_2 (`/Game/Blueprint/InteractiveObject/Pilar/BP_Pilar.CurrentTileCoord` Pilar1))
  (bind _returnvalue (not (`KismetArrayLibrary.Array_IsEmpty` (`/Game/Blueprint/InteractiveObject/Pilar/BP_Pilar.AllTargetLocation` (`local.Pilar1`)))))
  (bind _returnvalue_2 (not (`KismetArrayLibrary.Array_IsEmpty` (`/Game/Blueprint/InteractiveObject/Pilar/BP_Pilar.AllTargetLocation` (`local.Pilar2`)))))
  (`|ExecutionSequence`
    (:`then_0`
      (bind _canbypass_ (`self.AllowBypassDeadEnd?` _currenttilecoord_2))
      (bind _pathfound (`self.FindPathForPilar` :`Pos` _currenttilecoord_2 :`Goal` (`/Game/Blueprint/InteractiveObject/Pilar/BP_Pilar.CurrentTileCoord` Pilar2) :`CurrentPath` (`|MakeArray` _currenttilecoord_2) :`ByPassDeadEnd?` _canbypass_))
      (set `/Game/Blueprint/InteractiveObject/Pilar/BP_Pilar.AllTargetLocation` _pathfound (`local.Pilar1`)))
    (:`then_1`
      (bind _canbypass__2 (`self.AllowBypassDeadEnd?` _currenttilecoord))
      (bind _pathfound_2 (`self.FindPathForPilar` _currenttilecoord (`/Game/Blueprint/InteractiveObject/Pilar/BP_Pilar.CurrentTileCoord` Pilar1) (`|MakeArray` _currenttilecoord) (`/Game/Blueprint/InteractiveObject/Pilar/BP_Pilar.AllTargetLocation` Pilar1) _canbypass__2))
      (set `/Game/Blueprint/InteractiveObject/Pilar/BP_Pilar.AllTargetLocation` _pathfound_2 (`local.Pilar2`)))
    (:`then_2`
      (if (and _returnvalue _returnvalue_2)
        (`|ExecutionSequence`
          (:`then_0`
            (`/Game/Blueprint/InteractiveObject/Pilar/BP_Pilar.MoveTo` (`local.Pilar1`)))
          (:`then_1`
            (`/Game/Blueprint/InteractiveObject/Pilar/BP_Pilar.MoveTo` (`local.Pilar2`))))
        (else
          (`KismetSystemLibrary.PrintText` (`|FormatText` "Path For Pilar 1 IsEmpty? = {v} \nPath For Pilar 2 IsEmpty? = {c}" _returnvalue _returnvalue_2) false false (struct :`R` 1.0 :`B` 0.038177 :`A` 1.0) 10.0))))))

(fn `UserConstructionScript`
  (`parent.UserConstructionScript`))