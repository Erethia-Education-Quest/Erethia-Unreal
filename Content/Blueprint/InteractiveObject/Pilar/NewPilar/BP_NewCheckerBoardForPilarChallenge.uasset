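; Checkerboard for the pillar challenge that builds a tile grid labelled by Season and Ritual decals and tracks correctly solved pillars.
; CreationTiles spawns the grid and adds wall decals at every other row and column along two edges.
; On BeginPlay, each linked pillar gets one Season-Ritual pair from its array index via division and modulo.
; CheckPointState tallies correct pillars by season tag, firing each season's voice once when its count matches the Ritual count.
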(event `self.ReceiveBeginPlay`
  (`self.SetDecalOnPilar`))

(fn `CheckPointState`
  (locals (Season1GoodPilar :type "Float (double-precision)") (Season2GoodPilar :type "Float (double-precision)") (Season3GoodPilar :type "Float (double-precision)"))
  (bind _returnvalue (`KismetArrayLibrary.Array_Length` (`self.Ritual`)))
  (for _array_element (`self.CurrentlyCorrectPilars`)
    (bind _tagpilar (`/Game/Blueprint/InteractiveObject/Pilar/NewPilar/BP_NewPilar.TagPilar` _array_element))
    (if (`|EnumEquality` (enumliteral `/Game/Enum/E_PossiblePilarType` "NewEnumerator0") _tagpilar)
      (`/Engine/EditorBlueprintResources/StandardMacros.IncrementFloat` (`local.Season1GoodPilar`))
      (elif (`|EnumEquality` (enumliteral `/Game/Enum/E_PossiblePilarType` "NewEnumerator1") _tagpilar)
        (`/Engine/EditorBlueprintResources/StandardMacros.IncrementFloat` (`local.Season2GoodPilar`))
        (elif (`|EnumEquality` _tagpilar (enumliteral `/Game/Enum/E_PossiblePilarType` "NewEnumerator2"))
          (`/Engine/EditorBlueprintResources/StandardMacros.IncrementFloat` (`local.Season3GoodPilar`))))))
  (`|ExecutionSequence`
    (:`then_0`
      (if (`self.Season1PlayedSound`)
        _
        (elif (== (`local.Season1GoodPilar`) _returnvalue)
          (set `self.Season1PlayedSound` true)
          (`self.AtActivation` (`self.VoiceSeason1`)))))
    (:`then_1`
      (if (`self.Season2PlayedSound`)
        _
        (elif (== _returnvalue (`local.Season2GoodPilar`))
          (set `self.Season2PlayedSound` true)
          (`self.AtActivation` (`self.VoiceSeason2`)))))
    (:`then_2`
      (if (`self.Season3PlayedSound`)
        _
        (elif (== _returnvalue (`local.Season3GoodPilar`))
          (set `self.Season3PlayedSound` true)
          (`self.AtActivation` (`self.VoiceSeason3`)))))))

(fn `CreationTiles`
  (bind _materialindex (`self.MaterialIndex`))
  (bind _materialindex2 (`self.MaterialIndex2`))
  (bind (_currentlocation_0_x _currentlocation_0_y _currentlocation_0_z) (`KismetMathLibrary.BreakVector` (`self.CurrentLocation_0`)))
  (bind (_currentlocation_0_x_2 _currentlocation_0_y_2 _currentlocation_0_z_2) (`KismetMathLibrary.BreakVector` (`self.CurrentLocation_0`)))
  (bind (_returnvalue_x _returnvalue_y) (`KismetMathLibrary.BreakVector2D` (+ (`self.Actual Created Tile`) (0.0 1.0))))
  (for _index (range (`self.NbrBoxByRow`))
    (for _index_2 (range (`self.NbrBoxByLine`))
      (`self.SpawnAndSetUp`)
      (bind _output_get (set `self.CurrentLocation_0` (`KismetMathLibrary.MakeVector` (+ _currentlocation_0_x (* (`self.SizeX`) 2.0)) _currentlocation_0_y _currentlocation_0_z)))
      (if (and (== (mod _index 2) 0) (== _index_2 0))
        (`self.PutDecalOnWall` _output_get (`|GetArrayItem` (`self.Season`) _materialindex))
        (`/Engine/EditorBlueprintResources/StandardMacros.IncrementInt` _materialindex
          (:`  `
            _)))
      (if (and (== _index 0) (== (mod _index_2 2) 0))
        (`self.PutDecalOnWall` _output_get (`|GetArrayItem` (`self.Ritual`) _materialindex2) true)
        (`/Engine/EditorBlueprintResources/StandardMacros.IncrementInt` _materialindex2
          (:`  `
            _)))
      (set `self.Actual Created Tile` (+ (`self.Actual Created Tile`) (1.0 0.0))))
    (set `self.CurrentLocation_0` (`KismetMathLibrary.MakeVector` _currentlocation_0_x_2 (+ _currentlocation_0_y_2 (* (`self.SizeY`) 2.0)) _currentlocation_0_z_2))
    (`self.ResetX`)
    (set `self.Actual Created Tile` (`KismetMathLibrary.MakeVector2D` 0.0 _returnvalue_y))))

(fn `PutDecalOnWall`
  (params (TilePos :type "Vector Structure") (Material :type "MaterialInterface Object Reference") (Turn :type Boolean))
  (bind _decalscale (`self.DecalScale`))
  (bind (_decalrotation_roll _decalrotation_pitch _decalrotation_yaw) (`KismetMathLibrary.BreakRotator` (`self.DecalRotation`)))
  (if Turn
    (bind _returnvalue (`AddComponent|NODE_AddDecalComponent-0` :`RelativeTransform` (`KismetMathLibrary.MakeTransform` (+ TilePos (`KismetMathLibrary.MakeVector` (* (`self.SizeX`) -2.0) (`self.DecalDistanceFixX`))) (`KismetMathLibrary.MakeRotator` _decalrotation_roll _decalrotation_pitch _decalrotation_yaw) _decalscale)))
    (`DecalComponent.SetDecalMaterial` _returnvalue Material)
    (else
      (bind _returnvalue_2 (`AddComponent|NODE_AddDecalComponent-1` :`RelativeTransform` (`KismetMathLibrary.MakeTransform` (+ TilePos (`KismetMathLibrary.MakeVector` (`self.DecalDistanceFixY`))) (`KismetMathLibrary.MakeRotator` _decalrotation_roll _decalrotation_pitch (+ _decalrotation_yaw 90.0)) _decalscale)))
      (`DecalComponent.SetDecalMaterial` _returnvalue_2 Material))))

(fn `SetDecalOnPilar`
  (bind _ritual (`self.Ritual`))
  (bind _returnvalue (`KismetArrayLibrary.Array_Length` _ritual))
  (for (_array_element _array_index) (`self.AllLinkPilars`)
    (`/Game/Blueprint/InteractiveObject/Pilar/NewPilar/BP_NewPilar.SetDecalSeason` _array_element (`|GetArrayItem` (`self.Season`) (/ _array_index _returnvalue)))
    (`/Game/Blueprint/InteractiveObject/Pilar/NewPilar/BP_NewPilar.SetDecalRitual` _array_element (`|GetArrayItem` _ritual (mod _array_index _returnvalue)))))

(fn `UserConstructionScript`
  (`parent.UserConstructionScript`))