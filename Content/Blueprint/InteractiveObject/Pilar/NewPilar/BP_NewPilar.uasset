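; Networked interactive pillar that players select by hand overlap and that slides along a tile path, with settable season and ritual decals.
; The authority registers selection with RefChecker, swaps the highlight material, and relays select, unselect and move to each player controller through GS_Game.
; Movement runs a Timeline lerp between successive checker tiles, recursing until the path is consumed while an attached sound re-spawns to loop.
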(event `self.ReceiveBeginPlay`
  (`parent.ReceiveBeginPlay`)
  (`|ExecutionSequence`
    (:`then_0`
      (bind _asbp_game_instance (cast `/Game/Blueprint/GameInstance/BP_GameInstance` (`GameplayStatics.GetGameInstance`)))
      (set `self.RefGI_0` _asbp_game_instance))
    (:`then_1`
      (bind _asgs_game (cast `/Game/Blueprint/GameState/GS_Game` (`GameplayStatics.GetGameState`)))
      (set `self.RefGS_0` _asgs_game))
    (:`then_2`
      (set `self.NotSelectedMaterial` (`PrimitiveComponent.GetMaterial` (`self.Object`) 0)))
    (:`then_3`
      (`KismetSystemLibrary.Delay` 0.2)
      (set `self.StartPosition` (`self.K2_GetActorLocation`))
      (`self.K2_SetActorLocation` (0.0 0.0 0.0))
      (`self.K2_SetActorLocation` (`self.StartPosition`)))))

(event `self.Capsule.OnComponentBeginOverlap`
  (params (OverlappedComponent :type "PrimitiveComponent Object Reference") (OtherActor :type "Actor Object Reference") (OtherComp :type "PrimitiveComponent Object Reference") (OtherBodyIndex :type Integer) (bFromSweep :type Boolean) (SweepResult :type "HitResult Structure (by ref)"))
  (if (and (`self.HasAuthority`) (`ActorComponent.ComponentHasTag` OtherComp "Hand") (not (`self.IsMoving?`)))
    (`self.SelectedPilarServer`)
    (`/Engine/EditorBlueprintResources/StandardMacros.IsValid` (`self.RefGS_0`)
      (:`Is Valid`
        (bind _refgi_0 (`self.RefGI_0`)
          (:`then`
            (for _array_element (`/Game/Blueprint/GameInstance/BP_GameInstance.ListPlayerInfo` _refgi_0)
              (bind _aspc_game (cast `/Game/Blueprint/PlayerController/PC_Game` (`.PC_11_776544A84872013AA63BC881D8B483A2` (break `/Game/Struct/S_PlayerInfo` _array_element))))
              (`/Game/Blueprint/GameState/GS_Game.SelectedPilarClient` (`self.RefGS_0`) _aspc_game self)))
          (:`else`))))))

(event `self.Capsule.OnComponentEndOverlap`
  (params (OverlappedComponent :type "PrimitiveComponent Object Reference") (OtherActor :type "Actor Object Reference") (OtherComp :type "PrimitiveComponent Object Reference") (OtherBodyIndex :type Integer))
  (if (and (`self.HasAuthority`) (`ActorComponent.ComponentHasTag` OtherComp "Hand"))
    (`self.UnselectedPilarServer`)
    (`/Engine/EditorBlueprintResources/StandardMacros.IsValid` (`self.RefGS_0`)
      (:`Is Valid`
        (bind _refgi_0 (`self.RefGI_0`)
          (:`then`
            (for _array_element (`/Game/Blueprint/GameInstance/BP_GameInstance.ListPlayerInfo` _refgi_0)
              (bind _aspc_game (cast `/Game/Blueprint/PlayerController/PC_Game` (`.PC_11_776544A84872013AA63BC881D8B483A2` (break `/Game/Struct/S_PlayerInfo` _array_element))))
              (`/Game/Blueprint/GameState/GS_Game.UnselectedPilarClient` (`self.RefGS_0`) _aspc_game self)))
          (:`else`))))))

(event `SelectedPilarServer`
  (bind _refchecker (`self.RefChecker`)
    (:`then`
      (`/Game/Blueprint/InteractiveObject/Pilar/NewPilar/BP_NewCheckerBoard.AddPilarToBeMovedServer` _refchecker self))
    (:`else`
      _))
  (set `self.IsSelected?` true :!label _label)
  (`PrimitiveComponent.SetMaterial` (`self.Object`) 0 (`self.SelectedMaterial`)))

(event `SelectedPilarClient`
  (goto _label))

(event `UnselectedPilarServer`
  (bind _refchecker (`self.RefChecker`)
    (:`then`
      (`/Game/Blueprint/InteractiveObject/Pilar/NewPilar/BP_NewCheckerBoard.RemovePilarToBeMovedServer` _refchecker self))
    (:`else`
      _))
  (set `self.IsSelected?` true :!label _label_2)
  (`PrimitiveComponent.SetMaterial` (`self.Object`) 0 (`self.NotSelectedMaterial`)))

(event `UnselectedPilarClient`
  (goto _label_2))

(event `MovePilarServer`
  (`/Engine/EditorBlueprintResources/StandardMacros.IsValid` (`self.RefGS_0`)
    (:`Is Valid`
      (bind _refgi_0 (`self.RefGI_0`)
        (:`then`
          (for _array_element (`/Game/Blueprint/GameInstance/BP_GameInstance.ListPlayerInfo` _refgi_0)
            (bind _aspc_game (cast `/Game/Blueprint/PlayerController/PC_Game` (`.PC_11_776544A84872013AA63BC881D8B483A2` (break `/Game/Struct/S_PlayerInfo` _array_element))))
            (`/Game/Blueprint/GameState/GS_Game.MovePilarClient` (`self.RefGS_0`) _aspc_game self (`self.AllTargetLocation`)))
          (`/Engine/EditorBlueprintResources/StandardMacros.IsValid` (`self.RefChecker`) :!label _label_3
            (:`Is Valid`
              (`self.MovePilar`))))
        (:`else`)))))

(event `MovePilarClient`
  (params (AllTargetLocation :type "Array of Vector2D Structure"))
  (set `self.AllTargetLocation` AllTargetLocation)
  (goto _label_3))

(event `SetDecalSeason`
  (params (Material :type "MaterialInterface Object Reference"))
  (`DecalComponent.SetDecalMaterial` (`self.DecalSeason`) Material))

(event `SetDecalRitual`
  (params (Material :type "MaterialInterface Object Reference"))
  (`DecalComponent.SetDecalMaterial` (`self.DecalRitual`) Material))

(event `PlayLoopSound`
  (if (not (`self.IsMoving?`))
    (bind _returnvalue (`GameplayStatics.SpawnSoundAttached` (`self.PilarSound`) (`self.Object`) "None" (0.0 0.0 0.0) (struct) "KeepRelativeOffset" true 0.1 1.0 0.0 "/Game/Blueprint/InteractiveObject/Sound/SoundAttenuation/BP_SoundAttenuationVoice.BP_SoundAttenuationVoice" null :!label _label_4))
    (bind _output_get (set `self.LoopSoundRef` _returnvalue))
    (clear `AudioComponent.OnAudioFinished` _output_get)
    (add `AudioComponent.OnAudioFinished` _output_get (delegate `OnAudioFinished_Event`))))

(event `OnAudioFinished_Event`
  (`self.Again`))

(event `Again`
  (goto _label_4))

(event `StopLoopSound`
  (bind _loopsoundref (`self.LoopSoundRef`))
  (clear `AudioComponent.OnAudioFinished` _loopsoundref)
  (`AudioComponent.Stop` _loopsoundref))

(event `MovePilar`
  (bind (_returnvalue_x _returnvalue_y _returnvalue_z) (`KismetMathLibrary.BreakVector` (`self.K2_GetActorLocation`)))
  (bind (_returnvalue_x_2 _returnvalue_y_2 _returnvalue_z_2) (`KismetMathLibrary.BreakVector` (`self.K2_GetActorLocation`)))
  (if (> (`KismetArrayLibrary.Array_Length` (`self.AllTargetLocation`)) 1)
    (`self.PlayLoopSound`)
    (set `self.IsMoving?` true)
    (bind (_direction _distancetotravel) (`Timeline|Timeline` :!via `PlayFromStart`)
      (:`Update`
        (bind _tile (`/Game/Blueprint/InteractiveObject/Pilar/NewPilar/BP_NewCheckerBoard.GetTileAtPosition` (`self.RefChecker`) (`|GetArrayItem` (`self.AllTargetLocation`))))
        (bind _tile_2 (`/Game/Blueprint/InteractiveObject/Pilar/NewPilar/BP_NewCheckerBoard.GetTileAtPosition` (`self.RefChecker`) (`|GetArrayItem` (`self.AllTargetLocation`) 1)))
        (bind (_returnvalue_x_3 _returnvalue_y_3) (`KismetMathLibrary.BreakVector` (`SceneComponent.K2_GetComponentLocation` _tile)))
        (bind (_returnvalue_x_4 _returnvalue_y_4) (`KismetMathLibrary.BreakVector` (`SceneComponent.K2_GetComponentLocation` _tile_2)))
        (`self.K2_SetActorLocation` (`KismetMathLibrary.VLerp` (`KismetMathLibrary.MakeVector` _returnvalue_x_3 _returnvalue_y_3 _returnvalue_z_2) (`KismetMathLibrary.MakeVector` _returnvalue_x_4 _returnvalue_y_4 _returnvalue_z) _distancetotravel)))
      (:`Finished`
        (`KismetArrayLibrary.Array_Remove` (`self.AllTargetLocation`))
        (`self.MovePilar`)))
    (else
      (set `self.IsMoving?` false)
      (`self.StopLoopSound`))))

(fn `UserConstructionScript`
  (`parent.UserConstructionScript`))