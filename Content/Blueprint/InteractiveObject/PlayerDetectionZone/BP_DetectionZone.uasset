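; BP_DetectionZone is an interactive zone that tracks how many BP_Player actors stand inside its box and sets a completion state from that count.
; Box begin overlap increments the count on the authority only and sets complete when it reaches NbPlayerTarget.
; End overlap decrements it without an authority check and clears completion only when the reduced count equals that target, not when it falls below.
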(event `self.Box.OnComponentBeginOverlap`
  (params (OverlappedComponent :type "PrimitiveComponent Object Reference") (OtherActor :type "Actor Object Reference") (OtherComp :type "PrimitiveComponent Object Reference") (OtherBodyIndex :type Integer) (bFromSweep :type Boolean) (SweepResult :type "HitResult Structure (by ref)"))
  (if (and (== (`GameplayStatics.GetObjectClass` OtherActor) "/Game/Blueprint/Player/BP_Player.BP_Player_C") (`self.HasAuthority`))
    (bind _output_get (set `self.PlayerInZone` (+ (`self.PlayerInZone`) 1)))
    (if (== _output_get (`self.NbPlayerTarget`))
      (`self.ChangeCompleteState` true))))

(event `self.Box.OnComponentEndOverlap`
  (params (OverlappedComponent :type "PrimitiveComponent Object Reference") (OtherActor :type "Actor Object Reference") (OtherComp :type "PrimitiveComponent Object Reference") (OtherBodyIndex :type Integer))
  (if (== OtherActor "/Game/Blueprint/Player/BP_Player.BP_Player")
    (bind _output_get (set `self.PlayerInZone` (- (`self.PlayerInZone`) 1)))
    (if (== _output_get (`self.NbPlayerTarget`))
      (`self.ChangeCompleteState` false))))

(fn `UserConstructionScript`
  (`parent.UserConstructionScript`))