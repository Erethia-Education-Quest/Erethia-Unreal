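; BP_PlayAllSound is a networked sound player that queues sounds and plays them in turn, attached to its static mesh with voice attenuation.
; Each finished sound leaves the queue, and the next starts after a short delay.
; Add, stop and clear requests run server events, then reach each player in the GameInstance list through GS_Game client calls.
; ForcePlay clears the queue and plays the new sound immediately.
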(event `self.ReceiveBeginPlay`
  (bind _asbp_game_instance (cast `/Game/Blueprint/GameInstance/BP_GameInstance` (`GameplayStatics.GetGameInstance`)))
  (set `self.Ref_GI` _asbp_game_instance)
  (bind _asgs_game (cast `/Game/Blueprint/GameState/GS_Game` (`GameplayStatics.GetGameState`)))
  (set `self.Ref_GS` _asgs_game))

(event `StopSound`
  ;[1 1 1] StopSound
  (`self.StopSoundNetwork`))

(event `OnAudioFinished_Event`
  (set `self.IsPlaying` false)
  (`KismetArrayLibrary.Array_Remove` (`self.SoundList`))
  (`KismetSystemLibrary.Delay` 2.0)
  (`self.PlaySound`))

(event `StopSoundNetwork`
  (bind _ref_gi (`self.Ref_GI`))
  (bind _ref_gs (`self.Ref_GS`))
  ;[1 1 1] StopSound
  (`self.StopSoundServer`)
  (if (and (`KismetSystemLibrary.IsValid` _ref_gi) (`KismetSystemLibrary.IsValid` _ref_gs))
    (for _array_element (`/Game/Blueprint/GameInstance/BP_GameInstance.ListPlayerInfo` _ref_gi)
      (bind _aspc_game (cast `/Game/Blueprint/PlayerController/PC_Game` (`.PC_11_776544A84872013AA63BC881D8B483A2` (break `/Game/Struct/S_PlayerInfo` _array_element))))
      (`/Game/Blueprint/GameState/GS_Game.StopSoundClient` _ref_gs _aspc_game self))))

(event `PlaySound`
  (if (`self.IsPlaying`)
    _
    (elif (> (`KismetArrayLibrary.Array_Length` (`self.SoundList`)) 0)
      (bind _returnvalue (`GameplayStatics.SpawnSoundAttached` (`|GetArrayItem` (`self.SoundList`)) (`self.StaticMesh`) "None" (0.0 0.0 0.0) (struct) "KeepRelativeOffset" true 0.2 1.0 0.0 "/Game/Blueprint/InteractiveObject/Sound/SoundAttenuation/BP_SoundAttenuationVoice.BP_SoundAttenuationVoice" null))
      (bind _output_get (set `self.PlaySoundRef` _returnvalue))
      (clear `AudioComponent.OnAudioFinished` _output_get)
      (add `AudioComponent.OnAudioFinished` _output_get (delegate `OnAudioFinished_Event`))
      (set `self.IsPlaying` true))))

(event `StopSoundServer`
  (bind _playsoundref (`self.PlaySoundRef`))
  ;[1 1 1] StopSound
  (`/Engine/EditorBlueprintResources/StandardMacros.IsValid` _playsoundref
    (:`Is Valid`
      (`AudioComponent.Stop` _playsoundref)
      (set `self.IsPlaying` false)
      (`KismetArrayLibrary.Array_Remove` (`self.SoundList`)))))

(event `StopSoundClient`
  (bind _playsoundref (`self.PlaySoundRef`))
  ;[1 1 1] StopSound
  (`/Engine/EditorBlueprintResources/StandardMacros.IsValid` _playsoundref
    (:`Is Valid`
      (`AudioComponent.Stop` _playsoundref)
      (set `self.IsPlaying` false)
      (`KismetArrayLibrary.Array_Remove` (`self.SoundList`)))))

(event `AddSoundToList`
  (params (NewSound :type "SoundBase Object Reference") (ForcePlay :type Boolean))
  ;[1 1 1] AddSoundToList
  (`self.AddSoundToListNetwork` NewSound ForcePlay))

(event `ClearSound`
  ;[1 1 1] ClearSound
  (`self.ClearSoundNetwork`))

(event `ClearSoundNetwork`
  (bind _ref_gi (`self.Ref_GI`))
  (bind _ref_gs (`self.Ref_GS`))
  ;[1 1 1] ClearSound
  (`self.ClearSoundServer`)
  (if (and (`KismetSystemLibrary.IsValid` _ref_gi) (`KismetSystemLibrary.IsValid` _ref_gs))
    (for _array_element (`/Game/Blueprint/GameInstance/BP_GameInstance.ListPlayerInfo` _ref_gi)
      (bind _aspc_game (cast `/Game/Blueprint/PlayerController/PC_Game` (`.PC_11_776544A84872013AA63BC881D8B483A2` (break `/Game/Struct/S_PlayerInfo` _array_element))))
      (`/Game/Blueprint/GameState/GS_Game.ClearSoundClient` _ref_gs _aspc_game self))))

(event `AddSoundToListNetwork`
  (params (NewSound :type "SoundBase Object Reference") (ForcePlay :type Boolean))
  (bind _ref_gi (`self.Ref_GI`))
  (bind _ref_gs (`self.Ref_GS`))
  ;[1 1 1] AddSoundToList
  (`self.AddSoundToListServer` NewSound ForcePlay)
  (if (and (`KismetSystemLibrary.IsValid` _ref_gi) (`KismetSystemLibrary.IsValid` _ref_gs))
    (for _array_element (`/Game/Blueprint/GameInstance/BP_GameInstance.ListPlayerInfo` _ref_gi)
      (bind _aspc_game (cast `/Game/Blueprint/PlayerController/PC_Game` (`.PC_11_776544A84872013AA63BC881D8B483A2` (break `/Game/Struct/S_PlayerInfo` _array_element))))
      (`/Game/Blueprint/GameState/GS_Game.AddSoundToListClient` _ref_gs _aspc_game self NewSound ForcePlay))))

(event `ClearSoundServer`
  (bind _playsoundref (`self.PlaySoundRef`))
  ;[1 1 1] ClearSound
  (`KismetArrayLibrary.Array_Clear` (`self.SoundList`))
  (`/Engine/EditorBlueprintResources/StandardMacros.IsValid` _playsoundref
    (:`Is Valid`
      (`AudioComponent.Stop` _playsoundref))
    (:`Is Not Valid`
      _))
  (set `self.IsPlaying` false))

(event `AddSoundToListServer`
  (params (NewSound :type "SoundBase Object Reference") (ForcePlay :type Boolean))
  (bind _soundlist (`self.SoundList`))
  ;[1 1 1] AddSoundToList
  (if ForcePlay
    (`self.ClearSound`)
    (`KismetArrayLibrary.Array_AddUnique` _soundlist NewSound)
    (`self.PlaySound`)
    (else
      (`KismetArrayLibrary.Array_AddUnique` _soundlist NewSound)
      (`self.PlaySound`))))

(event `ClearSoundClient`
  (bind _playsoundref (`self.PlaySoundRef`))
  ;[1 1 1] ClearSound
  (`KismetArrayLibrary.Array_Clear` (`self.SoundList`))
  (`/Engine/EditorBlueprintResources/StandardMacros.IsValid` _playsoundref
    (:`Is Valid`
      (`AudioComponent.Stop` _playsoundref))
    (:`Is Not Valid`
      _))
  (set `self.IsPlaying` false))

(event `AddSoundToListClient`
  (params (NewSound :type "SoundBase Object Reference") (ForcePlay :type Boolean))
  (bind _soundlist (`self.SoundList`))
  ;[1 1 1] AddSoundToList
  (if ForcePlay
    (`self.ClearSound`)
    (`KismetArrayLibrary.Array_AddUnique` _soundlist NewSound)
    (`self.PlaySound`)
    (else
      (`KismetArrayLibrary.Array_AddUnique` _soundlist NewSound)
      (`self.PlaySound`))))

(fn `UserConstructionScript`)