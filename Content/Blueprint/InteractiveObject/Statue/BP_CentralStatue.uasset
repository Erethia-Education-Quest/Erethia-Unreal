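; Central statue puzzle object that turns its Cube toward the pedestal still awaiting activation, then toward its InteractWith target once all are active.
; It gathers every BP_Piedestal at BeginPlay and mirrors their on/off state through activation events.
; Once started, Tick reacts to a change flag, finds the first inactive pedestal, triggers its sound and rotates via MoveComponentTo.
; Deactivating any pedestal clears completion.
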(event `self.ReceiveBeginPlay`
  (`parent.ReceiveBeginPlay`)
  (bind _outactors (`GameplayStatics.GetAllActorsOfClass` "/Game/Blueprint/InteractiveObject/Piedestal/BP_Piedestal.BP_Piedestal_C"))
  (bind _output_get (set `self.AllPedestals` _outactors))
  (for _ _output_get
    (`KismetArrayLibrary.Array_Add` (`self.PiedestalsState`)))
  (set `self.HaveChanged` true)
  (`KismetSystemLibrary.PrintText` (`|FormatText` "Position pos status {pos}" (`KismetStringLibrary.Conv_VectorToString` (`self.K2_GetActorLocation`))) true true (struct :`R` 1.0 :`G` 0.75 :`A` 1.0) 10.0))

(event `OnPiedestalActivated`
  (params (piedestalIndex :type "/Game/Blueprint/InteractiveObject/Piedestal/BP_Piedestal Object Reference"))
  (for (_array_element _array_index) (`self.AllPedestals`)
    (if (== _array_element piedestalIndex)
      (`KismetArrayLibrary.Array_Set` (`self.PiedestalsState`) _array_index true)))
  (set `self.HaveChanged` true))

(event `OnPiedestalDesactivated`
  (params (piedestalIndex :type "/Game/Blueprint/InteractiveObject/Piedestal/BP_Piedestal Object Reference"))
  (for (_array_element _array_index) (`self.AllPedestals`)
    (if (== _array_element piedestalIndex)
      (`KismetArrayLibrary.Array_Set` (`self.PiedestalsState`) _array_index)))
  (set `self.HaveChanged` true)
  (set `self.IsCompleted?` false))

(event `self.ReceiveTick`
  (params (DeltaSeconds :type "Float (single-precision)"))
  (bind (_returnvalue_roll _returnvalue_pitch) (`KismetMathLibrary.BreakRotator` (`self.K2_GetActorRotation`)))
  (bind (_returnvalue_roll_2 _returnvalue_pitch_2) (`KismetMathLibrary.BreakRotator` (`self.K2_GetActorRotation`)))
  (bind _cube (`self.Cube`))
  (bind _cube_2 (`self.Cube`))
  (bind (_returnvalue_roll_3 _returnvalue_pitch_3 _returnvalue_yaw) (`KismetMathLibrary.BreakRotator` (`KismetMathLibrary.FindLookAtRotation` (`self.K2_GetActorLocation`) (`self.K2_GetActorLocation` (`self.InteractWith`)))))
  (if (`self.Start`)
    (if (`self.HaveChanged`)
      (if (`self.IsCompleted?`)
        (`self.PlayOBJSound` _cube_2)
        (set `self.HaveChanged` false)
        (`KismetSystemLibrary.MoveComponentTo` _cube_2 (`SceneComponent.RelativeLocation` _cube_2) (`KismetMathLibrary.MakeRotator` _returnvalue_roll_2 _returnvalue_pitch_2 (+ _returnvalue_yaw 180.0)) false false 4.3)
        (else
          (bind _output_get (set `self.NeedToBreak` false))
          (for (_array_element _array_index) (`self.PiedestalsState`)
            (if _output_get
              _
              (elif _array_element
                _
                (elif (== (`self.ActualIndexRotation`) _array_index)
                  (set `self.NeedToBreak` true)
                  (else
                    (set `self.ActualIndexRotation` _array_index)
                    (set `self.NeedToBreak` true)
                    (set `self.HaveChanged` false)
                    (`self.PlayOBJSound` _cube)
                    (bind _output (`|GetArrayItem` (`self.AllPedestals`) _array_index))
                    (`self.AtActivation` (`/Game/Blueprint/InteractiveObject/Piedestal/BP_Piedestal.SoundPlayer` _output))
                    (bind (_returnvalue_roll_4 _returnvalue_pitch_4 _returnvalue_yaw_2) (`KismetMathLibrary.BreakRotator` (`KismetMathLibrary.FindLookAtRotation` (`self.K2_GetActorLocation`) (`self.K2_GetActorLocation` _output))))
                    (`KismetSystemLibrary.MoveComponentTo` _cube (`SceneComponent.RelativeLocation` _cube) (`KismetMathLibrary.MakeRotator` _returnvalue_roll _returnvalue_pitch (+ _returnvalue_yaw_2 180.0)) false false 4.3)
                    (`self.StopSound`))))))
          (if (not _output_get)
            (set `self.HaveChanged` true)
            (`self.ChangeCompleteState` true)))))))

(event `self.AtActivation`
  (set `self.Start` true))

(fn `UserConstructionScript`
  (`parent.UserConstructionScript`))