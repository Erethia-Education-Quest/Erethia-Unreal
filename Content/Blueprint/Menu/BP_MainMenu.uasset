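; BP_MainMenu is a hand-attached menu actor that hosts WBP_MainMenu, with a Niagara laser and cursor for pointing.
; AttachMenu parents menu and laser to given hands, adds the keyboard mapping context, and finds the owner's Widget Interaction components by pointer index.
; When tracing, Tick stretches the laser to the right pointer's hit point.
; Click events press or release the pointers, while navigation and simulated click/hover calls forward to the widget.
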(event `self.ReceiveBeginPlay`
  (bind _aswbp_main_menu (cast `/Game/Blueprint/Widget/MainMenu/WBP_MainMenu` (`WidgetComponent.GetWidget` (`self.Menu`))))
  (set `self.RefWidget` _aswbp_main_menu))

(event `AttachMenu`
  (params (Owner :type "/Game/Blueprint/Player/BP_Player Object Reference") (HandToAttachMenu :type "StaticMeshComponent Object Reference") (handToAttachLaser :type "MotionControllerComponent Object Reference"))
  (`self.EnableInput` (`GameplayStatics.GetPlayerController` 0))
  (`EnhancedInputSubsystemInterface.AddMappingContext` (pcsubsystem `EnhancedInputLocalPlayerSubsystem` (`GameplayStatics.GetPlayerController` 0)) "/Game/IMC/IMC_KeyboardMenu.IMC_KeyboardMenu" 2 (struct))
  (`SceneComponent.K2_AttachToComponent` (`self.Menu`) HandToAttachMenu "None" "KeepRelative" "KeepRelative" "KeepRelative" true)
  (set `self.RefOwner` Owner)
  (`SceneComponent.K2_AttachToComponent` (`self.MenuLaser`) handToAttachLaser "None" "KeepRelative" "KeepRelative" "KeepRelative" true)
  (`self.SetWidgetInteractionReferences` (`self.RefOwner`)))

(event `CloseMenu`
  (`EnhancedInputSubsystemInterface.RemoveMappingContext` (pcsubsystem `EnhancedInputLocalPlayerSubsystem` (`GameplayStatics.GetPlayerController` 0)) "/Game/IMC/IMC_KeyboardMenu.IMC_KeyboardMenu" (struct)))

(event `self.ReceiveTick`
  (params (DeltaSeconds :type "Float (single-precision)"))
  (bind (_returnvalue_bblockinghit _returnvalue_binitialoverlap _returnvalue_time _returnvalue_distance _returnvalue_location _returnvalue_impactpoint) (`GameplayStatics.BreakHitResult` (`WidgetInteractionComponent.GetLastHitResult` (`self.WidgetInteractionRefRight`))))
  (if (`self.DisplayTrace?`)
    (`/Engine/EditorBlueprintResources/StandardMacros.IsValid` (`SceneComponent.GetAttachParent` (`self.MenuLaser`))
      (:`Is Valid`
        (`NiagaraDataInterfaceArrayFunctionLibrary.SetNiagaraArrayVectorValue` (`self.MenuLaser`) "User.PointArray" 0 (`SceneComponent.K2_GetComponentLocation` (`SceneComponent.GetAttachParent` (`self.MenuLaser`))))
        (`NiagaraDataInterfaceArrayFunctionLibrary.SetNiagaraArrayVectorValue` (`self.MenuLaser`) "User.PointArray" 1 _returnvalue_impactpoint)
        (`SceneComponent.K2_SetWorldLocation` (`self.Cursor`) _returnvalue_impactpoint false false)))))

(event `ClickRight`
  (`WidgetInteractionComponent.PressPointerKey` (`self.WidgetInteractionRefLeft`) "LeftMouseButton"))

(event `ClickLeft`
  (`WidgetInteractionComponent.PressPointerKey` (`self.WidgetInteractionRefRight`) "LeftMouseButton"))

(event `StopClickLeft`
  (`WidgetInteractionComponent.ReleasePointerKey` (`self.WidgetInteractionRefRight`) "LeftMouseButton"))

(event `StopClickRight`
  (`WidgetInteractionComponent.ReleasePointerKey` (`self.WidgetInteractionRefLeft`) "LeftMouseButton"))

(event `EnhancedInput|/Game/IMC/IA/Keyboard/IA_KeyboardClickMenu`
  (params (ActionValue :type Boolean) (ElapsedSeconds :type "Float (double-precision)") (TriggeredSeconds :type "Float (double-precision)") (InputAction :type "InputAction Object Reference" :default "/Game/IMC/IA/Keyboard/IA_KeyboardClickMenu.IA_KeyboardClickMenu"))
  (:`Started`
    (`self.ClickRight`)
    (`self.ClickLeft`))
  (:`Completed`
    (`self.StopClickRight`)
    (`self.StopClickLeft`)))

(event `NextButton`
  (`/Game/Blueprint/Widget/MainMenu/WBP_MainMenu.NextButton` (`self.RefWidget`)))

(event `PreviousButton`
  (`/Game/Blueprint/Widget/MainMenu/WBP_MainMenu.PreviousButton` (`self.RefWidget`)))

(event `SimulateClick`
  (`/Game/Blueprint/Widget/MainMenu/WBP_MainMenu.SimulateClick` (`self.RefWidget`)))

(event `SimulateHovered`
  (`/Game/Blueprint/Widget/MainMenu/WBP_MainMenu.SimulateHovered` (`self.RefWidget`)))

(fn `SetWidgetInteractionReferences`
  (params (Player :type "/Game/Blueprint/Player/BP_Player Object Reference"))
  (locals (LocalWidgetInteractionComponents :type "Array of WidgetInteractionComponent Object Reference"))
  (bind _returnvalue (`self.K2_GetComponentsByClass` Player "/Script/UMG.WidgetInteractionComponent"))
  (if (> (`KismetArrayLibrary.Array_Length` _returnvalue) 0)
    (bind _output_get (set `local.LocalWidgetInteractionComponents` _returnvalue))
    (for _array_element _output_get
      (if (== (`WidgetInteractionComponent.PointerIndex` _array_element) 0)
        (set `self.WidgetInteractionRefLeft` _array_element)
        (else
          (set `self.WidgetInteractionRefRight` _array_element))))
    (else
      (`KismetSystemLibrary.PrintString` "Warning: No WidgetInteractionComponent was found. Menu interaction will FAIL"))))

(fn `UserConstructionScript`)