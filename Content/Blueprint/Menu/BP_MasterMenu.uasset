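; BP_MasterMenu is a menu actor that sends up, down, confirm and back messages to its widget component.
; Overlap handlers accept components tagged Hand, skip child BP_MainMenuButton actors already being pressed, then message the widget and trigger the button's Pressed.
; GoUp, GoDown and Confirm events send the same messages directly.
; The code binding the overlap handlers to the buttons is disconnected, and BeginPlay is empty.
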(event `OverlapUp`
  (params (OverlappedComponent :type "PrimitiveComponent Object Reference") (OtherActor :type "Actor Object Reference") (OtherComp :type "PrimitiveComponent Object Reference") (OtherBodyIndex :type Integer) (bFromSweep :type Boolean) (SweepResult :type "HitResult Structure (by ref)"))
  (if (`ActorComponent.ComponentHasTag` OtherComp "Hand")
    (bind _asbp_main_menu_button (cast `/Game/Blueprint/InteractiveObject/Button/Menu/BP_MainMenuButton` (`ChildActorComponent.ChildActor` (`self.Up`))))
    (if (not (`/Game/Blueprint/InteractiveObject/Button/Menu/BP_MainMenuButton.IsBeingPressed?` _asbp_main_menu_button))
      (message `/Game/Blueprint/Interface/Menu/BPI_MenuInteraction.GoUp` (`WidgetComponent.GetWidget` (`self.Widget`)))
      (`/Game/Blueprint/InteractiveObject/Button/Menu/BP_MainMenuButton.Pressed` _asbp_main_menu_button))))

(event `self.ReceiveBeginPlay`)

(event `OverlapDown`
  (params (OverlappedComponent :type "PrimitiveComponent Object Reference") (OtherActor :type "Actor Object Reference") (OtherComp :type "PrimitiveComponent Object Reference") (OtherBodyIndex :type Integer) (bFromSweep :type Boolean) (SweepResult :type "HitResult Structure (by ref)"))
  (if (`ActorComponent.ComponentHasTag` OtherComp "Hand")
    (bind _asbp_main_menu_button (cast `/Game/Blueprint/InteractiveObject/Button/Menu/BP_MainMenuButton` (`ChildActorComponent.ChildActor` (`self.Down`))))
    (if (not (`/Game/Blueprint/InteractiveObject/Button/Menu/BP_MainMenuButton.IsBeingPressed?` _asbp_main_menu_button))
      (message `/Game/Blueprint/Interface/Menu/BPI_MenuInteraction.GoDown` (`WidgetComponent.GetWidget` (`self.Widget`)))
      (`/Game/Blueprint/InteractiveObject/Button/Menu/BP_MainMenuButton.Pressed` _asbp_main_menu_button))))

(event `OverlapConfirm`
  (params (OverlappedComponent :type "PrimitiveComponent Object Reference") (OtherActor :type "Actor Object Reference") (OtherComp :type "PrimitiveComponent Object Reference") (OtherBodyIndex :type Integer) (bFromSweep :type Boolean) (SweepResult :type "HitResult Structure (by ref)"))
  (if (`ActorComponent.ComponentHasTag` OtherComp "Hand")
    (bind _asbp_main_menu_button (cast `/Game/Blueprint/InteractiveObject/Button/Menu/BP_MainMenuButton` (`ChildActorComponent.ChildActor` (`self.ConfirmButton`))))
    (if (not (`/Game/Blueprint/InteractiveObject/Button/Menu/BP_MainMenuButton.IsBeingPressed?` _asbp_main_menu_button))
      (message `/Game/Blueprint/Interface/Menu/BPI_MenuInteraction.Confirm` (`WidgetComponent.GetWidget` (`self.Widget`)))
      (`/Game/Blueprint/InteractiveObject/Button/Menu/BP_MainMenuButton.Pressed` _asbp_main_menu_button))))

(event `OverlapGoBack`
  (params (OverlappedComponent :type "PrimitiveComponent Object Reference") (OtherActor :type "Actor Object Reference") (OtherComp :type "PrimitiveComponent Object Reference") (OtherBodyIndex :type Integer) (bFromSweep :type Boolean) (SweepResult :type "HitResult Structure (by ref)"))
  (if (`ActorComponent.ComponentHasTag` OtherComp "Hand")
    (bind _asbp_main_menu_button (cast `/Game/Blueprint/InteractiveObject/Button/Menu/BP_MainMenuButton` (`ChildActorComponent.ChildActor` (`self.Return`))))
    (if (not (`/Game/Blueprint/InteractiveObject/Button/Menu/BP_MainMenuButton.IsBeingPressed?` _asbp_main_menu_button))
      (message `/Game/Blueprint/Interface/Menu/BPI_MenuInteraction.GoBack` (`WidgetComponent.GetWidget` (`self.Widget`)))
      (`/Game/Blueprint/InteractiveObject/Button/Menu/BP_MainMenuButton.Pressed` _asbp_main_menu_button))))

(event `GoUp`
  (message `/Game/Blueprint/Interface/Menu/BPI_MenuInteraction.GoUp` (`WidgetComponent.GetWidget` (`self.Widget`))))

(event `GoDown`
  (message `/Game/Blueprint/Interface/Menu/BPI_MenuInteraction.GoDown` (`WidgetComponent.GetWidget` (`self.Widget`))))

(event `Confirm`
  (message `/Game/Blueprint/Interface/Menu/BPI_MenuInteraction.Confirm` (`WidgetComponent.GetWidget` (`self.Widget`))))

(fn `UserConstructionScript`)