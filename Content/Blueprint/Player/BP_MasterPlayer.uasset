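; Master player Blueprint, a base that claims a spawn point and drives an in-world main menu, with hooks suggesting VR use.
; After a BeginPlay delay, the server assigns a free BP_Spawner, then GameInstance and GameState are cached.
; The menu actor spawns at PosMenu, is hidden and reused, and receives navigation through Enhanced Input mapping contexts.
; SetupIMC and right-hand bind functions are empty stubs; left/right navigation only prints.
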(event `self.ReceiveBeginPlay`
  (`KismetSystemLibrary.Delay` 2.0)
  (`|ExecutionSequence`
    (:`then_0`
      (`/Engine/EditorBlueprintResources/ActorMacros.Switch Has Authority`
        (:`Authority`
          (bind _outactors (`GameplayStatics.GetAllActorsOfClass` "/Game/Blueprint/Spawner/BP_Spawner.BP_Spawner_C"))
          (for _array_element _outactors
            (if (and (not (`/Game/Blueprint/Spawner/BP_Spawner.AlreadyUsedForSpawn?` _array_element)) (not (`/Game/Blueprint/Spawner/BP_Spawner.AlreadyPlayerInside?` _array_element)))
              (bind _allowspawn_ (`/Game/Blueprint/Spawner/BP_Spawner.Set Player Fo Spawn` _array_element self))
              (if _allowspawn_
                (break)))))))
    (:`then_1`
      (`|ExecutionSequence`
        (:`then_0`
          (bind _asbp_game_instance (cast `/Game/Blueprint/GameInstance/BP_GameInstance` (`GameplayStatics.GetGameInstance`)))
          (set `self.RefGI` _asbp_game_instance))
        (:`then_1`
          (bind _asgs_master (cast `/Game/Blueprint/GameState/GS_Master` (`GameplayStatics.GetGameState`)))
          (set `self.RefGS` _asgs_master))
        (:`then_2`
          (`self.SetupIMC`))))))

(event `TimerForAuthorizationInteractionMenu`
  ;[0.05098 0.05098 0.05098] Menu
  (set `self.CanInteractWithMenu?` false)
  (`KismetSystemLibrary.K2_SetTimerDelegate` (delegate `AuthorizeMenuInteraction`) 0.2))

(event `EnhancedInput|/Game/IMC/IA/Menu/IA_OpenCloseMenu`
  (params (ActionValue :type Boolean) (ElapsedSeconds :type "Float (double-precision)") (TriggeredSeconds :type "Float (double-precision)") (InputAction :type "InputAction Object Reference" :default "/Game/IMC/IA/Menu/IA_OpenCloseMenu.IA_OpenCloseMenu"))
  ;[0.05098 0.05098 0.05098] Menu
  ;;[1 1 1] Open / Close Menu
  (:`Started`
    (if (not (`self.Is Menu Open?`))
      (`self.OpenMenu`)
      (else
        (`self.CloseMenu`)))))

(event `AuthorizeMenuInteraction`
  ;[0.05098 0.05098 0.05098] Menu
  (set `self.CanInteractWithMenu?` true))

(event `EnhancedInput|/Game/IMC/IA/Menu/IA_MoveInMenu`
  (params (ActionValue :type "Vector2D Structure") (ElapsedSeconds :type "Float (double-precision)") (TriggeredSeconds :type "Float (double-precision)") (InputAction :type "InputAction Object Reference" :default "/Game/IMC/IA/Menu/IA_MoveInMenu.IA_MoveInMenu"))
  ;[0.05098 0.05098 0.05098] Menu
  ;;[1 1 1] Inputs Menu
  (:`Started`
    (if (and (`KismetSystemLibrary.IsValid` (`self.RefMenu`)) (`self.Is Menu Open?`) (`self.CanInteractWithMenu?`))
      (if (and (< ActionValue_X 0.4) (> ActionValue_X -0.4))
        (if (and (!= ActionValue_Y 0.0) (< ActionValue_Y 0.0))
          (`/Game/Blueprint/Menu/BP_MasterMenu.GoUp` (`self.RefMenu`))
          (else
            (`/Game/Blueprint/Menu/BP_MasterMenu.GoDown` (`self.RefMenu`))))
        (elif (and (!= ActionValue_X 0.0) (> ActionValue_X 0.0))
          (`KismetSystemLibrary.PrintString` "Right")
          (else
            (`KismetSystemLibrary.PrintString` "Left")))))))

(event `OpenMenu`
  (bind _posmenu (`self.PosMenu`))
  (bind _refmenu (`self.RefMenu`))
  (bind _posmenu_2 (`self.PosMenu`))
  ;[0.05098 0.05098 0.05098] Menu
  ;;[1 1 1] Open / Close Menu
  (`/Engine/EditorBlueprintResources/StandardMacros.IsValid` _refmenu
    (:`Is Valid`
      (`self.K2_SetActorTransform` _refmenu (`KismetMathLibrary.MakeTransform` (`SceneComponent.K2_GetComponentLocation` _posmenu_2) (`SceneComponent.K2_GetComponentRotation` _posmenu_2)) false false)
      (`self.SetActorHiddenInGame` (`self.RefMenu`) false))
    (:`Is Not Valid`
      (bind _returnvalue (`|SpawnActorFromClass` "/Game/Blueprint/Menu/MainMenu/BP_NewMainMenu.BP_NewMainMenu_C" (`KismetMathLibrary.MakeTransform` (`SceneComponent.K2_GetComponentLocation` _posmenu) (`SceneComponent.K2_GetComponentRotation` _posmenu)) "Undefined" "MultiplyWithRoot" self self))
      (set `self.RefMenu` _returnvalue)))
  (`self.AddMenuIMC`)
  (set `self.Is Menu Open?` true))

(event `EnhancedInput|/Game/IMC/IA/Menu/IA_ConfirmMenu`
  (params (ActionValue :type Boolean) (ElapsedSeconds :type "Float (double-precision)") (TriggeredSeconds :type "Float (double-precision)") (InputAction :type "InputAction Object Reference" :default "/Game/IMC/IA/Menu/IA_ConfirmMenu.IA_ConfirmMenu"))
  ;[0.05098 0.05098 0.05098] Menu
  ;;[1 1 1] Inputs Menu
  (:`Started`
    (`KismetSystemLibrary.PrintText` "Hello")
    (if (and (`KismetSystemLibrary.IsValid` (`self.RefMenu`)) (`self.Is Menu Open?`) (`self.CanInteractWithMenu?`))
      (`/Game/Blueprint/Menu/BP_MasterMenu.Confirm` (`self.RefMenu`)))))

(event `CloseMenu`
  (bind _refmenu (`self.RefMenu`))
  ;[0.05098 0.05098 0.05098] Menu
  ;;[1 1 1] Open / Close Menu
  (`/Engine/EditorBlueprintResources/StandardMacros.IsValid` _refmenu
    (:`Is Valid`
      (`self.SetActorHiddenInGame` _refmenu true)
      (`self.RemoveMenuIMC`)
      (`self.RebindRightHand`)
      (set `self.Is Menu Open?` false))))

(fn `AddMenuIMC`
  (`self.Unbind Right Hand`)
  (`EnhancedInputSubsystemInterface.AddMappingContext` (pcsubsystem `EnhancedInputLocalPlayerSubsystem` (`self.RefPc`)) "/Game/IMC/IMC_BasicMenu.IMC_BasicMenu" 0 (struct)))

(fn `GetMenu`
  (returns (Menu :type "/Game/Blueprint/Menu/MainMenu/BP_NewMainMenu Object Reference"))
  (return null))

(fn `RebindRightHand`)

(fn `RemoveMenuIMC`
  (`EnhancedInputSubsystemInterface.RemoveMappingContext` (pcsubsystem `EnhancedInputLocalPlayerSubsystem` (`self.RefPc`)) "/Game/IMC/IMC_BasicMenu.IMC_BasicMenu" (struct))
  (`EnhancedInputSubsystemInterface.RemoveMappingContext` (pcsubsystem `EnhancedInputLocalPlayerSubsystem` (`self.RefPc`)) "/Game/IMC/IMC_MenuVR.IMC_MenuVR" (struct)))

(fn `SetupIMC`)

(fn `Unbind Right Hand`)

(fn `UserConstructionScript`)