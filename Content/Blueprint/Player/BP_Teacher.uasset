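; BP_Teacher is the teacher's player pawn, with directional movement and an in-game statistics overlay.
; BeginPlay configures the ACVRKeyboard component, while the Movement input drives movement along the actor's forward and right vectors.
; Statistics events create WBP_InGameStatistics for the owning PlayerController and remove it from the viewport.
; Getter functions expose the camera and player type, while hand, arrow and menu-state getters are empty or constant stubs.
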(event `self.ReceiveBeginPlay`
  (bind _ac_vrkeyboard (`self.AC_VRKeyboard`))
  (`parent.ReceiveBeginPlay`)
  (`/Game/Blueprint/Component/AC_VRKeyboard.StartConfig` _ac_vrkeyboard)
  (set `/Game/Blueprint/Component/AC_VRKeyboard.UpDownSpeed` 50.0 _ac_vrkeyboard))

(event `/Game/Blueprint/Interface/Players/BPI_PlayerInterface.Movement`
  (params (ActionValue :type "Vector2D Structure"))
  (bind (_x _y) (`KismetMathLibrary.BreakVector2D` ActionValue))
  (`self.AddMovementInput` (* (`self.GetActorForwardVector`) _y))
  (`self.AddMovementInput` (* _x (`self.GetActorRightVector`))))

(event `/Game/Blueprint/Interface/Players/BPI_PlayerInterface.DisplayStatisticMenu`
  (bind _asplayer_controller (cast `PlayerController` (`self.GetOwner`)))
  (bind _returnvalue (`|CreateWidget` "/Game/Blueprint/Widget/Menu/Statistics/WBP_InGameStatistics.WBP_InGameStatistics_C" _asplayer_controller))
  (bind _output_get (set `self.StatisticsMenu` _returnvalue))
  (`UserWidget.AddToViewport` _output_get 0))

(event `/Game/Blueprint/Interface/Players/BPI_PlayerInterface.RemoveStatistics`
  (bind _statisticsmenu (`self.StatisticsMenu`)
    (:`then`
      (`Widget.RemoveFromParent` _statisticsmenu))
    (:`else`)))

(fn `GetCamera`
  (returns (Camera :type "CameraComponent Object Reference"))
  (return (`self.Camera`)))

(fn `GetHand`
  (params (Hand :type "/Game/Enum/E_KeyboardControlTypes Enum" :default "NewEnumerator0"))
  (returns (Grip :type "MotionControllerComponent Object Reference") (Aim :type "MotionControllerComponent Object Reference"))
  (return null null))

(fn `GetPlayerType`
  (returns (Type :type "/Game/Enum/E_PlayerType Enum"))
  (return "NewEnumerator0"))

(fn `GetStateMenu`
  (returns (`IsOpen?` :type Boolean))
  (return false))

(fn `GetTopAndBottomArrow`
  (returns (Top :type "ArrowComponent Object Reference") (Bottom :type "ArrowComponent Object Reference"))
  (return null null))

(fn `UserConstructionScript`)