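; PC_Game is the game's player controller, acting as a relay for client-side puzzle and sound actions.
; Each Client-suffixed event checks an object reference, then forwards to the matching function on pedestals, frescoes, the central statue, pillars, the master hologram or the player sound object.
; Pedestal and fresco events validate the statuette or piece rather than the actor called.
; A CastGs override caches the game state as GS_Game and passes it to the parent.
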(event `GrabItemClient`
  (params (Piedestal :type "/Game/Blueprint/InteractiveObject/Piedestal/BP_Piedestal Object Reference") (Statuette :type "/Game/Blueprint/InteractiveObject/Gabable_OBJ/Statue/BP_MasterPuzzleStatue Object Reference"))
  (`/Engine/EditorBlueprintResources/StandardMacros.IsValid` Statuette
    (:`Is Valid`
      (`/Game/Blueprint/InteractiveObject/Piedestal/BP_Piedestal.GrabItemClient` Piedestal Statuette))))

(event `ReleaseAndSnapObjectClient`
  (params (FrescoPiece :type "Actor Object Reference") (FullFresco :type "/Game/AssetsErethia/objects/fresco/fresco01/BP_fresco01_incomplete Object Reference") (SnapPosition :type "StaticMeshComponent Object Reference"))
  (`/Engine/EditorBlueprintResources/StandardMacros.IsValid` FrescoPiece
    (:`Is Valid`
      (`/Game/AssetsErethia/objects/fresco/fresco01/BP_fresco01_incomplete.ReleaseAndSnapObjectClient` FullFresco FrescoPiece SnapPosition))))

(event `ReleaseAndSnapObjectClient2`
  (params (FrescoPiece :type "Actor Object Reference") (FullFresco :type "/Game/AssetsErethia/objects/fresco/fresco02/BP_fresco02_incomplete Object Reference") (SnapPosition :type "StaticMeshComponent Object Reference"))
  (`/Engine/EditorBlueprintResources/StandardMacros.IsValid` FrescoPiece
    (:`Is Valid`
      (`/Game/AssetsErethia/objects/fresco/fresco02/BP_fresco02_incomplete.ReleaseAndSnapObjectClient2` FullFresco FrescoPiece SnapPosition))))

(event `TurnStatueClient`
  (params (CentralStatue :type "/Game/Blueprint/InteractiveObject/Statue/BP_CentralStatue Object Reference"))
  (`/Engine/EditorBlueprintResources/StandardMacros.IsValid` CentralStatue
    (:`Is Valid`
      (`/Game/Blueprint/InteractiveObject/Statue/BP_CentralStatue.TurnStatueClient` CentralStatue))))

(event `ClearSoundClient`
  (params (PlayerSound :type "/Game/Blueprint/InteractiveObject/Sound/BP_PlayAllSound Object Reference"))
  (`/Engine/EditorBlueprintResources/StandardMacros.IsValid` PlayerSound
    (:`Is Valid`
      (`/Game/Blueprint/InteractiveObject/Sound/BP_PlayAllSound.ClearSoundClient` PlayerSound))))

(event `StopSoundClient`
  (params (PlayerSound :type "/Game/Blueprint/InteractiveObject/Sound/BP_PlayAllSound Object Reference"))
  (`/Engine/EditorBlueprintResources/StandardMacros.IsValid` PlayerSound
    (:`Is Valid`
      (`/Game/Blueprint/InteractiveObject/Sound/BP_PlayAllSound.StopSoundClient` PlayerSound))))

(event `AddSoundToListClient`
  (params (PlayerSound :type "/Game/Blueprint/InteractiveObject/Sound/BP_PlayAllSound Object Reference") (NewSound :type "SoundBase Object Reference") (ForcePlay :type Boolean))
  (`/Engine/EditorBlueprintResources/StandardMacros.IsValid` PlayerSound
    (:`Is Valid`
      (`/Game/Blueprint/InteractiveObject/Sound/BP_PlayAllSound.AddSoundToListClient` PlayerSound NewSound ForcePlay))))

(event `MovePilarClient`
  (params (Pilar :type "/Game/Blueprint/InteractiveObject/Pilar/NewPilar/BP_NewPilar Object Reference") (AllTargetLocation :type "Array of Vector2D Structure"))
  (`/Engine/EditorBlueprintResources/StandardMacros.IsValid` Pilar
    (:`Is Valid`
      (`/Game/Blueprint/InteractiveObject/Pilar/NewPilar/BP_NewPilar.MovePilarClient` Pilar AllTargetLocation))))

(event `SelectedPilarClient`
  (params (Pilar :type "/Game/Blueprint/InteractiveObject/Pilar/NewPilar/BP_NewPilar Object Reference"))
  (`/Engine/EditorBlueprintResources/StandardMacros.IsValid` Pilar
    (:`Is Valid`
      (`/Game/Blueprint/InteractiveObject/Pilar/NewPilar/BP_NewPilar.SelectedPilarClient` Pilar))))

(event `UnselectedPilarClient`
  (params (Pilar :type "/Game/Blueprint/InteractiveObject/Pilar/NewPilar/BP_NewPilar Object Reference"))
  (`/Engine/EditorBlueprintResources/StandardMacros.IsValid` Pilar
    (:`Is Valid`
      (`/Game/Blueprint/InteractiveObject/Pilar/NewPilar/BP_NewPilar.UnselectedPilarClient` Pilar))))

(event `ChangeOrientationClient`
  (params (MasterHologram :type "/Game/Blueprint/InteractiveObject/HologramDisplay/BP_MasterHologrameDisplay Object Reference") (OrientationIndex :type Integer))
  (`/Engine/EditorBlueprintResources/StandardMacros.IsValid` MasterHologram
    (:`Is Valid`
      (`/Game/Blueprint/InteractiveObject/HologramDisplay/BP_MasterHologrameDisplay.ChangeOrientationClient` MasterHologram OrientationIndex))))

(fn `CastGs`
  (params (AlreadyCastGs :type "/Game/Blueprint/GameState/GS_Master Object Reference"))
  (bind _asgs_game (cast `/Game/Blueprint/GameState/GS_Game` (`GameplayStatics.GetGameState`)))
  (bind _output_get (set `self.RefGSGame` _asgs_game))
  (`parent.CastGs` _output_get))

(fn `UserConstructionScript`
  (`parent.UserConstructionScript`))