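; Main menu player controller with temporary input shortcuts for hosting or joining a multiplayer session.
; The host action creates a session, then opens L_Level1 as a listen server.
; The keyboard join action runs a non-LAN session search and joins the first result without checking that any were found.
; Its CastGs function caches the game state as GS_MainMenu, then calls the parent version.
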(event `EnhancedInput|/Game/IMC/IA/Keyboard/IA_TemporaryStartServer`
  (params (ActionValue :type Boolean) (ElapsedSeconds :type "Float (double-precision)") (TriggeredSeconds :type "Float (double-precision)") (InputAction :type "InputAction Object Reference" :default "/Game/IMC/IA/Keyboard/IA_TemporaryStartServer.IA_TemporaryStartServer"))
  (:`Triggered`
    (`CreateSessionCallbackProxy.CreateSession` (`GameplayStatics.GetPlayerController` 0) 42
      (:`OnSuccess`
        (`GameplayStatics.OpenLevel` "L_Level1" true "?listen")))))

(event `EnhancedInput|/Game/IMC/IA/Keyboard/IA_KeyboardTemporaryJoinServer`
  (params (ActionValue :type Boolean) (ElapsedSeconds :type "Float (double-precision)") (TriggeredSeconds :type "Float (double-precision)") (InputAction :type "InputAction Object Reference" :default "/Game/IMC/IA/Keyboard/IA_KeyboardTemporaryJoinServer.IA_KeyboardTemporaryJoinServer"))
  (:`Triggered`
    (bind _results (`FindSessionsCallbackProxy.FindSessions` (`GameplayStatics.GetPlayerController` 0) 69)
      (:`OnSuccess`
        (`KismetSystemLibrary.PrintString` "Successfully found session")
        (`JoinSessionCallbackProxy.JoinSession` (`GameplayStatics.GetPlayerController` 0) (`|GetArrayItem` _results))))))

(fn `CastGs`
  (params (AlreadyCastGs :type "/Game/Blueprint/GameState/GS_Master Object Reference"))
  (bind _asgs_main_menu (cast `/Game/Blueprint/GameState/GS_MainMenu` (`GameplayStatics.GetGameState`)))
  (bind _output_get (set `self.RefGSMainMenu` _asgs_main_menu))
  (`parent.CastGs` _output_get))

(fn `UserConstructionScript`
  (`parent.UserConstructionScript`))