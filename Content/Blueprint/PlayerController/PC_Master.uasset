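; Master player controller for a multiplayer VR game, linking the player pawn, game instance and game state.
; BeginPlay caches these references after a short delay, then events sync player ID and player info through the game instance.
; Client-suffixed events relay grabs, grips, pressure plates, doors, object transforms and widget updates to their target actors.
; Disconnect events destroy the session, retrying on failure, then clean up and open the main menu.
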(event `self.ReceiveBeginPlay`
  (`KismetSystemLibrary.Delay` 0.2)
  (`|ExecutionSequence`
    (:`then_0`
      (`self.GetClientGameInstance`)
      (`self.GetServGameInstance`)
      (`self.GetClientID`))
    (:`then_1`
      (bind _asbp_player (cast `/Game/Blueprint/Player/BP_Player` (`self.K2_GetPawn`)))
      (bind _output_get (set `self.RefPlayer` _asbp_player))
      (set `/Game/Blueprint/Player/BP_Player.RefPc` self _output_get))
    (:`then_2`
      (`self.CastGs` null))))

(event `GetClientGameInstance`
  (bind _asbp_game_instance (cast `/Game/Blueprint/GameInstance/BP_GameInstance` (`GameplayStatics.GetGameInstance`)))
  (set `self.RefGI` _asbp_game_instance))

(event `GetServGameInstance`
  (bind _asbp_game_instance (cast `/Game/Blueprint/GameInstance/BP_GameInstance` (`GameplayStatics.GetGameInstance`)))
  (set `self.RefGI` _asbp_game_instance))

(event `GetClientID`
  (bind _refgi (`self.RefGI`))
  (bind _playerinfo_id (break `/Game/Struct/S_PlayerInfo` (`/Game/Blueprint/GameInstance/BP_GameInstance.PlayerInfo` _refgi)))
  (`/Engine/EditorBlueprintResources/StandardMacros.IsValid` _refgi
    (:`Is Valid`
      (bind _output_get (set `self.ID` _playerinfo_id))
      (`self.SetID` _output_get))))

(event `NewPlayerInfo`
  (params (PlayerInfo :type "/Game/Struct/S_PlayerInfo Structure"))
  (bind _refgi (`self.RefGI`))
  (`/Engine/EditorBlueprintResources/StandardMacros.IsValid` _refgi
    (:`Is Valid`
      (bind _output_get (set `/Game/Blueprint/GameInstance/BP_GameInstance.PlayerInfo` PlayerInfo _refgi))
      (`/Engine/EditorBlueprintResources/StandardMacros.IsValid` (`.Pawn_16_F0557B3940946A7D12EB85B39451416E` (break `/Game/Struct/S_PlayerInfo` _output_get))
        (:`Is Valid`
          (bind _asbp_player (cast `/Game/Blueprint/Player/BP_Player` (`.Pawn_16_F0557B3940946A7D12EB85B39451416E` (break `/Game/Struct/S_PlayerInfo` _output_get))))
          (set `/Game/Blueprint/Player/BP_Player.RefPc` self _asbp_player))))
    (:`Is Not Valid`
      (`KismetSystemLibrary.PrintString` "GI not valid"))))

(event `NewListOfAllPlayerInfo`
  (params (ListPlayerInfo :type "Array of /Game/Struct/S_PlayerInfo Structure"))
  (`self.CheckAndSetGI`
    (:`Valid`
      (set `/Game/Blueprint/GameInstance/BP_GameInstance.ListPlayerInfo` ListPlayerInfo (`self.RefGI`)))))

(event `SetID`
  (params (ID :type Integer))
  (set `self.ID` ID))

(event `SetupNewPlayer`
  (params (PlayerInfo :type "/Game/Struct/S_PlayerInfo Structure"))
  (bind _asbp_player (cast `/Game/Blueprint/Player/BP_Player` PlayerInfo_Pawn_16_F0557B3940946A7D12EB85B39451416E))
  (set `/Game/Blueprint/Player/BP_Player.ID` PlayerInfo_ID_8_D4FD95844269CA8856CBAD9AA89464B1 _asbp_player))

(event `GrabClient`
  (params (Pawn :type "/Game/Blueprint/Player/BP_Player Object Reference") (Component :type "/Game/VRTemplate/Blueprints/GrabComponent Object Reference") (Hand :type "/Game/Enum/E_KeyboardControlTypes Enum" :default "NewEnumerator0"))
  (`/Engine/EditorBlueprintResources/StandardMacros.IsValid` Pawn
    (:`Is Valid`
      (`/Game/Blueprint/Player/BP_Player.GrabClient` Pawn Component Hand))))

(event `ReleaseClient`
  (params (Pawn :type "/Game/Blueprint/Player/BP_Player Object Reference") (Hand :type "/Game/Enum/E_KeyboardControlTypes Enum" :default "NewEnumerator0"))
  (`/Engine/EditorBlueprintResources/StandardMacros.IsValid` Pawn
    (:`Is Valid`
      (`/Game/Blueprint/Player/BP_Player.ReleaseClient` Pawn Hand))))

(event `ActivateInteractiveForChallengeManager`
  (params (Manager :type "/Game/Blueprint/Challenge/BP_ChallengeManager Object Reference"))
  (`/Game/Blueprint/Challenge/BP_ChallengeManager.ActivateInteractiveClient` Manager))

(event `PressPlateClient`
  (params (PressurePlate :type "/Game/Blueprint/InteractiveObject/PressurePlate/PressurePlate Object Reference"))
  (`/Engine/EditorBlueprintResources/StandardMacros.IsValid` PressurePlate
    (:`Is Valid`
      (`/Game/Blueprint/InteractiveObject/PressurePlate/PressurePlate.PressPLateClient` PressurePlate))))

(event `UnpressPlateClient`
  (params (PressurePlate :type "/Game/Blueprint/InteractiveObject/PressurePlate/PressurePlate Object Reference"))
  (`/Engine/EditorBlueprintResources/StandardMacros.IsValid` PressurePlate
    (:`Is Valid`
      (`/Game/Blueprint/InteractiveObject/PressurePlate/PressurePlate.UnpressPlateClient` PressurePlate))))

(event `MoveDoorClient`
  (params (Door :type "/Game/Blueprint/InteractiveObject/Door/BP_DoorLeftRight Object Reference"))
  (`/Engine/EditorBlueprintResources/StandardMacros.IsValid` Door
    (:`Is Valid`
      (`/Game/Blueprint/InteractiveObject/Door/BP_DoorLeftRight.MoveDoorClient` Door))))

(event `DisconnectPlayerClient`
  (`DestroySessionCallbackProxy.DestroySession` self
    (:`OnSuccess`
      (`/Game/Blueprint/GameInstance/BP_GameInstance.CleanUp` (`self.RefGI`))
      (`GameplayStatics.OpenLevel` "L_MainMenu"))
    (:`OnFailure`
      (`self.DisconnectPlayerClient`))))

(event `DisconnectPlayerServer`
  (`DestroySessionCallbackProxy.DestroySession` self
    (:`OnSuccess`
      (`/Game/Blueprint/GameInstance/BP_GameInstance.CleanUp` (`self.RefGI`))
      (`GameplayStatics.OpenLevel` "L_MainMenu"))
    (:`OnFailure`
      (`self.DisconnectPlayerServer`))))

(event `UpdateWidgetClient`
  (params (WidgetManager :type "/Game/Blueprint/Widget/Menu/LobbyMenu/BP_ListPlayersManager Object Reference") (PlayerToAdd :type "Array of Text") (PlayerToRemove :type "Array of Text"))
  (`/Engine/EditorBlueprintResources/StandardMacros.IsValid` WidgetManager
    (:`Is Valid`
      (`/Game/Blueprint/Widget/Menu/LobbyMenu/BP_ListPlayersManager.UpdateWidgetClient` WidgetManager PlayerToAdd PlayerToRemove))))

(event `CheckupBoardIsUpdatedClient`
  (params (WidgetManager :type "/Game/Blueprint/Widget/Menu/LobbyMenu/BP_ListPlayersManager Object Reference") (AllPlayers :type "Array of Text"))
  (`/Engine/EditorBlueprintResources/StandardMacros.IsValid` WidgetManager
    (:`Is Valid`
      (`/Game/Blueprint/Widget/Menu/LobbyMenu/BP_ListPlayersManager.CheckupBoardIsUpdatedClient` WidgetManager AllPlayers))))

(event `UpdateControllerGripClient`
  (params (Player :type "/Game/Blueprint/Player/BP_Player Object Reference") (MotionController :type "MotionControllerComponent Object Reference") (Controller :type "/Game/Enum/E_KeyboardControlTypes Enum" :default "NewEnumerator0"))
  (`/Engine/EditorBlueprintResources/StandardMacros.IsValid` Player
    (:`Is Valid`
      (`/Game/Blueprint/Player/BP_Player.UpdateControllerGripClient` Player MotionController Controller))))

(event `SetTransformObjectClient`
  (params (Object :type "/Game/Blueprint/InteractiveObject/BP_MasterInteractive Object Reference") (ObjectTransform :type "Transform Structure"))
  (`/Engine/EditorBlueprintResources/StandardMacros.IsValid` Object
    (:`Is Valid`
      (`/Game/Blueprint/InteractiveObject/BP_MasterInteractive.SetTransformObjectClient` Object ObjectTransform))))

(event `UpdateGrabblePosition`
  (params (Object :type "/Game/Blueprint/InteractiveObject/Gabable_OBJ/BP_MasterGrabbableObjects Object Reference") (Location :type "Vector Structure") (Rotation :type "Rotator Structure"))
  (`/Engine/EditorBlueprintResources/StandardMacros.IsValid` Object
    (:`Is Valid`
      (`/Game/Blueprint/InteractiveObject/Gabable_OBJ/BP_MasterGrabbableObjects.UpdateGrabblePosition` Object Location Rotation))))

(fn `CastGs`
  (params (AlreadyCastGs :type "/Game/Blueprint/GameState/GS_Master Object Reference"))
  (`/Engine/EditorBlueprintResources/StandardMacros.IsValid` AlreadyCastGs
    (:`Is Valid`
      (set `self.RefGSMaster` AlreadyCastGs))
    (:`Is Not Valid`
      (bind _asgs_master (cast `/Game/Blueprint/GameState/GS_Master` (`GameplayStatics.GetGameState`)))
      (set `self.RefGSMaster` _asgs_master))))

(fn `UserConstructionScript`)