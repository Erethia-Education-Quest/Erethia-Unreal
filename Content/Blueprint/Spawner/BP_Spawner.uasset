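; BP_Spawner is a typed player spawn point marked by a capsule that tracks whether a BP_Player is standing inside it.
; Capsule overlap events set an occupancy flag, reacting only to the player's capsule component.
; SetPlayerFoSpawn compares the player's type with the spawner's SpawnType, then either moves the player to the capsule's transform and flags it as used, or prints a mismatch message and returns false.
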(event `self.Capsule.OnComponentBeginOverlap`
  (params (OverlappedComponent :type "PrimitiveComponent Object Reference") (OtherActor :type "Actor Object Reference") (OtherComp :type "PrimitiveComponent Object Reference") (OtherBodyIndex :type Integer) (bFromSweep :type Boolean) (SweepResult :type "HitResult Structure (by ref)"))
  (if (and (== (`GameplayStatics.GetObjectClass` OtherActor) "/Game/Blueprint/Player/BP_Player.BP_Player_C") (== (`GameplayStatics.GetObjectClass` OtherComp) "/Script/Engine.CapsuleComponent"))
    (set `self.AlreadyPlayerInside?` true)))

(event `self.Capsule.OnComponentEndOverlap`
  (params (OverlappedComponent :type "PrimitiveComponent Object Reference") (OtherActor :type "Actor Object Reference") (OtherComp :type "PrimitiveComponent Object Reference") (OtherBodyIndex :type Integer))
  (if (and (== (`GameplayStatics.GetObjectClass` OtherActor) "/Game/Blueprint/Player/BP_Player.BP_Player_C") (== (`GameplayStatics.GetObjectClass` OtherComp) "/Script/Engine.CapsuleComponent"))
    (set `self.AlreadyPlayerInside?` false)))

(fn `Set Player Fo Spawn`
  (params (Player :type "/Game/Blueprint/Player/BP_MasterPlayer Object Reference"))
  (returns (`AllowSpawn?` :type Boolean))
  (locals (TempoBite :type "/Game/Enum/E_PlayerType Enum" :default "NewEnumerator2"))
  (bind (_returnvalue_location _returnvalue_rotation) (`KismetMathLibrary.BreakTransform` (`SceneComponent.K2_GetComponentToWorld` (`self.Capsule`))))
  (bind _type (message `/Game/Blueprint/Interface/Players/BPI_PlayerInterface.GetPlayerType` Player))
  (bind _output_get (set `local.TempoBite` _type))
  (if (`|EnumEquality` _output_get (`self.SpawnType`))
    (`self.K2_SetActorTransform` Player (`KismetMathLibrary.MakeTransform` _returnvalue_location _returnvalue_rotation) false false)
    (bind _output_get_2 (set `self.AlreadyUsedForSpawn?` true))
    (`KismetSystemLibrary.PrintString` "Set Spawn")
    (return _output_get_2)
    (else
      (`KismetSystemLibrary.PrintText` (`|FormatText` "Wrong Type {x} but should be {y} for pawn {z}" (`|GetEnumeratorNameAsString` (`local.TempoBite`)) (`|GetEnumeratorNameAsString` (`self.SpawnType`)) (`KismetSystemLibrary.GetDisplayName` Player)))
      (return false))))

(fn `UserConstructionScript`)