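; Statistics manager actor that reports which challenges in the level are finished.
; It gathers all BP_ChallengeManager actors at construction and BeginPlay, printing the first one's status on refresh.
; ExportStats appends each challenge's status to a string, prints it, and opens a save dialog with that string as default filename, writing no file.
; Export runs at BeginPlay and every Tick, even when the completion check breaks on an unfinished challenge.
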(event `self.ReceiveBeginPlay`
  (`self.Refresh Challenges`)
  (`self.ExportStats`))

(event `self.ReceiveTick`
  (params (DeltaSeconds :type "Float (single-precision)"))
  (for _array_element (`self.Challenges`)
    (bind (_name _isfinished_) (`/Game/Blueprint/Challenge/BP_ChallengeManager.Get Challenge Name and Validation` _array_element))
    (if (not _isfinished_)
      (break)))
  (`self.ExportStats`))

(fn `ExportStats`
  (for _array_element (`self.Challenges`)
    (bind (_name _isfinished_) (`/Game/Blueprint/Challenge/BP_ChallengeManager.Get Challenge Name and Validation` _array_element))
    (bind _output_get (set `self.FileString` (`KismetStringLibrary.Concat_StrStr` (`self.FileString`) (`KismetTextLibrary.Conv_TextToString` (`|FormatText` "[STATS] {name challenge}: {x}/1" _name (select `bool` _isfinished_ :`false` "0" :`true` "1" :!type "Text"))))))
    (`KismetSystemLibrary.PrintText` (`KismetTextLibrary.Conv_StringToText` _output_get)))
  (`EFDFunctionLibrary.SaveFileDialog` (`KismetTextLibrary.Conv_TextToString` (`|FormatText` "Statistic Report : {levelname}" (`self.LevelName`))) "" (`self.FileString`) "" ".txt" "Single"))

(fn `Refresh Challenges`
  (bind _outactors (`GameplayStatics.GetAllActorsOfClass` "/Game/Blueprint/Challenge/BP_ChallengeManager.BP_ChallengeManager_C"))
  (set `self.Challenges` _outactors)
  (for _array_element (`self.Challenges`)
    (bind (_name _isfinished_) (`/Game/Blueprint/Challenge/BP_ChallengeManager.Get Challenge Name and Validation` _array_element))
    (`|GenericCreateObject` "/Script/UMG.TextBlock")
    (`KismetSystemLibrary.PrintText` (`|FormatText` "[STATS] {name challenge}: {x}/1" _name (select `bool` _isfinished_ :`false` "0" :`true` "1" :!type "Text")) true true (struct :`G` 0.66 :`B` 1.0 :`A` 1.0) 20.0)
    (return)))

(fn `UserConstructionScript`
  (bind _outactors (`GameplayStatics.GetAllActorsOfClass` "/Game/Blueprint/Challenge/BP_ChallengeManager.BP_ChallengeManager_C"))
  (set `self.Challenges` _outactors))