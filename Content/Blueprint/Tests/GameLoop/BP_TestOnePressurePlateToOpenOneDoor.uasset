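; Functional test checking that pressing pressure plates opens a left/right door in a challenge setup.
; PrepareTest computes the expected open position from the first triggered door's relative location, offset on Z by its OpenWide value.
; StartTest presses every plate in the ChallengeManager's list through PressPlateServer, with fixed delays before and after.
; It then compares door positions to that target within a small tolerance, reporting expected and actual locations on failure.
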(event `self.ReceivePrepareTest`
  (`parent.ReceivePrepareTest`)
  (bind _asbp_door_left_right (cast `/Game/Blueprint/InteractiveObject/Door/BP_DoorLeftRight` (`|GetArrayItem` (`/Game/Blueprint/Challenge/BP_ChallengeManager.ItemToTrigger` (`self.ChallengeManager`)))))
  (bind _returnvalue_location (`KismetMathLibrary.BreakTransform` (`SceneComponent.GetRelativeTransform` (`/Game/Blueprint/InteractiveObject/Door/BP_DoorLeftRight.Door` _asbp_door_left_right))))
  (set `self.LocationToArrive` (+ _returnvalue_location (`KismetMathLibrary.MakeVector` 0.0 0.0 (`KismetMathLibrary.Conv_IntToDouble` (`/Game/Blueprint/InteractiveObject/Door/BP_DoorLeftRight.OpenWide` _asbp_door_left_right))))))

(event `self.ReceiveStartTest`
  (bind _locationtoarrive (`self.LocationToArrive`))
  (bind _challengemanager (`self.ChallengeManager`))
  (`KismetSystemLibrary.Delay` 2.0)
  (for _array_element (`/Game/Blueprint/Challenge/BP_ChallengeManager.ListChallenge` _challengemanager)
    (bind _aspressure_plate (cast `/Game/Blueprint/InteractiveObject/PressurePlate/PressurePlate` _array_element))
    (`/Game/Blueprint/InteractiveObject/PressurePlate/PressurePlate.PressPlateServer` _aspressure_plate))
  (`KismetSystemLibrary.Delay` 2.0)
  (for _array_element_2 (`/Game/Blueprint/Challenge/BP_ChallengeManager.ItemToTrigger` _challengemanager)
    (bind _asbp_door_left_right (cast `/Game/Blueprint/InteractiveObject/Door/BP_DoorLeftRight` _array_element_2))
    (bind _relativelocation (`SceneComponent.RelativeLocation` (`/Game/Blueprint/InteractiveObject/Door/BP_DoorLeftRight.Door` _asbp_door_left_right)))
    (if (== _relativelocation _locationtoarrive :`ErrorTolerance` 0.1)
      (`self.FinishTest` "Succeeded")
      (else
        (`self.FinishTest` "Failed" (`KismetTextLibrary.Conv_TextToString` (`|FormatText` "Wrong Door Position. Should Be \"{x}\" but was \"{y}\"" (`KismetStringLibrary.Conv_VectorToString` _locationtoarrive) (`KismetStringLibrary.Conv_VectorToString` _relativelocation))))))))

(fn `UserConstructionScript`
  (`parent.UserConstructionScript`))