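; BP_MasterTestMenu is a functional test, apparently a base for main menu tests, that spawns the menu on TestActor.
; StartTest calls CreateAndAttachMenu with the left menu position and left aim controller for the laser.
; It fails if TestActor or PositionMenuLeft is missing, but has no failure branch for the controller.
; An unwired chain would validate RefMenu and cache its WBP_MainMenu widget, but never runs.
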(event `self.ReceiveStartTest`
  (bind _testactor (`self.TestActor`))
  (bind _positionmenuleft (`/Game/Blueprint/Player/BP_Player.PositionMenuLeft` _testactor))
  (bind _motioncontrollerleftaim (`/Game/Blueprint/Player/BP_Player.MotionControllerLeftAim` _testactor))
  (`/Engine/EditorBlueprintResources/StandardMacros.IsValid` _testactor
    (:`Is Valid`
      (`/Engine/EditorBlueprintResources/StandardMacros.IsValid` _positionmenuleft
        (:`Is Valid`
          (`/Engine/EditorBlueprintResources/StandardMacros.IsValid` _motioncontrollerleftaim
            (:`Is Valid`
              (`/Game/Blueprint/Player/BP_Player.CreateAndAttachMenu` _testactor _positionmenuleft _motioncontrollerleftaim))))
        (:`Is Not Valid`
          (`self.FinishTest` "Failed" "No PositionMenuLeft"))))
    (:`Is Not Valid`
      (`self.FinishTest` "Failed" "No Test Actor"))))

(fn `UserConstructionScript`)