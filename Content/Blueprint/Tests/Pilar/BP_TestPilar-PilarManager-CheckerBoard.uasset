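; Functional test for the checkerboard PilarManager puzzle, driving two preselected pilars.
; PrepareTest and StartTest share one chain that calls AdminSelection on both pilars if valid, then waits six seconds.
; The check on the door being open and the manager finished is disconnected, and both its branches report success, so the test never calls FinishTest.
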(event `self.ReceivePrepareTest`
  (bind _selectedpilar (`self.SelectedPilar`))
  (bind _output (`|GetArrayItem` _selectedpilar))
  (bind _output_2 (`|GetArrayItem` _selectedpilar 1))
  (if (and (`KismetSystemLibrary.IsValid` _output) (`KismetSystemLibrary.IsValid` _output_2)) :!label _label
    (`/Game/Blueprint/InteractiveObject/Pilar/BP_Pilar.AdminSelection` _output)
    (`/Game/Blueprint/InteractiveObject/Pilar/BP_Pilar.AdminSelection` _output_2)
    (`KismetSystemLibrary.Delay` 6.0)))

(event `self.ReceiveStartTest`
  (goto _label))

(fn `UserConstructionScript`)