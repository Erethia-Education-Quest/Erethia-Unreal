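; BP_Button is an interactive button that activates linked objects when something begins overlapping its Box.
; An overlap sinks the Press component slightly, then calls AtActivation on every valid entry in InteractWith.
; After a zero-length Delay, Press rises back automatically, without waiting for the overlap to end.
; The IsPressed flag ignores further overlaps until that cycle finishes.
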(event `self.Box.OnComponentBeginOverlap`
  (params (OverlappedComponent :type "PrimitiveComponent Object Reference") (OtherActor :type "Actor Object Reference") (OtherComp :type "PrimitiveComponent Object Reference") (OtherBodyIndex :type Integer) (bFromSweep :type Boolean) (SweepResult :type "HitResult Structure (by ref)"))
  (bind _press (`self.press`))
  (bind _press_2 (`self.press`))
  (bind (_returnvalue_location _returnvalue_rotation) (`KismetMathLibrary.BreakTransform` (`SceneComponent.GetRelativeTransform` _press)))
  (bind (_returnvalue_location_2 _returnvalue_rotation_2) (`KismetMathLibrary.BreakTransform` (`SceneComponent.GetRelativeTransform` _press_2)))
  (if (not (`self.IsPressed`))
    (set `self.IsPressed` true)
    (`KismetSystemLibrary.MoveComponentTo` _press_2 (- _returnvalue_location_2 (0.0 0.0 2.0)) _returnvalue_rotation_2 false false 0.1)
    (for _array_element (`self.InteractWith`)
      (`/Engine/EditorBlueprintResources/StandardMacros.IsValid` _array_element
        (:`Is Valid`
          (`/Game/InteractiveObject/BP_MasterInteractive.AtActivation` _array_element))))
    (`KismetSystemLibrary.Delay` 0.0)
    (`KismetSystemLibrary.MoveComponentTo` _press (+ _returnvalue_location (0.0 0.0 2.0)) _returnvalue_rotation false false 0.1)
    (set `self.IsPressed` false)))

(fn `UserConstructionScript`)