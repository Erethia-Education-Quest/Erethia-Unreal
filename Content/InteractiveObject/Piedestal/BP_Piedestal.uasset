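; BP_Piedestal is an interactive pedestal that reports its activation state to a referenced statue.
; Its Box trigger activates it on begin overlap and deactivates it on end overlap, with no filter on the overlapping actor.
; Both events share one toggle that calls the statue's activated or deactivated handler, passing itself.
; Redundant overlaps only print a debug message, so the first exit deactivates it even if other overlaps remain.
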(event `self.ReceiveBeginPlay`
  (`parent.ReceiveBeginPlay`)
  (set `self.IsActivated` false))

(event `self.Box.OnComponentBeginOverlap`
  (params (OverlappedComponent :type "PrimitiveComponent Object Reference") (OtherActor :type "Actor Object Reference") (OtherComp :type "PrimitiveComponent Object Reference") (OtherBodyIndex :type Integer) (bFromSweep :type Boolean) (SweepResult :type "HitResult Structure (by ref)"))
  (bind _statueref (`self.StatueRef`))
  (if (`self.IsActivated`)
    (`KismetSystemLibrary.PrintText` "piedestal is already activated")
    (else
      (bind _output_get (set `self.IsActivated` (not (`self.IsActivated`)) :!label _label))
      (if _output_get
        (`/Game/InteractiveObject/Statue/BP_CentralStatue.OnPiedestalActivated` _statueref self)
        (else
          (`/Game/InteractiveObject/Statue/BP_CentralStatue.OnPiedestalDesactivated` _statueref self))))))

(event `self.Box.OnComponentEndOverlap`
  (params (OverlappedComponent :type "PrimitiveComponent Object Reference") (OtherActor :type "Actor Object Reference") (OtherComp :type "PrimitiveComponent Object Reference") (OtherBodyIndex :type Integer))
  (if (`self.IsActivated`)
    (goto _label)
    (else
      (`KismetSystemLibrary.PrintText` "piedestal is already desactivated"))))

(fn `UserConstructionScript`
  (`parent.UserConstructionScript`))