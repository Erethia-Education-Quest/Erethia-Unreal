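; BP_Pilar is a selectable pillar that moves across board tiles along a list of destinations.
; A Grabbable_SmallCube overlap asks PilarManager to change its color, and ChangeColor swaps the material and toggles selection.
; MoveTo starts a Tick-driven XY interpolation through each waypoint, keeping current height.
; While idle, overlaps with board tiles record the current tile coordinate; BeginPlay briefly teleports it to origin and back, apparently to refresh overlaps.
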(event `self.ReceiveBeginPlay`
  (`parent.ReceiveBeginPlay`)
  (set `self.PosStart` (`self.K2_GetActorLocation`))
  (`self.K2_SetActorLocation` (0.0 0.0 0.0))
  (`KismetSystemLibrary.Delay` 0.2)
  (`self.K2_SetActorLocation` (`self.PosStart`))
  (set `self.IsSelected` false)
  (set `self.IsMoving?` false))

(event `ChangeColor`
  (params (Material :type "Material Object Reference"))
  (`PrimitiveComponent.SetMaterial` (`self.Cube`) 0 Material)
  (set `self.IsSelected` (not (`self.IsSelected`))))

(event `MoveTo`
  (params (Destination :type "Array of Vector2D Structure"))
  (set `self.AllTargetLocation` Destination)
  (set `self.IsMoving?` true)
  (set `self.Increment` 0))

(event `self.ReceiveTick`
  (params (DeltaSeconds :type "Float (single-precision)"))
  (bind (_returnvalue_x _returnvalue_y _returnvalue_z) (`KismetMathLibrary.BreakVector` (`self.K2_GetActorLocation`)))
  (bind (_returnvalue_x_2 _returnvalue_y_2 _returnvalue_z_2) (`KismetMathLibrary.BreakVector` (`self.K2_GetActorLocation`)))
  (bind (_targetlocation_x _targetlocation_y) (`KismetMathLibrary.BreakVector2D` (`self.TargetLocation`)))
  (bind (_targetlocation_x_2 _targetlocation_y_2) (`KismetMathLibrary.BreakVector2D` (`self.TargetLocation`)))
  (bind _returnvalue (+ (`self.Increment`) 1))
  (if (`self.IsMoving?`)
    (set `self.TargetLocation` (`|GetArrayItem` (`self.AllTargetLocation`) (`self.Increment`)))
    (`self.K2_SetActorLocation` (`KismetMathLibrary.VInterpTo` (`KismetMathLibrary.MakeVector` _returnvalue_x _returnvalue_y _returnvalue_z) (`KismetMathLibrary.MakeVector` _targetlocation_x _targetlocation_y _returnvalue_z) (`GameplayStatics.GetWorldDeltaSeconds`) (`self.MoveSpeed`)))
    (if (== (`KismetMathLibrary.MakeVector` _returnvalue_x_2 _returnvalue_y_2 _returnvalue_z_2) (`KismetMathLibrary.MakeVector` _targetlocation_x_2 _targetlocation_y_2 _returnvalue_z_2))
      (if (`KismetArrayLibrary.Array_IsValidIndex` (`self.AllTargetLocation`) _returnvalue)
        (set `self.Increment` _returnvalue)
        (else
          (set `self.IsMoving?` false))))))

(event `self.Box.OnComponentBeginOverlap`
  (params (OverlappedComponent :type "PrimitiveComponent Object Reference") (OtherActor :type "Actor Object Reference") (OtherComp :type "PrimitiveComponent Object Reference") (OtherBodyIndex :type Integer) (bFromSweep :type Boolean) (SweepResult :type "HitResult Structure (by ref)"))
  (if (`self.IsMoving?`)
    _
    (elif (== (`GameplayStatics.GetObjectClass` OtherActor) "/Game/VRTemplate/Blueprints/Grabbable_SmallCube.Grabbable_SmallCube_C")
      (`/Game/InteractiveObject/Pilar/BP_PilarManager.ChangePilarColor` (`self.PilarManager`) self (`self.IsSelected`))
      (`self.Debug` "Position Pilar   " (`KismetStringLibrary.Conv_VectorToString` (`self.K2_GetActorLocation` self)))
      (else
        (bind _asbox_collision (cast `BoxComponent` OtherComp))
        (if (`.ReturnValue` (`BlueprintMapLibrary.Map_Find` (`/Game/InteractiveObject/Pilar/BP_CheckerBoard.AllTilesRefBoxColision` (`/Game/InteractiveObject/Pilar/BP_PilarManager.RefBoard` (`self.PilarManager`))) _asbox_collision))
          (bind (_returnvalue_x _returnvalue_y) (`KismetMathLibrary.BreakVector` (`SceneComponent.K2_GetComponentLocation` _asbox_collision)))
          (set `self.CurentTileCoord` (`KismetMathLibrary.MakeVector2D` _returnvalue_x _returnvalue_y))
          (`KismetSystemLibrary.PrintText` (`|FormatText` "In Collision with actor {name}" (`KismetSystemLibrary.GetDisplayName` _asbox_collision))))))))

(fn `UserConstructionScript`
  (`parent.UserConstructionScript`))