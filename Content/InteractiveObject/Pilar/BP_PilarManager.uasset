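; Manager actor for checkerboard pillars that highlights selected ones and, once two are selected, sends each along a path to the other's tile.
; PathFinding1 runs a level-by-level breadth-first search in four directions over unflagged tiles from BP_CheckerBoard.
; It rebuilds the route from a visited-parent map, returning it in goal-to-start order for the pillar's MoveTo.
; A helper converts tile coordinates to world positions through the board's collision boxes.
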(event `self.ReceiveBeginPlay`
  (bind _directionarray (`self.DirectionArray`))
  (`parent.ReceiveBeginPlay`)
  (bind _outactors (`GameplayStatics.GetAllActorsOfClass` "/Game/InteractiveObject/Pilar/BP_Pilar.BP_Pilar_C"))
  (set `self.AllPilar` _outactors)
  (bind _returnvalue (`GameplayStatics.GetActorOfClass` "/Game/InteractiveObject/Pilar/BP_CheckerBoard.BP_CheckerBoard_C"))
  (set `self.SizeX` (`/Game/InteractiveObject/Pilar/BP_CheckerBoard.SizeX` _returnvalue))
  (set `self.Sizey` (`/Game/InteractiveObject/Pilar/BP_CheckerBoard.SizeY` _returnvalue))
  (bind _returnvalue_2 (`GameplayStatics.GetActorOfClass` "/Game/InteractiveObject/Pilar/BP_CheckerBoard.BP_CheckerBoard_C"))
  (bind _output_get (set `self.RefBoard` _returnvalue_2))
  (set `self.AvalableTiles` (`/Game/InteractiveObject/Pilar/BP_CheckerBoard.AllTIles` _output_get))
  (`KismetArrayLibrary.Array_Add` _directionarray (1.0 0.0))
  (`KismetArrayLibrary.Array_Add` _directionarray (-1.0 0.0))
  (`KismetArrayLibrary.Array_Add` _directionarray (0.0 1.0))
  (`KismetArrayLibrary.Array_Add` _directionarray (0.0 -1.0)))

(event `ChangePilarColor`
  (params (Pilar :type "/Game/InteractiveObject/Pilar/BP_Pilar Object Reference") (IsSelected :type Boolean))
  (bind _selectedpilar (`self.SelectedPilar`))
  (bind _selectedpilar_2 (`self.SelectedPilar`))
  (if IsSelected
    (`/Game/InteractiveObject/Pilar/BP_Pilar.ChangeColor` Pilar (`self.BaseMaterial`))
    (`KismetArrayLibrary.Array_RemoveItem` _selectedpilar Pilar)
    (else
      (`/Game/InteractiveObject/Pilar/BP_Pilar.ChangeColor` Pilar (`self.SelectedMaterial`))
      (`KismetArrayLibrary.Array_Add` _selectedpilar Pilar)
      (if (== (`KismetArrayLibrary.Array_Length` _selectedpilar) 2)
        (`self.SwitchPilarPosition` (`|GetArrayItem` _selectedpilar_2) (`|GetArrayItem` _selectedpilar_2 1))
        (for _array_element (`self.SelectedPilar`)
          (`/Game/InteractiveObject/Pilar/BP_Pilar.ChangeColor` _array_element (`self.BaseMaterial`))
          (`KismetArrayLibrary.Array_RemoveItem` (`self.SelectedPilar`) _array_element))))))

(event `SwitchPilarPosition`
  (params (Pilar1 :type "/Game/InteractiveObject/Pilar/BP_Pilar Object Reference") (Pilar2 :type "/Game/InteractiveObject/Pilar/BP_Pilar Object Reference"))
  (bind _curenttilecoord (`/Game/InteractiveObject/Pilar/BP_Pilar.CurentTileCoord` Pilar2))
  (bind _curenttilecoord_2 (`/Game/InteractiveObject/Pilar/BP_Pilar.CurentTileCoord` Pilar1))
  (`|ExecutionSequence`
    (:`then_0`
      (bind _path (`self.Path Finding 1` _curenttilecoord_2 _curenttilecoord))
      (`/Game/InteractiveObject/Pilar/BP_Pilar.MoveTo` Pilar1 _path))
    (:`then_1`
      (bind _path_2 (`self.Path Finding 1` _curenttilecoord _curenttilecoord_2))
      (`/Game/InteractiveObject/Pilar/BP_Pilar.MoveTo` Pilar2 _path_2))))

(fn `GetBoxWorldPosition`
  (params (BoxRelativePosition :type "Vector2D Structure"))
  (returns (NewParam :type "Vector Structure"))
  (bind _returnvalue (`GameplayStatics.GetActorOfClass` "/Game/InteractiveObject/Pilar/BP_CheckerBoard.BP_CheckerBoard_C"))
  (bind _output_get (set `self.RefBoard` _returnvalue))
  (bind _alltilesrefboxcolision (`/Game/InteractiveObject/Pilar/BP_CheckerBoard.AllTilesRefBoxColision` _output_get))
  (bind _keys (`BlueprintMapLibrary.Map_Keys` _alltilesrefboxcolision))
  (bind _values (`BlueprintMapLibrary.Map_Values` _alltilesrefboxcolision))
  (for (_array_element _array_index) _values
    (if (== BoxRelativePosition _array_element)
      (break)))
  (return (`SceneComponent.K2_GetComponentLocation` (`|GetArrayItem` _keys _array_index))))

(fn `Path Finding 1`
  (params (StartTile :type "Vector2D Structure") (FinalTile :type "Vector2D Structure"))
  (returns (Path :type "Array of Vector2D Structure"))
  (bind _pf1_queue (`self.PF1_Queue`))
  (bind _pf1_visited (`self.PF1_Visited`))
  (bind _pf1_finalpath (`self.PF1_FinalPath`))
  (bind _alltilestotest (`self.AllTIlesToTest`))
  (bind _curenttile (`self.CurentTile`))
  (bind _pf1_queue_2 (`self.PF1_Queue`))
  (bind _curenttile_2 (`self.CurentTile`))
  (bind _value (`BlueprintMapLibrary.Map_Find` (`self.PF1_Visited`) _curenttile))
  (`KismetArrayLibrary.Array_Clear` (`self.AllTIlesToTest`))
  (`BlueprintMapLibrary.Map_Clear` (`self.PF1_Visited`))
  (`KismetArrayLibrary.Array_Clear` (`self.PF1_FinalPath`))
  (`KismetArrayLibrary.Array_Clear` _pf1_queue)
  (`KismetArrayLibrary.Array_Add` _pf1_queue StartTile)
  (set `self.PF1_FoundPath` false)
  (`BlueprintMapLibrary.Map_Add` (`self.PF1_Visited`) StartTile StartTile)
  (`KismetArrayLibrary.Array_Add` (`self.PF1_FinalPath`) FinalTile)
  (if (> (`KismetArrayLibrary.Array_Length` (`self.PF1_Queue`)) 0) :!label _label
    (bind _output_get (set `self.CurentTile` (`|GetArrayItem` _pf1_queue_2)))
    (`KismetArrayLibrary.Array_Add` (`self.AllTIlesToTest`) (`|GetArrayItem` _pf1_queue_2))
    (`KismetArrayLibrary.Array_Remove` _pf1_queue_2)
    (if (== _output_get FinalTile)
      (set `self.CurentTile` FinalTile)
      (while (!= _curenttile StartTile)
        (`KismetArrayLibrary.Array_Add` _pf1_finalpath _value)
        (set `self.CurentTile` _value))
      (return _pf1_finalpath)
      (else
        (goto _label)))
    (else
      (for _array_element _alltilestotest
        (set `self.CurentTile` _array_element)
        (for _array_element_2 (`self.DirectionArray`)
          (bind _returnvalue (+ _curenttile_2 _array_element_2))
          (bind (_value_2 _returnvalue_2) (`BlueprintMapLibrary.Map_Find` (`self.AvalableTiles`) _returnvalue))
          (if _returnvalue_2
            (if _value_2
              _
              (elif (not (`.ReturnValue` (`BlueprintMapLibrary.Map_Find` _pf1_visited _returnvalue)))
                (`KismetArrayLibrary.Array_Add` (`self.PF1_Queue`) _returnvalue)
                (`BlueprintMapLibrary.Map_Add` _pf1_visited _returnvalue _curenttile_2))))))
      (`KismetArrayLibrary.Array_Clear` _alltilestotest)
      (goto _label))))

(fn `UserConstructionScript`
  (`parent.UserConstructionScript`))