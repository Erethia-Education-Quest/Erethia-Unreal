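; BP_PilarMaster is a manager actor for pillar interaction that lets two selected BP_Pilar actors swap positions.
; BeginPlay caches every BP_Pilar, though this graph never reads that list.
; ChangePilarColor toggles a pillar's material and membership in SelectedPilar.
; When two are selected, SwitchPilarPosition moves each to the other's location, then a loop resets materials while removing entries from the array it iterates.
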(event `self.ReceiveBeginPlay`
  (`parent.ReceiveBeginPlay`)
  (bind _outactors (`GameplayStatics.GetAllActorsOfClass` "/Game/InteractiveObject/Pilar/BP_Pilar.BP_Pilar_C"))
  (set `self.AllPilar` _outactors))

(event `ChangePilarColor`
  (params (Pilar :type "/Game/InteractiveObject/Pilar/BP_Pilar Object Reference") (IsSelected :type Boolean))
  (bind _selectedpilar (`self.SelectedPilar`))
  (bind _selectedpilar_2 (`self.SelectedPilar`))
  (if IsSelected
    (`/Game/InteractiveObject/Pilar/BP_Pilar.ChangeColor` Pilar (`self.BaseMaterial`))
    (`KismetArrayLibrary.Array_RemoveItem` _selectedpilar Pilar)
    (else
      (`/Game/InteractiveObject/Pilar/BP_Pilar.ChangeColor` Pilar (`self.SelectedMaterial`))
      (`KismetArrayLibrary.Array_Add` _selectedpilar Pilar)
      (if (== (`KismetArrayLibrary.Array_Length` _selectedpilar) 2)
        (`self.SwitchPilarPosition` (`|GetArrayItem` _selectedpilar_2) (`|GetArrayItem` _selectedpilar_2 1))
        (for _array_element (`self.SelectedPilar`)
          (`/Game/InteractiveObject/Pilar/BP_Pilar.ChangeColor` _array_element (`self.BaseMaterial`))
          (`KismetArrayLibrary.Array_RemoveItem` (`self.SelectedPilar`) _array_element))))))

(event `SwitchPilarPosition`
  (params (Pilar1 :type "/Game/InteractiveObject/Pilar/BP_Pilar Object Reference") (Pilar2 :type "/Game/InteractiveObject/Pilar/BP_Pilar Object Reference"))
  (bind _output_get (set `self.Temp1` (`self.K2_GetActorLocation` Pilar1)))
  (bind _output_get_2 (set `self.Temps2` (`self.K2_GetActorLocation` Pilar2)))
  (`/Game/InteractiveObject/Pilar/BP_Pilar.MoveTo` Pilar1 _output_get_2)
  (`/Game/InteractiveObject/Pilar/BP_Pilar.MoveTo` Pilar2 _output_get))

(fn `UserConstructionScript`
  (`parent.UserConstructionScript`))