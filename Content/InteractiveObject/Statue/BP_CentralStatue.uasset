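; Central statue that turns its Cube component to face the first inactive pedestal in the level.
; On BeginPlay it gathers every BP_Piedestal actor and builds a parallel array of activation states, all starting false.
; Activation and deactivation events update the matching state and set a dirty flag.
; When flagged, Tick finds the first inactive entry and uses MoveComponentTo with a look-at yaw to rotate the cube smoothly toward that pedestal.
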(event `self.ReceiveBeginPlay`
  (`parent.ReceiveBeginPlay`)
  (bind _outactors (`GameplayStatics.GetAllActorsOfClass` "/Game/InteractiveObject/Piedestal/BP_Piedestal.BP_Piedestal_C"))
  (bind _output_get (set `self.AllPedestals` _outactors))
  (for _ _output_get
    (`KismetArrayLibrary.Array_Add` (`self.PiedestalsState`)))
  (set `self.HaveChanged` true))

(event `OnPiedestalActivated`
  (params (piedestalIndex :type "/Game/InteractiveObject/Piedestal/BP_Piedestal Object Reference"))
  (for (_array_element _array_index) (`self.AllPedestals`)
    (if (== _array_element piedestalIndex)
      (`KismetArrayLibrary.Array_Set` (`self.PiedestalsState`) _array_index true)))
  (set `self.HaveChanged` true))

(event `OnPiedestalDesactivated`
  (params (piedestalIndex :type "/Game/InteractiveObject/Piedestal/BP_Piedestal Object Reference"))
  (for (_array_element _array_index) (`self.AllPedestals`)
    (if (== _array_element piedestalIndex)
      (`KismetArrayLibrary.Array_Set` (`self.PiedestalsState`) _array_index)))
  (set `self.HaveChanged` true))

(event `self.ReceiveTick`
  (params (DeltaSeconds :type "Float (single-precision)"))
  (if (`self.HaveChanged`)
    (for (_array_element _array_index) (`self.PiedestalsState`)
      (if (== false _array_element)
        (bind (_returnvalue_roll _returnvalue_pitch _returnvalue_yaw) (`KismetMathLibrary.BreakRotator` (`KismetMathLibrary.FindLookAtRotation` (`self.K2_GetActorLocation`) (`self.K2_GetActorLocation` (`|GetArrayItem` (`self.AllPedestals`) _array_index)))))
        (`KismetSystemLibrary.MoveComponentTo` (`self.Cube`) (0.0 0.0 0.0) (`KismetMathLibrary.MakeRotator` 0.0 0.0 _returnvalue_yaw) false false 1.0)
        (break)))
    (set `self.HaveChanged` false)))

(fn `UserConstructionScript`
  (`parent.UserConstructionScript`))